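; RoadTrack is a Blueprint that builds a road from spline mesh segments along its RoadTrack spline.
; The construction script divides the spline length by Distance and adds a SplineMeshComponent with StaticMesh for each interval, including a final one for the remainder.
; Segment endpoints are sampled in local space, with tangents computed as those positions times Tangent rather than read from the spline.
; The event graph has no active logic.
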(fn `UserConstructionScript`
  (bind _roadtrack (`self.RoadTrack`))
  (bind _distance (`self.Distance`))
  (for _index (range (+ (`.ReturnValue` (`KismetMathLibrary.FMod` (`SplineComponent.GetSplineLength` (`self.RoadTrack`)) (`self.Distance`))) 1))
    (bind _returnvalue (`AddComponent|NODE_AddSplineMeshComponent-0`))
    (`StaticMeshComponent.SetStaticMesh` _returnvalue (`self.Static Mesh`))
    (bind _returnvalue_2 (* _index _distance))
    (bind _returnvalue_3 (+ _returnvalue_2 _distance))
    (`SplineMeshComponent.SetStartAndEnd` _returnvalue (`SplineComponent.GetLocationAtDistanceAlongSpline` _roadtrack _returnvalue_2 "Local") (* (`SplineComponent.GetLocationAtDistanceAlongSpline` _roadtrack _returnvalue_2 "Local") (`self.Tangent`)) (`SplineComponent.GetLocationAtDistanceAlongSpline` _roadtrack _returnvalue_3 "Local") (* (`SplineComponent.GetLocationAtDistanceAlongSpline` _roadtrack _returnvalue_3 "Local") (`self.Tangent`)) true)))