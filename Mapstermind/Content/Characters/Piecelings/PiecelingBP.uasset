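; Player-controlled Pieceling character for a local multiplayer game, able to carry task items, pull levers, and show shout and countdown indicators.
; Capsule overlaps set the current item, which Interact picks up or drops through per-type casts.
; The held item type steers a widget compass toward the matching task actor, rotated relative to control yaw each tick.
; Timed events alter walk speed or invert controls, and Tick gates input on trap and start-sequence state.
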(event `self.ReceiveBeginPlay`
  (`PrimitiveComponent.SetCastShadow` (`self.Compass`) false)
  (`PrimitiveComponent.SetCastShadow` (`self.Countdown`) false)
  (`PrimitiveComponent.SetCastShadow` (`self.Shout`) false)
  (bind _returnvalue (`GameplayStatics.GetActorOfClass` "/Game/Blueprints/Tasks/TheaterTask.TheaterTask_C"))
  (set `self.Theater` _returnvalue)
  (bind _returnvalue_2 (`GameplayStatics.GetActorOfClass` "/Game/Blueprints/Tasks/Stadium.Stadium_C"))
  (set `self.Stadium` _returnvalue_2)
  (bind _returnvalue_3 (`GameplayStatics.GetActorOfClass` "/Game/Blueprints/Tasks/HourglassCollector.HourglassCollector_C"))
  (set `self.ClockTower` _returnvalue_3)
  (bind _returnvalue_4 (`GameplayStatics.GetActorOfClass` "/Game/Blueprints/Tutorial/Tasks/TutorialTheaterTask.TutorialTheaterTask_C"))
  (set `self.TutorialTheater` _returnvalue_4)
  (bind _returnvalue_5 (`GameplayStatics.GetActorOfClass` "/Game/Blueprints/Tutorial/Tasks/TutorialStadium.TutorialStadium_C"))
  (set `self.TutorialStadium` _returnvalue_5)
  (bind _returnvalue_6 (`GameplayStatics.GetActorOfClass` "/Game/Blueprints/Tutorial/Tasks/TutorialHourglassCollector.TutorialHourglassCollector_C"))
  (set `self.TutorialClock` _returnvalue_6)
  (if (`NavMovementComponent.IsFalling` (`self.CharacterMovement`))
    (`self.DisableInput` null))
  (bind _aslocal_mpgame_mode (cast `/Game/Blueprints/Modes_States/LocalMPGameMode` (`GameplayStatics.GetGameMode`)))
  (set `self.GameMode` _aslocal_mpgame_mode))

(event `self.ReceiveTick`
  (params (DeltaSeconds :type "Float (single-precision)"))
  (`|ExecutionSequence`
    (:`then_0`
      (if (`self.Trapped`)
        (`self.DisableInput` null)
        (else
          (`self.EnableInput` null))))
    (:`then_1`
      (`self.PointCompass`)
      (`/Engine/EditorBlueprintResources/StandardMacros.IsValid` (`self.HeldItem`)
        (:`Is Valid`
          _)
        (:`Is Not Valid`
          (set `self.CompassRotating` false)))
      (if (`NavMovementComponent.IsFalling` (`self.CharacterMovement`))
        _
        (elif (`/Game/Blueprints/Modes_States/LocalMPGameMode.StartSequenceEnded` (`self.GameMode`))
          (`self.EnableInput` null))))))

(event `InputAxis|PullLever`
  (params (AxisValue :type "Float (single-precision)"))
  (bind _currentlever (`self.CurrentLever`))
  (bind _currentlever_2 (`self.CurrentLever`))
  ;[0 0.7751 1] Pull Lever
  (`/Engine/EditorBlueprintResources/StandardMacros.IsValid` _currentlever
    (:`Is Valid`
      (if (and (< AxisValue -0.5) (`Lever.CanActivate` _currentlever))
        (if (`self.PullingLever`)
          (bind _assingle_lever (cast `/Game/Blueprints/Tasks/SingleLever` _currentlever_2)
            (:`then`
              (`/Game/Blueprints/Tasks/SingleLever.Activate` _assingle_lever))
            (:`CastFailed`
              (bind _asalternate_lever (cast `/Game/Blueprints/Tasks/AlternateLever` _currentlever_2))
              (`/Game/Blueprints/Tasks/LeverManager.FlipLever` (`/Game/Blueprints/Tasks/AlternateLever.Manager` _asalternate_lever) _asalternate_lever self))))))))

(event `self.CapsuleComponent.OnComponentBeginOverlap`
  (params (OverlappedComponent :type "PrimitiveComponent Object Reference") (OtherActor :type "Actor Object Reference") (OtherComp :type "PrimitiveComponent Object Reference") (OtherBodyIndex :type Integer) (bFromSweep :type Boolean) (SweepResult :type "HitResult Structure (by ref)"))
  (`self.CheckItemPickup` OtherActor)
  (bind _asmask (cast `/Game/Blueprints/Tasks/Mask` OtherActor))
  (set `self.CurrentItem` _asmask))

(event `InputAction|Shout`
  (params (Key :type "Key Structure"))
  (bind _shout (`self.Shout`))
  (bind (_returnvalue_x _returnvalue_y _returnvalue_z) (`KismetMathLibrary.BreakVector` (`SceneComponent.K2_GetComponentLocation` (`self.CapsuleComponent`))))
  ;[1 0.807 0.1156] Shout
  (:`Pressed`
    (if (not (`self.ShoutCoolDown`))
      (set `self.ShoutCoolDown` true)
      (`SceneComponent.K2_SetWorldLocation` _shout (`KismetMathLibrary.MakeVector` _returnvalue_x _returnvalue_y (+ _returnvalue_z 700.0)) false false)
      (`SceneComponent.SetVisibility` _shout true false)
      (`KismetSystemLibrary.Delay` 0.5)
      (set `self.ShoutCoolDown` false)
      (`KismetSystemLibrary.Delay` 2.0)
      (`SceneComponent.SetVisibility` _shout false false))))

(event `self.CapsuleComponent.OnComponentEndOverlap`
  (params (OverlappedComponent :type "PrimitiveComponent Object Reference") (OtherActor :type "Actor Object Reference") (OtherComp :type "PrimitiveComponent Object Reference") (OtherBodyIndex :type Integer))
  (`self.CheckItemDrop` OtherActor)
  (cast `/Game/Blueprints/Tasks/Mask` OtherActor)
  (set `self.CurrentItem` null))

(event `InputAction|Interact`
  (params (Key :type "Key Structure"))
  (bind _currentlever (`self.CurrentLever`))
  (bind _currentlever_2 (`self.CurrentLever`))
  ;[1 0.3315 0] Interact with items
  (:`Pressed`
    (`|ExecutionSequence`
      (:`then_0`
        (`/Engine/EditorBlueprintResources/StandardMacros.IsValid` (`self.CurrentItem`)
          (:`Is Valid`
            (`/Engine/EditorBlueprintResources/StandardMacros.IsValid` (`self.HeldItem`)
              (:`Is Valid`
                (`self.DropItem`))
              (:`Is Not Valid`
                (`GameplayStatics.PlaySoundAtLocation` "/Game/Audio/SoundEffects/ObjectAttach.ObjectAttach" (0.0 0.0 0.0) (struct) 0.8 0.8 0.0 null null null)
                (bind _output_get (set `self.HeldItem` (`self.CurrentItem`)))
                (`self.Pickup` _output_get)
                (bind _asmask (cast `/Game/Blueprints/Tasks/Mask` _output_get))
                (if (not (`/Game/Blueprints/Tasks/Mask.Grabbed` _asmask))
                  (`/Game/Blueprints/Tasks/Mask.PickUp` _asmask self (`SceneComponent.K2_GetComponentLocation` (`self.ItemPoint`)))
                  (set `self.HeldItemType` "NewEnumerator2")
                  (set `self.CompassRotating` true)))))))
      (:`then_1`
        (`/Engine/EditorBlueprintResources/StandardMacros.IsValid` _currentlever
          (:`Is Valid`
            (if (`Lever.CanActivate` _currentlever)
              (`CharacterMovementComponent.DisableMovement` (`self.CharacterMovement`))
              (set `self.PullingLever` true)
              (bind _assingle_lever (cast `/Game/Blueprints/Tasks/SingleLever` _currentlever_2)
                (:`then`
                  (bind _aslever_hud (cast `/Game/Blueprints/Widgets/Level/LeverHUD` (`WidgetComponent.GetWidget` (`/Game/Blueprints/Tasks/SingleLever.Widget` _assingle_lever))))
                  (`/Game/Blueprints/Widgets/Level/LeverHUD.ShowPull` _aslever_hud))
                (:`CastFailed`
                  (bind _asalternate_lever (cast `/Game/Blueprints/Tasks/AlternateLever` _currentlever_2))
                  (bind _aslever_hud_2 (cast `/Game/Blueprints/Widgets/Level/LeverHUD` (`WidgetComponent.GetWidget` (`/Game/Blueprints/Tasks/AlternateLever.Widget` _asalternate_lever))))
                  (`/Game/Blueprints/Widgets/Level/LeverHUD.ShowPull` _aslever_hud_2))))))))))

(event `InputAction|Countdown`
  (params (Key :type "Key Structure"))
  ;[1 1 1] Countdown
  (:`Pressed`
    (if (not (`self.TimeCoolDown`))
      (set `self.Counter` 3)
      (set `self.CountingDown` true)
      (set `self.TimeCoolDown` true)
      (`SceneComponent.SetVisibility` (`self.Countdown`) true false)
      (`KismetSystemLibrary.K2_SetTimer` null "DecrementTimer" 1.0 (`self.CountingDown`))
      (`KismetSystemLibrary.Delay` 6.0)
      (set `self.TimeCoolDown` false))))

(event `PointCompass`
  (bind _clocktower (`self.ClockTower`))
  (bind _theater (`self.Theater`))
  (bind _compass (`self.Compass`))
  ;[1 1 1] Task Compass
  (if (`self.CompassRotating`)
    (`/Engine/EditorBlueprintResources/StandardMacros.IsValid` (`self.HeldItem`)
      (:`Is Valid`
        (`SceneComponent.SetVisibility` _compass true false)
        (switch `/Game/Blueprints/Traps/ItemTypes` (`self.HeldItemType`)
          (:`NewEnumerator0`
            (`/Engine/EditorBlueprintResources/StandardMacros.IsValid` _clocktower
              (:`Is Valid`
                (`self.SetCompassTarget` _clocktower))
              (:`Is Not Valid`
                (`self.SetCompassTarget` (`self.TutorialClock`)))))
          (:`NewEnumerator2`
            (`/Engine/EditorBlueprintResources/StandardMacros.IsValid` _theater
              (:`Is Valid`
                (`self.SetCompassTarget` _theater))
              (:`Is Not Valid`
                (`self.SetCompassTarget` (`self.TutorialTheater`) :!label _label))))
          (:`NewEnumerator3`
            (`self.SetCompassTarget` (`self.Stadium`)))
          (:`NewEnumerator4`
            (`self.SetCompassTarget` (`self.TutorialStadium`)))
          (:`NewEnumerator6`
            (goto _label))
          (:`NewEnumerator7`
            (bind _returnvalue (`GameplayStatics.GetActorOfClass` "/Game/Blueprints/Tasks/GiantClam.GiantClam_C" :!label _label_2))
            (`self.SetCompassTarget` _returnvalue))
          (:`NewEnumerator8`
            (goto _label_2))
          (:`NewEnumerator9`
            (bind _returnvalue_2 (`GameplayStatics.GetActorOfClass` "/Game/Blueprints/Tasks/MermaidTask.MermaidTask_C" :!label _label_3))
            (`self.SetCompassTarget` _returnvalue_2))
          (:`NewEnumerator10`
            (goto _label_3))
          (:`NewEnumerator11`
            (goto _label_3))))
      (:`Is Not Valid`
        (set `self.CompassRotating` false)
        (`SceneComponent.SetVisibility` _compass false false :!label _label_4)))
    (else
      (goto _label_4))))

(event `ChangeSpeed`
  (params (NewSpeed :type "Float (double-precision)") (Time :type "Float (double-precision)"))
  (bind _charactermovement (`self.CharacterMovement`))
  (bind _output_get (set `CharacterMovementComponent.MaxWalkSpeed` (/ (`CharacterMovementComponent.MaxWalkSpeed` _charactermovement) NewSpeed) _charactermovement))
  (`KismetSystemLibrary.Delay` Time)
  (set `CharacterMovementComponent.MaxWalkSpeed` (* _output_get NewSpeed) _charactermovement)
  (if (`self.Slowed`)
    (set `self.Slowed` false)))

(event `ReverseControls`
  (params (Time :type "Float (double-precision)"))
  (set `self.invertMovement` true)
  (`KismetSystemLibrary.Delay` Time)
  (set `self.invertMovement` false))

(event `DropItem`
  ;[0 1 0.2992] Drop Items
  (`self.Drop` (`self.HeldItem`))
  (switch `/Game/Blueprints/Traps/ItemTypes` (`self.HeldItemType`)
    (:`NewEnumerator2`
      (bind _asmask (cast `/Game/Blueprints/Tasks/Mask` (`self.HeldItem`)))
      (`/Game/Blueprints/Tasks/Mask.Drop` _asmask self)
      (set `self.HeldItem` null)
      (set `self.CompassRotating` false))))

(fn `CheckItemDrop`
  (params (Actor :type "Actor Object Reference"))
  (bind _currentitem (`self.CurrentItem`))
  (bind _asitem (cast `Item` Actor))
  (switch `EItemType` (`Item.itemType` _asitem)
    (:`MASK`
      (set `self.CurrentItem` null :!label _label))
    (:`BASEBALL`
      (bind _asbaseball (cast `/Game/Blueprints/Tasks/Baseball` _currentitem))
      (`/Game/Blueprints/Tasks/Baseball.PickupUI_Invisible` _asbaseball)
      (goto _label))
    (:`HOURGLASS`
      (bind _ashourglass (cast `/Game/Blueprints/Tasks/Hourglass` _currentitem))
      (`/Game/Blueprints/Tasks/Hourglass.PickupUI_Invisible` _ashourglass)
      (goto _label))
    (:`CLAMHAT`
      (cast `/Game/Blueprints/Tasks/ClamHat` _currentitem))))

(fn `CheckItemPickup`
  (params (Actor :type "Actor Object Reference"))
  (bind _currentitem (`self.CurrentItem`))
  (bind _asitem (cast `Item` Actor))
  (set `self.CurrentItem` _asitem)
  (switch `EItemType` (`Item.itemType` _asitem)
    (:`BASEBALL`
      (bind _asbaseball (cast `/Game/Blueprints/Tasks/Baseball` _currentitem))
      (`/Game/Blueprints/Tasks/Baseball.PickupUI_Visible` _asbaseball))
    (:`HOURGLASS`
      (bind _ashourglass (cast `/Game/Blueprints/Tasks/Hourglass` _currentitem))
      (`/Game/Blueprints/Tasks/Hourglass.PickupUI_Visible` _ashourglass))
    (:`CLAMHAT`
      (cast `/Game/Blueprints/Tasks/ClamHat` _currentitem))))

(fn `DecrementTimer`
  (bind _output_get (set `self.Counter` (- (`self.Counter`) 1)))
  (if (<= _output_get 0)
    (set `self.CountingDown` false)
    (`SceneComponent.SetVisibility` (`self.Countdown`) false false)
    (set `self.Counter` 3)))

(fn `Drop`
  (params (Item :type "Actor Object Reference"))
  (bind _asitem (cast `Item` Item))
  (switch `EItemType` (`Item.itemType` _asitem)
    (:`BASEBALL`
      (bind _asbaseball (cast `/Game/Blueprints/Tasks/Baseball` _asitem))
      (`/Game/Blueprints/Tasks/Baseball.Drop` _asbaseball self)
      (set `self.CompassRotating` false))
    (:`HOURGLASS`
      (bind _ashourglass (cast `/Game/Blueprints/Tasks/Hourglass` _asitem))
      (`/Game/Blueprints/Tasks/Hourglass.Drop` _ashourglass)
      (set `self.CompassRotating` false))
    (:`TUTORIAL`
      (bind _astutorial_baseball (cast `/Game/Blueprints/Tasks/TutorialBaseball` _asitem))
      (`/Game/Blueprints/Tasks/TutorialBaseball.Drop` _astutorial_baseball self))
    (:`CLAMHAT`
      (bind _asclam_hat (cast `/Game/Blueprints/Tasks/ClamHat` _asitem))
      (`/Game/Blueprints/Tasks/ClamHat.Drop` _asclam_hat))
    (:`CLAMEYES`
      (bind _asclam_eyes (cast `/Game/Blueprints/Tasks/ClamEyes` _asitem))
      (`/Game/Blueprints/Tasks/ClamEyes.Drop` _asclam_eyes))
    (:`PEARL`
      (bind _aspearl (cast `/Game/Blueprints/Tasks/Pearl` _asitem))
      (`/Game/Blueprints/Tasks/Pearl.Drop` _aspearl))
    (:`CROWN`
      (bind _ascrown_pickup (cast `/Game/Blueprints/Tasks/CrownPickup` _asitem))
      (`/Game/Blueprints/Tasks/CrownPickup.Drop` _ascrown_pickup))
    (:`Goblet`
      (bind _asgoblet (cast `/Game/Blueprints/Tasks/Goblet` _asitem))
      (`/Game/Blueprints/Tasks/Goblet.Drop` _asgoblet)))
  (set `self.HeldItem` null)
  (set `self.HeldItemType` "NewEnumerator5"))

(fn `Pickup`
  (params (Item :type "Actor Object Reference"))
  (bind _returnvalue (`SceneComponent.K2_GetComponentLocation` (`self.ItemPoint`)))
  (bind _asitem (cast `Item` Item))
  (switch `EItemType` (`Item.itemType` _asitem)
    (:`BASEBALL`
      (bind _asbaseball (cast `/Game/Blueprints/Tasks/Baseball` _asitem))
      (`/Game/Blueprints/Tasks/Baseball.PickUp` _asbaseball self _returnvalue)
      (set `self.CompassRotating` true)
      (set `self.HeldItemType` "NewEnumerator3"))
    (:`HOURGLASS`
      (bind _ashourglass (cast `/Game/Blueprints/Tasks/Hourglass` _asitem))
      (`/Game/Blueprints/Tasks/Hourglass.PickUp` _ashourglass self _returnvalue)
      (set `self.CompassRotating` true)
      (set `self.HeldItemType` "NewEnumerator0"))
    (:`TUTORIAL`
      (bind _astutorial_baseball (cast `/Game/Blueprints/Tasks/TutorialBaseball` _asitem))
      (`/Game/Blueprints/Tasks/TutorialBaseball.PickUp` _astutorial_baseball self _returnvalue)
      (set `self.CompassRotating` true)
      (set `self.HeldItemType` "NewEnumerator4"))
    (:`CLAMHAT`
      (bind _asclam_hat (cast `/Game/Blueprints/Tasks/ClamHat` _asitem))
      (`/Game/Blueprints/Tasks/ClamHat.PickUp` _asclam_hat self _returnvalue)
      (set `self.CompassRotating` true)
      (set `self.HeldItemType` "NewEnumerator8"))
    (:`CLAMEYES`
      (bind _asclam_eyes (cast `/Game/Blueprints/Tasks/ClamEyes` _asitem))
      (`/Game/Blueprints/Tasks/ClamEyes.PickUp` _asclam_eyes self _returnvalue)
      (set `self.CompassRotating` true)
      (set `self.HeldItemType` "NewEnumerator7"))
    (:`PEARL`
      (bind _aspearl (cast `/Game/Blueprints/Tasks/Pearl` _asitem))
      (`/Game/Blueprints/Tasks/Pearl.PickUp` _aspearl self _returnvalue)
      (set `self.CompassRotating` true)
      (set `self.HeldItemType` "NewEnumerator11"))
    (:`CROWN`
      (bind _ascrown_pickup (cast `/Game/Blueprints/Tasks/CrownPickup` _asitem))
      (`/Game/Blueprints/Tasks/CrownPickup.Pickup` _ascrown_pickup self _returnvalue)
      (set `self.CompassRotating` true)
      (set `self.HeldItemType` "NewEnumerator9"))
    (:`Goblet`
      (bind _asgoblet (cast `/Game/Blueprints/Tasks/Goblet` _asitem))
      (`/Game/Blueprints/Tasks/Goblet.PickUp` _asgoblet self _returnvalue)
      (set `self.CompassRotating` true)
      (set `self.HeldItemType` "NewEnumerator10"))))

(fn `SetCompassTarget`
  (params (Target :type "Actor Object Reference"))
  (bind (_returnvalue_roll _returnvalue_pitch _returnvalue_yaw) (`KismetMathLibrary.BreakRotator` (`self.GetControlRotation`)))
  (bind _compass (`self.Compass`))
  (bind (_returnvalue_roll_2 _returnvalue_pitch_2 _returnvalue_yaw_2) (`KismetMathLibrary.BreakRotator` (`KismetMathLibrary.FindLookAtRotation` (`self.K2_GetActorLocation` Target) (`SceneComponent.K2_GetComponentLocation` _compass))))
  (`Widget.SetRenderTransformAngle` (`WidgetComponent.GetWidget` _compass) (- _returnvalue_yaw_2 _returnvalue_yaw)))

(fn `UserConstructionScript`)