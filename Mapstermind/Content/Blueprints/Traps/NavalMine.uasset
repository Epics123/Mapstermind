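; Naval mine trap that knocks back and stuns any Pieceling touching its collider.
; On overlap it launches the character with a high-arc suggested velocity using identical start and end points, disables input, and plays an explosion sound at world origin.
; After the stun delay it restores input and tells its Manager to destroy the mines.
; A Rise event animates the mine up to a given location by timeline; the timed self-destroy is unwired.
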(event `self.ActivatePlacedTrap`)

(event `self.ReceiveDestroyed`)

(event `Start Timer`)

(event `self.PiecelingCollider.OnComponentBeginOverlap`
  (params (OverlappedComponent :type "PrimitiveComponent Object Reference") (OtherActor :type "Actor Object Reference") (OtherComp :type "PrimitiveComponent Object Reference") (OtherBodyIndex :type Integer) (bFromSweep :type Boolean) (SweepResult :type "HitResult Structure (by ref)"))
  (bind _playerref (`self.PlayerRef`))
  (bind _aspieceling_bp (cast `/Game/Characters/Piecelings/PiecelingBP` OtherActor))
  (bind _output_get (set `self.PlayerRef` _aspieceling_bp))
  (bind _returnvalue (`self.K2_GetActorLocation` _output_get))
  (bind _tossvelocity (`GameplayStatics.BlueprintSuggestProjectileVelocity` _returnvalue _returnvalue (`self.KnockbackSpeed`) 0.0 "DoNotTrace" 0.0 true))
  (`Character.LaunchCharacter` _playerref _tossvelocity true true)
  (`self.DisableInput` _playerref null)
  (`GameplayStatics.PlaySoundAtLocation` "/Game/Audio/SoundEffects/GavinsSounds/NAVAL_MINE_UNDERWATER_EXPLOSION.NAVAL_MINE_UNDERWATER_EXPLOSION" (0.0 0.0 0.0) (struct) 1.0 1.0 0.0 null null null)
  (`KismetSystemLibrary.Delay` (`self.StunDuration`))
  (`self.EnableInput` _playerref null)
  (`/Game/Blueprints/Traps/NavalMinesManager.DestroyMines` (`self.Manager`)))

(event `Rise`
  (params (Location :type "Vector Structure"))
  (bind (_direction _move) (`Timeline|RiseTL` :!via `PlayFromStart`)
    (:`Update`
      (`self.K2_SetActorRelativeLocation` (`KismetMathLibrary.MakeVector` Location_X Location_Y (`KismetMathLibrary.Lerp` -850.0 Location_Z _move))))))

(fn `UserConstructionScript`)