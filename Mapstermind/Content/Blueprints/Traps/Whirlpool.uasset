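; Whirlpool trap that pulls every Pieceling to its center, holds them, then flings them to random landing spots.
; ActivateWhirlpool shows the effect, drops held items, disables input and launches characters on high suggested-projectile arcs.
; Timed delays separate zero-gravity suspension, relaunch, and restoring input as the effect hides.
; GetNextLocation draws from a shrinking copy of LandingLocations, but selection and removal use separate random rolls, so spots can repeat.
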(event `self.ReceiveBeginPlay`
  (`NiagaraComponent.SetPaused` (`self.Whirlpool`) true)
  (`SceneComponent.SetVisibility` (`self.Whirlpool`) false false))

(event `LaunchPlayer`
  (params (Player :type "/Game/Characters/Piecelings/PiecelingBP Object Reference") (LandingLocation :type "Vector Structure"))
  (bind _tossvelocity (`GameplayStatics.BlueprintSuggestProjectileVelocity` (`self.K2_GetActorLocation` Player) LandingLocation (`self.Launch Speed`) 0.0 "DoNotTrace" 0.0 true))
  (`Character.LaunchCharacter` Player _tossvelocity true true))

(event `ActivateWhirlpool`
  (bind _whirlpool (`self.Whirlpool`))
  (bind _whirlpool_2 (`self.Whirlpool`))
  (`SceneComponent.SetVisibility` _whirlpool_2 true false)
  (`NiagaraComponent.SetPaused` _whirlpool_2 false)
  (bind _outactors (`GameplayStatics.GetAllActorsOfClass` "/Game/Characters/Piecelings/PiecelingBP.PiecelingBP_C"))
  (bind _output_get (set `self.Piecelings` _outactors))
  (for _array_element _output_get
    (`/Game/Characters/Piecelings/PiecelingBP.DropItem` _array_element)
    (`self.DisableInput` _array_element null)
    (`self.LaunchPlayer` _array_element (`SceneComponent.K2_GetComponentLocation` (`self.Center`))))
  (`KismetSystemLibrary.Delay` (`self.LaunchTime`))
  (for _array_element_2 (`self.Piecelings`)
    (bind _capsulecomponent (`Character.CapsuleComponent` _array_element_2))
    (`PrimitiveComponent.SetEnableGravity` _capsulecomponent false)
    (`PrimitiveComponent.SetAllPhysicsLinearVelocity` _capsulecomponent (0.0 0.0 0.0) false))
  (`KismetSystemLibrary.Delay` (`self.WhirlpoolTime`))
  (set `self.LandingLocationsMinusUsed` (`self.LandingLocations`))
  (for _array_element_3 (`self.Piecelings`)
    (`PrimitiveComponent.SetEnableGravity` (`Character.CapsuleComponent` _array_element_3) true)
    (`self.GetNextLocation`)
    (`self.LaunchPlayer` _array_element_3 (`self.SelectedLocation`)))
  (`KismetSystemLibrary.Delay` (`self.LaunchTime`))
  (for _array_element_4 (`self.Piecelings`)
    (`self.EnableInput` _array_element_4 (`GameplayStatics.GetPlayerController` (`/Game/Characters/Piecelings/PiecelingBP.Index` _array_element_4))))
  (`SceneComponent.SetVisibility` _whirlpool false false)
  (`NiagaraComponent.SetPaused` _whirlpool true))

(event `GetNextLocation`
  (bind _returnvalue (`KismetMathLibrary.RandomIntegerInRange` 0 (- (`KismetArrayLibrary.Array_Length` (`self.LandingLocationsMinusUsed`)) 1)))
  (set `self.SelectedLocation` (`|GetArrayItem` (`self.LandingLocationsMinusUsed`) _returnvalue))
  (`KismetArrayLibrary.Array_Remove` (`self.LandingLocationsMinusUsed`) _returnvalue))

(fn `UserConstructionScript`)