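; PufferFish is a placeable trap that patrols in a straight line and temporarily changes the speed of Piecelings it touches.
; Before activation it rotates in 90-degree yaw steps; activation locks in the mesh's forward direction and starts a lifespan timer that destroys it.
; Tick drives movement with MoveComponentTo, reversing direction after PathCollider overlaps any non-Pieceling.
; A separate PiecelingCollider calls ChangeSpeed on overlapping Piecelings.
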(event `self.ReceiveBeginPlay`)

(event `self.ActivatePlacedTrap`
  (set `self.SetDirection` (`KismetMathLibrary.GetForwardVector` (`SceneComponent.K2_GetComponentRotation` (`self.StaticMesh`))))
  (set `self.Active` true)
  (`KismetSystemLibrary.K2_SetTimerDelegate` (delegate `DeactivatePuffer`) (`self.Lifespan`)))

(event `DeactivatePuffer`
  (`self.K2_DestroyActor`))

(event `self.ReceiveTick`
  (params (DeltaSeconds :type "Float (single-precision)"))
  (if (`self.Active`)
    (if (`self.Collide`)
      (set `self.SetDirection` (* (`self.SetDirection`) -1.0))
      (set `self.Collide` false)
      (else
        (`KismetSystemLibrary.MoveComponentTo` (`self.StaticMesh`) (+ (* (`self.SetDirection`) (`self.Distance`)) (`SceneComponent.K2_GetComponentLocation` (`self.StaticMesh`))) (`SceneComponent.K2_GetComponentRotation` (`self.StaticMesh`)) false false (`self.TimeToEndPoint`))))))

(event `self.PathCollider.OnComponentBeginOverlap`
  (params (OverlappedComponent :type "PrimitiveComponent Object Reference") (OtherActor :type "Actor Object Reference") (OtherComp :type "PrimitiveComponent Object Reference") (OtherBodyIndex :type Integer) (bFromSweep :type Boolean) (SweepResult :type "HitResult Structure (by ref)"))
  (cast `/Game/Characters/Piecelings/PiecelingBP` OtherActor
    (:`CastFailed`
      (set `self.Collide` true))))

(event `self.PiecelingCollider.OnComponentBeginOverlap`
  (params (OverlappedComponent :type "PrimitiveComponent Object Reference") (OtherActor :type "Actor Object Reference") (OtherComp :type "PrimitiveComponent Object Reference") (OtherBodyIndex :type Integer) (bFromSweep :type Boolean) (SweepResult :type "HitResult Structure (by ref)"))
  (bind _aspieceling_bp (cast `/Game/Characters/Piecelings/PiecelingBP` OtherActor))
  (`/Game/Characters/Piecelings/PiecelingBP.ChangeSpeed` _aspieceling_bp (`self.NewPiecelingSpeed`) (`self.SpeedChangeDuration`)))

(event `self.RotateTrap`
  (bind _staticmesh (`self.StaticMesh`))
  (bind (_returnvalue_roll _returnvalue_pitch _returnvalue_yaw) (`KismetMathLibrary.BreakRotator` (`SceneComponent.K2_GetComponentRotation` _staticmesh)))
  (if (not (`self.Active`))
    (`SceneComponent.K2_SetWorldRotation` _staticmesh (`KismetMathLibrary.MakeRotator` _returnvalue_roll _returnvalue_pitch (+ _returnvalue_yaw 90.0)) false false)))

(fn `UserConstructionScript`)