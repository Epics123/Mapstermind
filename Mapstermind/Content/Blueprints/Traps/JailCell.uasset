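; JailCell is a placeable trap actor that imprisons overlapping Pieceling players for a set time.
; Once placed, Tick activates it, showing the cage, sliding it along Z with a timeline, and flagging players tracked by its collision component as Trapped.
; A timer then reverses the movement, clears Trapped on every Pieceling in the world, resets the road block's trap flag and color, and destroys the actor.
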(event `self.ReceiveBeginPlay`)

(event `self.ReceiveTick`
  (params (DeltaSeconds :type "Float (single-precision)"))
  (if (`self.Activated`)
    _
    (elif (`self.IsPlaced`)
      (set `self.Activated` true)
      (`self.ActivateJailCell`))))

(event `ActivateJailCell`
  ;[1 1 1] Activate Jail Cell
  (`SceneComponent.SetVisibility` (`self.JailCellMesh`) true false)
  (`PrimitiveComponent.SetCollisionEnabled` (`self.JailCellMesh`) "NoCollision")
  (`self.MoveJailCell`)
  (for _array_element (`self.OverlapingPlayers`)
    (set `/Game/Characters/Piecelings/PiecelingBP.Trapped` true _array_element))
  (`KismetSystemLibrary.K2_SetTimerDelegate` (delegate `FreeTrapedPlayers`) (`self.TrapTime`)))

(event `self.JailCellCollision.OnComponentBeginOverlap`
  (params (OverlappedComponent :type "PrimitiveComponent Object Reference") (OtherActor :type "Actor Object Reference") (OtherComp :type "PrimitiveComponent Object Reference") (OtherBodyIndex :type Integer) (bFromSweep :type Boolean) (SweepResult :type "HitResult Structure (by ref)"))
  (bind _aspieceling_bp (cast `/Game/Characters/Piecelings/PiecelingBP` OtherActor))
  (`KismetArrayLibrary.Array_Add` (`self.OverlapingPlayers`) _aspieceling_bp))

(event `self.JailCellCollision.OnComponentEndOverlap`
  (params (OverlappedComponent :type "PrimitiveComponent Object Reference") (OtherActor :type "Actor Object Reference") (OtherComp :type "PrimitiveComponent Object Reference") (OtherBodyIndex :type Integer))
  (bind _aspieceling_bp (cast `/Game/Characters/Piecelings/PiecelingBP` OtherActor))
  (`KismetArrayLibrary.Array_RemoveItem` (`self.OverlapingPlayers`) _aspieceling_bp))

(event `FreeTrapedPlayers`
  ;[1 1 1] Free Trapped Players
  (`self.ResetJailCellPosition`)
  (`PrimitiveComponent.SetCollisionEnabled` (`self.JailCellMesh`) "QueryAndPhysics")
  (bind _outactors (`GameplayStatics.GetAllActorsOfClass` "/Game/Characters/Piecelings/PiecelingBP.PiecelingBP_C"))
  (for _array_element _outactors
    (if (`/Game/Characters/Piecelings/PiecelingBP.Trapped` _array_element)
      (set `/Game/Characters/Piecelings/PiecelingBP.Trapped` false _array_element)))
  (`KismetSystemLibrary.Delay` 0.2)
  (`SceneComponent.SetVisibility` (`self.JailCellMesh`) false false)
  (`self.ResetRoadColor`)
  (`self.K2_DestroyActor`))

(event `MoveJailCell`
  (bind (_meshstartlocation_x _meshstartlocation_y _meshstartlocation_z) (`KismetMathLibrary.BreakVector` (`self.MeshStartLocation`)))
  (bind _jailcellmesh (`self.JailCellMesh`))
  (bind (_meshendlocation_x _meshendlocation_y _meshendlocation_z) (`KismetMathLibrary.BreakVector` (`self.MeshEndLocation`)))
  (bind (_relativelocation_x _relativelocation_y) (`KismetMathLibrary.BreakVector` (`SceneComponent.RelativeLocation` _jailcellmesh)))
  ;[1 1 1] Move Jail Cell Mesh
  (bind (_direction _interp) (`Timeline|JailCellMovement` :!via `PlayFromStart` :!label _label)
    (:`Update`
      (`SceneComponent.K2_SetRelativeLocation` _jailcellmesh (`KismetMathLibrary.MakeVector` _relativelocation_x _relativelocation_y (`KismetMathLibrary.Lerp` _meshstartlocation_z _meshendlocation_z _interp)) false false))
    (:`Finished`
      (`PrimitiveComponent.SetCollisionEnabled` (`self.JailCellMesh`) "QueryAndPhysics"))))

(event `ResetJailCellPosition`
  ;[1 1 1] Move Jail Cell Mesh
  (goto _label :!via `ReverseFromEnd`))

(fn `ResetRoadColor`
  (bind _road (`self.Road`))
  (set `Road.HasTrap` false _road)
  (bind _asnon_road_block (cast `/Game/Blueprints/Level/NonRoadBlock` _road))
  (bind _plane (`/Game/Blueprints/Level/NonRoadBlock.Plane` _asnon_road_block))
  (bind _returnvalue (`PrimitiveComponent.CreateDynamicMaterialInstance` _plane 0 "/Game/Materials/Environment/GrassMat2.GrassMat2" "None"))
  (`MaterialInstanceDynamic.SetVectorParameterValue` _returnvalue "Color" (struct :`R` 1.0 :`G` 1.0 :`B` 1.0 :`A` 1.0))
  (`PrimitiveComponent.SetMaterial` _plane 0 _returnvalue))

(fn `UserConstructionScript`
  (set `self.IsJailCell` true))