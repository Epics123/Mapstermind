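; Manhole trap placed on a road block that throws overlapping Pieceling players into the air when activated.
; A collider tracks the players on it, and ActivateManhole makes each drop their item, then launches them using a high-arc projectile velocity aimed back at their own location.
; The cover is swapped for a slippery mesh until a delay ends, then the road's trap flag and color are reset and the actor is destroyed.
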(event `self.ManholeCollider.OnComponentBeginOverlap`
  (params (OverlappedComponent :type "PrimitiveComponent Object Reference") (OtherActor :type "Actor Object Reference") (OtherComp :type "PrimitiveComponent Object Reference") (OtherBodyIndex :type Integer) (bFromSweep :type Boolean) (SweepResult :type "HitResult Structure (by ref)"))
  (bind _aspieceling_bp (cast `/Game/Characters/Piecelings/PiecelingBP` OtherActor))
  (`KismetArrayLibrary.Array_Add` (`self.OverlappingPlayers`) _aspieceling_bp))

(event `self.ManholeCollider.OnComponentEndOverlap`
  (params (OverlappedComponent :type "PrimitiveComponent Object Reference") (OtherActor :type "Actor Object Reference") (OtherComp :type "PrimitiveComponent Object Reference") (OtherBodyIndex :type Integer))
  (bind _aspieceling_bp (cast `/Game/Characters/Piecelings/PiecelingBP` OtherActor))
  (`KismetArrayLibrary.Array_RemoveItem` (`self.OverlappingPlayers`) _aspieceling_bp))

(event `ActivateManhole`
  (bind _slipperymesh (`self.SlipperyMesh`))
  (for _array_element (`self.OverlappingPlayers`)
    (`/Game/Characters/Piecelings/PiecelingBP.DropItem` _array_element)
    (bind _returnvalue (`self.K2_GetActorLocation` _array_element))
    (bind _tossvelocity (`GameplayStatics.BlueprintSuggestProjectileVelocity` _returnvalue _returnvalue 2500.0 0.0 "DoNotTrace" 0.0 true))
    (bind _output_get (set `self.LaunchVelocity` _tossvelocity))
    (`Character.LaunchCharacter` _array_element _output_get true true))
  (`PrimitiveComponent.SetCollisionEnabled` (`self.ManholeCoverMesh`) "NoCollision")
  (`SceneComponent.SetVisibility` _slipperymesh true false)
  (`PrimitiveComponent.SetCollisionEnabled` _slipperymesh "QueryAndPhysics")
  (`SceneComponent.SetVisibility` (`self.ManholeCoverMesh`) false false)
  (`KismetSystemLibrary.Delay` (`self.SlipperyTime`))
  (`self.ResetRoadColor`)
  (`self.K2_DestroyActor`))

(fn `ResetRoadColor`
  (bind _road (`self.Road`))
  (set `Road.HasTrap` false _road)
  (bind _asgrass_block_trap (cast `/Game/Blueprints/Level/GrassBlockTrap` _road))
  (bind _blankblock_v2 (`/Game/Blueprints/Level/GrassBlockTrap.blankBlock_V2` _asgrass_block_trap))
  (bind _returnvalue (`PrimitiveComponent.CreateDynamicMaterialInstance` _blankblock_v2 0 "/Game/ArtAssets/LevelCity/Environment/OldMat/GrassMat.GrassMat" "None"))
  (`MaterialInstanceDynamic.SetVectorParameterValue` _returnvalue "Color" (struct :`R` 1.0 :`G` 1.0 :`B` 1.0 :`A` 1.0))
  (`PrimitiveComponent.SetMaterial` _blankblock_v2 0 _returnvalue))

(fn `UserConstructionScript`)