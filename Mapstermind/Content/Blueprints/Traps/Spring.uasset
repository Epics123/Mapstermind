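; Spring trap that launches PiecelingBP characters standing on it toward a landing location.
; Box overlap events keep a list of the Piecelings inside.
; ActivateSpring briefly shows the spring mesh and launches each listed character, using a suggested high-arc projectile velocity to override its movement.
; The construction script marks the actor as not a jail cell.
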(event `ActivateSpring`
  (`SceneComponent.SetVisibility` (`self.SpringMesh`) true false)
  (for _array_element (`self.OverlapingPlayers`)
    (bind _tossvelocity (`GameplayStatics.BlueprintSuggestProjectileVelocity` (`self.K2_GetActorLocation` _array_element) (`self.LandingLocation`) 2500.0 0.0 "DoNotTrace" 0.0 true))
    (set `self.LaunchVelocity` _tossvelocity)
    (`Character.LaunchCharacter` _array_element (`self.LaunchVelocity`) true true))
  (`KismetSystemLibrary.Delay` 2.0)
  (`SceneComponent.SetVisibility` (`self.SpringMesh`) false false))

(event `self.Box.OnComponentBeginOverlap`
  (params (OverlappedComponent :type "PrimitiveComponent Object Reference") (OtherActor :type "Actor Object Reference") (OtherComp :type "PrimitiveComponent Object Reference") (OtherBodyIndex :type Integer) (bFromSweep :type Boolean) (SweepResult :type "HitResult Structure (by ref)"))
  (bind _aspieceling_bp (cast `/Game/Characters/Piecelings/PiecelingBP` OtherActor))
  (`KismetArrayLibrary.Array_Add` (`self.OverlapingPlayers`) _aspieceling_bp))

(event `self.Box.OnComponentEndOverlap`
  (params (OverlappedComponent :type "PrimitiveComponent Object Reference") (OtherActor :type "Actor Object Reference") (OtherComp :type "PrimitiveComponent Object Reference") (OtherBodyIndex :type Integer))
  (bind _aspieceling_bp (cast `/Game/Characters/Piecelings/PiecelingBP` OtherActor))
  (`KismetArrayLibrary.Array_RemoveItem` (`self.OverlapingPlayers`) _aspieceling_bp))

(fn `UserConstructionScript`
  (set `self.IsJailCell` false))