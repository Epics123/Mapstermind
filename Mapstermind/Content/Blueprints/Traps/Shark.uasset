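; Shark trap that, once activated, patrols a track spline by timeline until its lifespan ends, then turns off looping and resets to sleeping.
; Overlapping a Pieceling pauses the patrol at its saved path offset and starts a short attack cooldown.
; The attack lobs the Pieceling toward a knockback location on a high arc, drops its item and briefly disables its input before the patrol resumes.
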(event `self.ReceiveTick`
  (params (DeltaSeconds :type "Float (single-precision)")))

(event `self.ReceiveBeginPlay`)

(event `self.ActivatePlacedTrap`
  (set `self.Sleeping` false)
  (`self.Move`)
  (`KismetSystemLibrary.Delay` (`self.Lifespan`))
  (`self.ReturnToShip`))

(event `Move`
  (bind _sharkspline (`/Game/Blueprints/Traps/SharkTrack.SharkSpline` (`self.TrackRef`)))
  (bind _returnvalue (`KismetMathLibrary.Lerp` 0.0 (`SplineComponent.GetSplineLength` _sharkspline) (`self.Alpha`)))
  (if (`self.Attacking`)
    (`self.Stop`)
    (else
      (`TimelineComponent.SetPlayRate` (`self.SharkTL`) (/ 1.0 (`self.Speed`)))
      (`TimelineComponent.SetNewTime` (`self.SharkTL`) (`self.PathOffset`))
      (bind (_direction _alpha) (`Timeline|SharkTL` :!label _label)
        (:`Update`
          (set `self.Alpha` _alpha)
          (`self.K2_SetActorLocationAndRotation` (`SplineComponent.GetLocationAtDistanceAlongSpline` _sharkspline _returnvalue "World") (`SplineComponent.GetRotationAtDistanceAlongSpline` _sharkspline _returnvalue "World")))))))

(event `Stop`
  (set `self.PathOffset` (`self.Alpha`))
  (goto _label :!via `Stop`))

(event `Attack`
  (params (Pieceling :type "/Game/Characters/Piecelings/PiecelingBP Object Reference"))
  (bind _tossvelocity (`GameplayStatics.BlueprintSuggestProjectileVelocity` (`self.K2_GetActorLocation` Pieceling) (`self.KockBackLocation`) (`self.LaunchSpeed`) 0.0 "DoNotTrace" 0.0 true))
  (`Character.LaunchCharacter` Pieceling _tossvelocity true true)
  (`/Game/Characters/Piecelings/PiecelingBP.DropItem` Pieceling)
  (`self.DisableInput` Pieceling null)
  (`KismetSystemLibrary.Delay` 2.0)
  (set `self.Attacking` false)
  (`self.Move`)
  (`self.EnableInput` Pieceling null))

(event `self.PiecelingCollider.OnComponentBeginOverlap`
  (params (OverlappedComponent :type "PrimitiveComponent Object Reference") (OtherActor :type "Actor Object Reference") (OtherComp :type "PrimitiveComponent Object Reference") (OtherBodyIndex :type Integer) (bFromSweep :type Boolean) (SweepResult :type "HitResult Structure (by ref)"))
  (if (not (`self.AttackCooldown`))
    (bind _aspieceling_bp (cast `/Game/Characters/Piecelings/PiecelingBP` OtherActor))
    (set `self.AttackCooldown` true)
    (set `self.Attacking` true)
    (`self.Move`)
    (`self.Attack` _aspieceling_bp)
    (`KismetSystemLibrary.Delay` 2.0)
    (set `self.AttackCooldown` false)))

(event `ReturnToShip`
  (`TimelineComponent.SetLooping` (`self.SharkTL`) false)
  (set `self.Sleeping` true)
  (set `self.Alpha` 0.0)
  (set `self.PathOffset` 0.0))

(fn `LifespanTimer`)

(fn `UserConstructionScript`)