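; Clamlings is a placeable trap that reverses the controls of a PiecelingBP that overlaps its path collider.
; When mobile, activation starts it moving along its facing via Tick, flipping direction on a collide flag; it can be rotated in quarter turns while inactive.
; On a hit it destroys the collider, and while active it stays snapped to the victim.
; A timer started on mobile activation or hit destroys it.
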(event `self.ReceiveBeginPlay`)

(event `StartLifespan`
  ;[1 0.6954 0.1875] Placed in World
  (`KismetSystemLibrary.K2_SetTimerDelegate` (delegate `DeactivateClamlings`) (`self.Duration`) :!label _label))

(event `self.PathCollider.OnComponentBeginOverlap`
  (params (OverlappedComponent :type "PrimitiveComponent Object Reference") (OtherActor :type "Actor Object Reference") (OtherComp :type "PrimitiveComponent Object Reference") (OtherBodyIndex :type Integer) (bFromSweep :type Boolean) (SweepResult :type "HitResult Structure (by ref)"))
  (bind _aspieceling_bp (cast `/Game/Characters/Piecelings/PiecelingBP` OtherActor))
  (set `self.PlayerRef` _aspieceling_bp)
  (`/Game/Characters/Piecelings/PiecelingBP.ReverseControls` _aspieceling_bp (`self.Time`))
  (set `self.Attached` true)
  (`ActorComponent.K2_DestroyComponent` (`self.PathCollider`))
  (`self.StartLifespan`))

(event `self.ActivatePlacedTrap`
  ;[1 0.6954 0.1875] Placed in World
  (if (`self.Mobile`)
    (set `self.SetDirection` (`KismetMathLibrary.GetForwardVector` (`SceneComponent.K2_GetComponentRotation` (`self.StaticMesh`))))
    (set `self.Active` true)
    (goto _label)))

(event `DeactivateClamlings`
  ;[1 0.6954 0.1875] Placed in World
  (`self.K2_DestroyActor`))

(event `self.ReceiveTick`
  (params (DeltaSeconds :type "Float (single-precision)"))
  (bind _staticmesh (`self.StaticMesh`))
  ;[1 0.6954 0.1875] Placed in World
  (if (`self.Active`)
    (if (`self.Collide`)
      (set `self.SetDirection` (* (`self.SetDirection`) -1.0))
      (set `self.Collide` false)
      (elif (`self.Attached`)
        (`self.K2_AttachToActor` (`self.PlayerRef`) "None" "SnapToTarget" "KeepRelative" "KeepRelative")
        (`SceneComponent.K2_SetRelativeLocation` (`self.StaticMesh`) (0.0 0.0 0.0) false false)
        (elif (`self.Mobile`)
          (`KismetSystemLibrary.MoveComponentTo` (`self.StaticMesh`) (+ (* (`self.SetDirection`) (`self.Distance`)) (`SceneComponent.K2_GetComponentLocation` _staticmesh)) (`SceneComponent.K2_GetComponentRotation` _staticmesh) false false (/ 1.0 (`self.Speed`))))))))

(event `self.RotateTrap`
  (bind _staticmesh (`self.StaticMesh`))
  (bind (_returnvalue_roll _returnvalue_pitch _returnvalue_yaw) (`KismetMathLibrary.BreakRotator` (`SceneComponent.K2_GetComponentRotation` _staticmesh)))
  ;[1 0.6954 0.1875] Placed in World
  (if (not (`self.Active`))
    (`SceneComponent.K2_SetWorldRotation` _staticmesh (`KismetMathLibrary.MakeRotator` _returnvalue_roll _returnvalue_pitch (+ _returnvalue_yaw 90.0)) false false)))

(fn `UserConstructionScript`)