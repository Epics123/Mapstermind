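; Bulldozer trap that, once placed, drives along its right vector for a limited time and tosses any Pieceling it contacts.
; Tick snaps the capsule above the root once, reveals the mesh, sets physics velocity and counts down to self-destruction.
; Hit and overlap launch Piecelings using a high-arc projectile velocity with identical start and end points.
; Overlap also makes them drop their item and briefly disables their input.
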(event `self.ReceiveTick`
  (params (DeltaSeconds :type "Float (single-precision)"))
  (if (<= (`self.Timer`) 0.0)
    (`self.K2_DestroyActor`)
    (elif (`self.IsPlaced`)
      (if (`self.Set Location`)
        (`SceneComponent.K2_SetWorldLocation` (`self.Capsule`) (+ (`SceneComponent.K2_GetComponentLocation` (`self.DefaultSceneRoot`)) (0.0 0.0 100.0)) false false)
        (set `self.Set Location` false))
      (if (not (`SceneComponent.IsVisible` (`self.StaticMesh`)))
        (`SceneComponent.SetVisibility` (`self.StaticMesh`) true false))
      (set `self.Timer` (- (`self.Timer`) DeltaSeconds))
      (`PrimitiveComponent.SetPhysicsLinearVelocity` (`self.Capsule`) (* (`KismetMathLibrary.Vector_Right`) (`self.MovementSpeed`)) false "None"))))

(event `Destroy`
  (`self.K2_DestroyActor`))

(event `self.ReceiveHit`
  (params (MyComp :type "PrimitiveComponent Object Reference") (Other :type "Actor Object Reference") (OtherComp :type "PrimitiveComponent Object Reference") (bSelfMoved :type Boolean) (HitLocation :type "Vector Structure") (HitNormal :type "Vector Structure") (NormalImpulse :type "Vector Structure") (Hit :type "HitResult Structure (by ref)"))
  (if (`self.IsPlaced`)
    (bind _aspieceling_bp (cast `/Game/Characters/Piecelings/PiecelingBP` Other))
    (bind _returnvalue (`self.K2_GetActorLocation` _aspieceling_bp))
    (bind _tossvelocity (`GameplayStatics.BlueprintSuggestProjectileVelocity` _returnvalue _returnvalue (`self.LaunchSpeed`) 0.0 "DoNotTrace" 0.0 true))
    (`Character.LaunchCharacter` _aspieceling_bp _tossvelocity true true)))

(event `self.ReceiveActorBeginOverlap`
  (params (OtherActor :type "Actor Object Reference"))
  (if (`self.IsPlaced`)
    (bind _aspieceling_bp (cast `/Game/Characters/Piecelings/PiecelingBP` OtherActor))
    (bind _returnvalue (`self.K2_GetActorLocation` _aspieceling_bp))
    (bind _tossvelocity (`GameplayStatics.BlueprintSuggestProjectileVelocity` _returnvalue _returnvalue (`self.LaunchSpeed`) 0.0 "DoNotTrace" 0.0 true))
    (`Character.LaunchCharacter` _aspieceling_bp _tossvelocity true true)
    (`/Game/Characters/Piecelings/PiecelingBP.DropItem` _aspieceling_bp)
    (`self.DisableInput` _aspieceling_bp null)
    (`KismetSystemLibrary.Delay` 2.0)
    (`self.EnableInput` _aspieceling_bp null)))

(fn `UserConstructionScript`)