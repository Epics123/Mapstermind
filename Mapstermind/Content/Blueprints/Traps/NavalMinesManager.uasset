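; NavalMinesManager is a trap actor that deploys a group of naval mines and owns their cleanup.
; On BeginPlay, ActivateMines re-calls itself after a short Delay to spawn mines one by one, standing in for a loop.
; Each mine gets a manager reference, attaches below its preset relative location and is told to rise to it.
; DestroyMines removes all mines and the manager; the duration-based self-destruct is unconnected.
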(event `self.ReceiveBeginPlay`
  (`self.ActivateMines`))

(event `self.ReceiveDestroyed`)

(event `self.ActivatePlacedTrap`)

(event `Start Timer`)

(event `ActivateMines`
  (bind _count (`self.Count`))
  (if (>= (`self.Quantity`) (`self.Count`))
    (`self.SpawnMine` _count)
    (`/Engine/EditorBlueprintResources/StandardMacros.IncrementInt` _count
      (:`  `
        (`KismetSystemLibrary.Delay` 0.5) ; couldn't do loop because delay
        (`self.ActivateMines`)))))

(event `SpawnMine`
  (params (ind :type Integer))
  (bind (_output_x _output_y _output_z) (`KismetMathLibrary.BreakVector` (`|GetArrayItem` (`self.Locations`) ind)))
  (bind _returnvalue (`|SpawnActorFromClass` "/Game/Blueprints/Traps/NavalMine.NavalMine_C" (`KismetMathLibrary.MakeTransform` (0.0 0.0 0.0)) "DontSpawnIfColliding" "OverrideRootScale" null null))
  (`KismetArrayLibrary.Array_Add` (`self.Mines`) _returnvalue)
  (set `/Game/Blueprints/Traps/NavalMine.Manager` self _returnvalue)
  (`self.K2_AttachToActor` _returnvalue self "None" "KeepRelative" "KeepRelative" "KeepRelative" true)
  (`self.K2_SetActorRelativeLocation` _returnvalue (`KismetMathLibrary.MakeVector` _output_x _output_y -850.0) false false)
  (`/Game/Blueprints/Traps/NavalMine.Rise` _returnvalue (`KismetMathLibrary.MakeVector` _output_x _output_y _output_z)))

(event `DestroyMines`
  (for _array_element (`self.Mines`)
    (`self.K2_DestroyActor` _array_element))
  (`self.K2_DestroyActor`))

(fn `UserConstructionScript`)