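; Trap spawn point that places one trap of a chosen type, replacing any existing one.
; SpawnTrap, gated by CanSpawn (off at start in TutorialScene), spawns the trap showing only its hidden-state mesh, with effects and optional tutorial cards.
; Reset hides that mesh, restores some real meshes, then releases the reference and returns the type, with no Bulldozer case.
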(event `self.ReceiveBeginPlay`
  (bind _returnvalue (`GameplayStatics.GetCurrentLevelName` true))
  (if (`KismetStringLibrary.EqualEqual_StrStr` _returnvalue "TutorialScene")
    (`GameplayStatics.GetActorOfClass` "/Game/Blueprints/Tutorial/TutorialController.TutorialController_C")
    (set `self.CanSpawn` false)
    (else
      (`GameplayStatics.GetActorOfClass` "/Game/Blueprints/Tutorial/TutorialController.TutorialController_C")
      (set `self.CanSpawn` true))))

(event `SpawnTrap`
  (params (TrapType :type "/Game/Blueprints/Traps/TrapTypes Enum" :default "NewEnumerator5"))
  (bind _trap (`self.Trap`))
  (for _array_element (`self.TrapCards`)
    (`self.SetActorHiddenInGame` _array_element true))
  (if (`self.CanSpawn`)
    (`GameplayStatics.PlaySoundAtLocation` "/Game/Audio/SoundEffects/WoodenBat2.WoodenBat2" (0.0 0.0 0.0) (struct) 0.5 1.0 0.0 null null null)
    (set `self.TrapType` TrapType)
    (`/Engine/EditorBlueprintResources/StandardMacros.IsValid` _trap
      (:`Is Valid`
        (`self.K2_DestroyActor` _trap)
        (set `self.Trap` null))
      (:`Is Not Valid`
        _))
    (switch `/Game/Blueprints/Traps/TrapTypes` (`self.TrapType`)
      (:`NewEnumerator0`
        (bind _returnvalue (`|SpawnActorFromClass` "/Game/Blueprints/Traps/JailCell.JailCell_C" (`KismetMathLibrary.MakeTransform` (`self.K2_GetActorLocation`)) "Undefined" "OverrideRootScale" null null))
        (`SceneComponent.SetVisibility` (`/Game/Blueprints/Traps/JailCell.JailCellMesh` _returnvalue) false false)
        (`SceneComponent.SetVisibility` (`/Game/Blueprints/Traps/JailCell.HiddenMesh` _returnvalue) true false)
        (set `self.Trap` _returnvalue)
        (if (`self.IsTutorial`)
          (`self.SetActorHiddenInGame` (`|GetArrayItem` (`self.TrapCards`)) false)))
      (:`NewEnumerator2`
        (bind _returnvalue_2 (`|SpawnActorFromClass` "/Game/Blueprints/Traps/RoadBlock.RoadBlock_C" (`KismetMathLibrary.MakeTransform` (`self.K2_GetActorLocation`)) "Undefined" "OverrideRootScale" null null))
        (`SceneComponent.SetVisibility` (`/Game/Blueprints/Traps/RoadBlock.StaticMesh` _returnvalue_2) false true)
        (`SceneComponent.SetVisibility` (`/Game/Blueprints/Traps/RoadBlock.HiddenMesh` _returnvalue_2) true false)
        (set `self.Trap` _returnvalue_2)
        (if (`self.IsTutorial`)
          (`self.SetActorHiddenInGame` (`|GetArrayItem` (`self.TrapCards`) 1) false)))
      (:`NewEnumerator3`
        (bind _returnvalue_3 (`|SpawnActorFromClass` "/Game/Blueprints/Traps/FakeTrap.FakeTrap_C" (`KismetMathLibrary.MakeTransform` (`self.K2_GetActorLocation`)) "Undefined" "OverrideRootScale" null null))
        (`SceneComponent.SetVisibility` (`/Game/Blueprints/Traps/FakeTrap.HiddenMesh` _returnvalue_3) true false)
        (set `self.Trap` _returnvalue_3)
        (if (`self.IsTutorial`)
          (`self.SetActorHiddenInGame` (`|GetArrayItem` (`self.TrapCards`) 2) false)))
      (:`NewEnumerator4`
        (bind _returnvalue_4 (`|SpawnActorFromClass` "/Game/Blueprints/Traps/Spring.Spring_C" (`KismetMathLibrary.MakeTransform` (`self.K2_GetActorLocation`)) "Undefined" "OverrideRootScale" null (0.0 0.0 0.0) null))
        (`SceneComponent.SetVisibility` (`/Game/Blueprints/Traps/Spring.SpringMesh` _returnvalue_4) false false)
        (`SceneComponent.SetVisibility` (`/Game/Blueprints/Traps/Spring.HiddenMesh` _returnvalue_4) true false)
        (set `self.Trap` _returnvalue_4)
        (if (`self.IsTutorial`)
          (`self.SetActorHiddenInGame` (`|GetArrayItem` (`self.TrapCards`) 3) false)))
      (:`NewEnumerator6`
        (bind _returnvalue_5 (`|SpawnActorFromClass` "/Game/Blueprints/Traps/Bulldozer.Bulldozer_C" (`KismetMathLibrary.MakeTransform` (`self.K2_GetActorLocation`)) "Undefined" "OverrideRootScale" null null))
        (`SceneComponent.SetVisibility` (`/Game/Blueprints/Traps/Bulldozer.StaticMesh` _returnvalue_5) false false)
        (`SceneComponent.SetVisibility` (`/Game/Blueprints/Traps/Bulldozer.HiddenMesh` _returnvalue_5) true false)
        (set `self.Trap` _returnvalue_5)
        (if (`self.IsTutorial`)
          (`self.SetActorHiddenInGame` (`|GetArrayItem` (`self.TrapCards`) 2) false)))
      (:`NewEnumerator7`
        (bind _returnvalue_6 (`|SpawnActorFromClass` "/Game/Blueprints/Traps/Manhole.Manhole_C" (`KismetMathLibrary.MakeTransform` (- (`self.K2_GetActorLocation`) (0.0 0.0 100.0))) "Undefined" "OverrideRootScale" null null))
        (`SceneComponent.SetVisibility` (`/Game/Blueprints/Traps/Manhole.ManholeCoverMesh` _returnvalue_6) false false)
        (`SceneComponent.SetVisibility` (`/Game/Blueprints/Traps/Manhole.HiddenMesh` _returnvalue_6) true false)
        (set `self.Trap` _returnvalue_6)
        (if (`self.IsTutorial`)
          (`self.SetActorHiddenInGame` (`|GetArrayItem` (`self.TrapCards`) 3) false))))
    (`GameplayStatics.SpawnEmitterAtLocation` "/Game/ParticleSystems/TrapSpawn.TrapSpawn" (`self.K2_GetActorLocation` (`self.Trap`)))))

(fn `Reset`
  (returns (Type :type "/Game/Blueprints/Traps/TrapTypes Enum"))
  (switch `/Game/Blueprints/Traps/TrapTypes` (`self.TrapType`)
    (:`NewEnumerator0`
      (bind _asjail_cell (cast `/Game/Blueprints/Traps/JailCell` (`self.Trap`)))
      (`self.ResetTrapVisibility` (`/Game/Blueprints/Traps/JailCell.HiddenMesh` _asjail_cell)))
    (:`NewEnumerator2`
      (bind _asroad_block (cast `/Game/Blueprints/Traps/RoadBlock` (`self.Trap`)))
      (`self.ResetTrapVisibility` (`/Game/Blueprints/Traps/RoadBlock.HiddenMesh` _asroad_block) (`/Game/Blueprints/Traps/RoadBlock.StaticMesh` _asroad_block)))
    (:`NewEnumerator3`
      (bind _asfake_trap (cast `/Game/Blueprints/Traps/FakeTrap` (`self.Trap`)))
      (bind _hiddenmesh (`/Game/Blueprints/Traps/FakeTrap.HiddenMesh` _asfake_trap))
      (`self.ResetTrapVisibility` _hiddenmesh)
      (`PrimitiveComponent.SetCollisionEnabled` _hiddenmesh "NoCollision"))
    (:`NewEnumerator4`
      (bind _asspring (cast `/Game/Blueprints/Traps/Spring` (`self.Trap`)))
      (`self.ResetTrapVisibility` (`/Game/Blueprints/Traps/Spring.HiddenMesh` _asspring)))
    (:`NewEnumerator7`
      (bind _asmanhole (cast `/Game/Blueprints/Traps/Manhole` (`self.Trap`)))
      (`self.ResetTrapVisibility` (`/Game/Blueprints/Traps/Manhole.HiddenMesh` _asmanhole) (`/Game/Blueprints/Traps/Manhole.ManholeCoverMesh` _asmanhole))))
  (set `self.Trap` null)
  (return (`self.TrapType`)))

(fn `ResetTrapVisibility`
  (params (HideMesh :type "StaticMeshComponent Object Reference") (ShowMesh :type "StaticMeshComponent Object Reference"))
  (`/Engine/EditorBlueprintResources/StandardMacros.IsValid` HideMesh
    (:`Is Valid`
      (`SceneComponent.SetVisibility` HideMesh false true)
      (`/Engine/EditorBlueprintResources/StandardMacros.IsValid` ShowMesh
        (:`Is Valid`
          (`SceneComponent.SetVisibility` ShowMesh true true))))))

(fn `UserConstructionScript`)