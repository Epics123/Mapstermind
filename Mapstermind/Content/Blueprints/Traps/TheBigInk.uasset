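; TheBigInk is a trap actor that creates a temporary ink area hiding the skeletal meshes of Piecelings entering it.
; ActivateInk spawns the ink particle effect, resizes the box horizontally to the ink radius, sets Active, then calls DeactivateInk after the lifetime delay.
; Box begin overlap hides a Pieceling only while Active, and end overlap shows it again.
; DeactivateInk destroys the effect and restores visibility for Piecelings still overlapping.
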(event `ActivateInk`
  (bind _inkradius (`self.InkRadius`))
  (bind _box (`self.Box`))
  (bind (_boxextent_x _boxextent_y _boxextent_z) (`KismetMathLibrary.BreakVector` (`BoxComponent.BoxExtent` _box)))
  (bind _returnvalue (`GameplayStatics.SpawnEmitterAtLocation` "/Game/ParticleSystems/InkPS.InkPS" (`self.K2_GetActorLocation`)))
  (set `self.InkPS` _returnvalue)
  (`BoxComponent.SetBoxExtent` _box (`KismetMathLibrary.MakeVector` _inkradius _inkradius _boxextent_z) true)
  (set `self.Active` true)
  (`KismetSystemLibrary.Delay` (`self.InkLifetime`))
  (`self.DeactivateInk`))

(event `DeactivateInk`
  (`ActorComponent.K2_DestroyComponent` (`self.InkPS`))
  (set `self.Active` false)
  (for _array_element (`self.GetOverlappingActors` "/Game/Characters/Piecelings/PiecelingBP.PiecelingBP_C")
    (bind _aspieceling_bp (cast `/Game/Characters/Piecelings/PiecelingBP` _array_element))
    (`SceneComponent.SetVisibility` (`/Game/Characters/Piecelings/PiecelingBP.SkeletalMesh` _aspieceling_bp) true false)))

(event `self.Box.OnComponentBeginOverlap`
  (params (OverlappedComponent :type "PrimitiveComponent Object Reference") (OtherActor :type "Actor Object Reference") (OtherComp :type "PrimitiveComponent Object Reference") (OtherBodyIndex :type Integer) (bFromSweep :type Boolean) (SweepResult :type "HitResult Structure (by ref)"))
  (bind _aspieceling_bp (cast `/Game/Characters/Piecelings/PiecelingBP` OtherActor))
  (if (`self.Active`)
    (`SceneComponent.SetVisibility` (`/Game/Characters/Piecelings/PiecelingBP.SkeletalMesh` _aspieceling_bp) false false)))

(event `self.Box.OnComponentEndOverlap`
  (params (OverlappedComponent :type "PrimitiveComponent Object Reference") (OtherActor :type "Actor Object Reference") (OtherComp :type "PrimitiveComponent Object Reference") (OtherBodyIndex :type Integer))
  (bind _aspieceling_bp (cast `/Game/Characters/Piecelings/PiecelingBP` OtherActor))
  (`SceneComponent.SetVisibility` (`/Game/Characters/Piecelings/PiecelingBP.SkeletalMesh` _aspieceling_bp) true false))

(fn `UserConstructionScript`)