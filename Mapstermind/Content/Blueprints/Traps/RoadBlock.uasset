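; RoadBlock is a timed trap on a road tile that slows any PiecelingBP entering its box.
; Overlap calls ChangeSpeed with the slow speed and timer duration, while leaving restores a hard-coded walk speed.
; StartTimer waits, resets the tile through HandBP, then destroys the actor.
; Both expiry and destruction set HandBP's right trap count to one and free the tile, with destruction also resetting its material color.
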(event `Start Timer`
  (bind _road (`self.Road`))
  (`KismetSystemLibrary.Delay` (`self.Timer`))
  (bind _returnvalue (`GameplayStatics.GetActorOfClass` "/Game/Characters/Mapster/HandBP.HandBP_C"))
  (set `/Game/Characters/Mapster/HandBP.RightTrapCount` 1 _returnvalue)
  (set `Road.HasTrap` false _road)
  (`/Game/Characters/Mapster/HandBP.ResetTile` _returnvalue _road false)
  (`self.K2_DestroyActor`))

(event `self.ReceiveDestroyed`
  (bind _returnvalue (`GameplayStatics.GetActorOfClass` "/Game/Characters/Mapster/HandBP.HandBP_C"))
  (set `/Game/Characters/Mapster/HandBP.RightTrapCount` 1 _returnvalue)
  (`self.ResetRoadColor`))

(event `self.Box.OnComponentBeginOverlap`
  (params (OverlappedComponent :type "PrimitiveComponent Object Reference") (OtherActor :type "Actor Object Reference") (OtherComp :type "PrimitiveComponent Object Reference") (OtherBodyIndex :type Integer) (bFromSweep :type Boolean) (SweepResult :type "HitResult Structure (by ref)"))
  (bind _aspieceling_bp (cast `/Game/Characters/Piecelings/PiecelingBP` OtherActor))
  (`/Game/Characters/Piecelings/PiecelingBP.ChangeSpeed` _aspieceling_bp (`self.SlowSpeed`) (`self.Timer`)))

(event `self.Box.OnComponentEndOverlap`
  (params (OverlappedComponent :type "PrimitiveComponent Object Reference") (OtherActor :type "Actor Object Reference") (OtherComp :type "PrimitiveComponent Object Reference") (OtherBodyIndex :type Integer))
  (bind _aspieceling_bp (cast `/Game/Characters/Piecelings/PiecelingBP` OtherActor))
  (set `CharacterMovementComponent.MaxWalkSpeed` 800.0 (`Character.CharacterMovement` _aspieceling_bp)))

(fn `ResetRoadColor`
  (bind _road (`self.Road`))
  (`/Engine/EditorBlueprintResources/StandardMacros.IsValid` _road
    (:`Is Valid`
      (set `Road.HasTrap` false _road)
      (bind _asgrass_block_trap (cast `/Game/Blueprints/Level/GrassBlockTrap` _road))
      (bind _blankblock_v2 (`/Game/Blueprints/Level/GrassBlockTrap.blankBlock_V2` _asgrass_block_trap))
      (bind _returnvalue (`PrimitiveComponent.CreateDynamicMaterialInstance` _blankblock_v2 0 "/Game/ArtAssets/LevelCity/Environment/OldMat/GrassMat.GrassMat" "None"))
      (`MaterialInstanceDynamic.SetVectorParameterValue` _returnvalue "Color" (struct :`R` 1.0 :`G` 1.0 :`B` 1.0 :`A` 1.0))
      (`PrimitiveComponent.SetMaterial` _blankblock_v2 0 _returnvalue))))

(fn `UserConstructionScript`)