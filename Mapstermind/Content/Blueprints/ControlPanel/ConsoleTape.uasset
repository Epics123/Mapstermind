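; ConsoleTape is a control panel label actor that shows a Description text on a ConsoleTapeWidget_V1 widget component.
; On BeginPlay it casts the component's widget and sets its Description text from the actor's Description variable.
; The UpdateTapeDescription event repeats the same write so the label can be refreshed after the variable changes.
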(event `self.ReceiveBeginPlay`
  (bind _asconsole_tape_widget_v1 (cast `/Game/Blueprints/Widgets/Level/ConsoleTapeWidget_V1` (`WidgetComponent.GetWidget` (`self.Widget`))))
  (`TextBlock.SetText` (`/Game/Blueprints/Widgets/Level/ConsoleTapeWidget_V1.Description` _asconsole_tape_widget_v1) (`self.Description`)))

(event `UpdateTapeDescription`
  (bind _asconsole_tape_widget_v1 (cast `/Game/Blueprints/Widgets/Level/ConsoleTapeWidget_V1` (`WidgetComponent.GetWidget` (`self.Widget`))))
  (`TextBlock.SetText` (`/Game/Blueprints/Widgets/Level/ConsoleTapeWidget_V1.Description` _asconsole_tape_widget_v1) (`self.Description`)))

(fn `UserConstructionScript`)