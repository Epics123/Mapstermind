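; VR control panel button that activates every placed Manhole in the level when pressed by a hand.
; Hand overlap drives a custom-depth highlight, with stencil values distinguishing ready, unavailable and pressed states.
; ActivateButton checks the left or right press and readiness, then after a delay triggers the manholes, animation and sound before resetting on cooldown.
; In tutorial mode, a press can advance the TutorialController's console check once.
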(event `self.ReceiveBeginPlay`
  (bind _outactors (`GameplayStatics.GetAllActorsOfClass` "/Game/Blueprints/Traps/Manhole.Manhole_C"))
  (set `self.Manholes` _outactors)
  (bind _returnvalue (`GameplayStatics.GetActorOfClass` "/Game/Blueprints/Tutorial/TutorialController.TutorialController_C"))
  (set `self.TutorialController` _returnvalue))

(event `self.ReceiveTick`
  (params (DeltaSeconds :type "Float (single-precision)"))
  (if (`self.Hovered`)
    (`PrimitiveComponent.SetRenderCustomDepth` (`self.SkeletalMesh`) true)
    (if (`self.CanActivate`)
      (`PrimitiveComponent.SetCustomDepthStencilValue` (`self.SkeletalMesh`) 1)
      (goto _label :!via `Reset`)
      (else
        (`PrimitiveComponent.SetCustomDepthStencilValue` (`self.SkeletalMesh`) 0)
        (goto _label :!via `Reset`)))
    (else
      (`/Engine/EditorBlueprintResources/StandardMacros.DoOnce` false :!label _label
        (:`Completed`
          (`PrimitiveComponent.SetRenderCustomDepth` (`self.SkeletalMesh`) false))))))

(event `self.ActivateButton`
  (params (Hand :type "Character Object Reference") (isLeft :type Boolean))
  (`/Engine/EditorBlueprintResources/StandardMacros.IsValid` Hand
    (:`Is Valid`
      (if isLeft
        (bind _ashand_bp (cast `/Game/Characters/Mapster/HandBP` Hand))
        (if (`Hand.LPressed` _ashand_bp)
          (if (`self.CanActivate`)
            (set `self.Pressed` true)
            (set `self.CanActivate` false)
            (`PrimitiveComponent.SetRenderCustomDepth` (`self.SkeletalMesh`) true :!label _label_2)
            (`PrimitiveComponent.SetCustomDepthStencilValue` (`self.SkeletalMesh`) 2)
            (bind _outactors (`GameplayStatics.GetAllActorsOfClass` "/Game/Blueprints/Traps/Manhole.Manhole_C"))
            (set `self.Manholes` _outactors)
            (if (`self.IsTutorial`)
              (`self.IncrementTutorial`))
            (`KismetSystemLibrary.Delay` (`self.SoundDelay`))
            (for _array_element (`self.Manholes`)
              (if (`Trap.IsPlaced` _array_element)
                (`/Game/Blueprints/Traps/Manhole.ActivateManhole` _array_element)))
            (`SkeletalMeshComponent.PlayAnimation` (`self.SkeletalMesh`) "/Game/ArtAssets/ControlPanel/ControlPanelAnims/SmallButton/SButton_v_02_Anim_Montage.SButton_v_02_Anim_Montage" false)
            (`GameplayStatics.PlaySoundAtLocation` "/Game/Audio/SoundEffects/ButtonPress.ButtonPress" (0.0 0.0 0.0) (struct) 1.0 1.0 0.0 null null null)
            (`KismetSystemLibrary.Delay` (- (`self.Cooldown`) (`self.SoundDelay`)))
            (`self.ResetButton`)))
        (else
          (bind _ashand_bp_2 (cast `/Game/Characters/Mapster/HandBP` Hand))
          (if (`Hand.RPressed` _ashand_bp_2)
            (if (`self.CanActivate`)
              (set `self.Pressed` true)
              (set `self.CanActivate` false)
              (goto _label_2))))))))

(event `ResetButton`
  (set `self.Pressed` false)
  (set `self.CanActivate` true))

(event `self.ReceiveActorBeginOverlap`
  (params (OtherActor :type "Actor Object Reference"))
  (cast `/Game/Characters/Mapster/HandBP` OtherActor)
  (set `self.Hovered` true))

(event `self.ReceiveActorEndOverlap`
  (params (OtherActor :type "Actor Object Reference"))
  (cast `/Game/Characters/Mapster/HandBP` OtherActor)
  (set `self.Hovered` false))

(event `IncrementTutorial`
  (if (< (`/Game/Blueprints/Tutorial/TutorialController.SlideIndex` (`self.TutorialController`)) 2)
    _
    (elif (> (`KismetArrayLibrary.Array_Length` (`self.Manholes`)) 0)
      (if (not (`self.Completed`))
        (`/Game/Blueprints/Tutorial/TutorialController.IncrementConsole` (`self.TutorialController`) (`self.TutorialCheckIndex`))
        (set `self.Completed` true)))))

(fn `UserConstructionScript`)