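; Control panel button that a HandBP presses to remove every placed Trap from the level.
; Activation with either hand, gated by a cooldown, restores each trap's road material and HasTrap flag, destroys the traps, resets the player's trap counts and plays sound and animation.
; Hand overlap drives a custom-depth outline, with stencil values for ready, unavailable and pressed.
; In tutorial mode, the first press with traps present advances the TutorialController console.
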(event `self.ReceiveBeginPlay`
  (bind _outactors (`GameplayStatics.GetAllActorsOfClass` "/Game/Blueprints/Traps/JailCell.JailCell_C"))
  (set `self.JailCells` _outactors)
  (bind _returnvalue (`GameplayStatics.GetActorOfClass` "/Game/Blueprints/Tutorial/TutorialController.TutorialController_C"))
  (set `self.TutorialController` _returnvalue))

(event `self.ReceiveTick`
  (params (DeltaSeconds :type "Float (single-precision)"))
  (if (`self.Hovered`)
    (`PrimitiveComponent.SetRenderCustomDepth` (`self.SkeletalMesh`) true)
    (if (`self.CanActivate`)
      (`PrimitiveComponent.SetCustomDepthStencilValue` (`self.SkeletalMesh`) 1)
      (goto _label :!via `Reset`)
      (else
        (`PrimitiveComponent.SetCustomDepthStencilValue` (`self.SkeletalMesh`) 0)
        (goto _label :!via `Reset`)))
    (else
      (`/Engine/EditorBlueprintResources/StandardMacros.DoOnce` false :!label _label
        (:`Completed`
          (`PrimitiveComponent.SetRenderCustomDepth` (`self.SkeletalMesh`) false))))))

(event `self.ActivateButton`
  (params (Hand :type "Character Object Reference") (isLeft :type Boolean))
  (bind _skeletalmesh (`self.SkeletalMesh`))
  (`/Engine/EditorBlueprintResources/StandardMacros.IsValid` Hand
    (:`Is Valid`
      (if isLeft
        (bind _ashand_bp (cast `/Game/Characters/HandBP` Hand))
        (if (`Hand.LPressed` _ashand_bp)
          (if (`self.CanActivate`)
            (set `self.Pressed` true)
            (set `self.CanActivate` false)
            (`KismetSystemLibrary.PrintString` "LButton Pressed!" true true (struct :`R` 1.0 :`G` 0.9675 :`A` 1.0))
            (`PrimitiveComponent.SetRenderCustomDepth` _skeletalmesh true :!label _label_2)
            (`PrimitiveComponent.SetCustomDepthStencilValue` _skeletalmesh 2)
            (bind _outactors (`GameplayStatics.GetAllActorsOfClass` "/Script/CapstonePrototype1.Trap"))
            (if (`self.IsTutorial`)
              (`self.IncrementTutorial` _outactors))
            (`KismetSystemLibrary.Delay` (`self.SoundDelay`))
            (for _array_element _outactors
              (bind _ashand_bp_2 (cast `/Game/Characters/HandBP` (`GameplayStatics.GetPlayerCharacter` 0)))
              (bind _road (`Trap.Road` _array_element))
              (`/Game/Characters/HandBP.SetRoadMat` _ashand_bp_2 _road (struct :`R` 1.0 :`G` 1.0 :`B` 1.0 :`A` 1.0))
              (`/Engine/EditorBlueprintResources/StandardMacros.IsValid` _road
                (:`Is Valid`
                  (set `Road.HasTrap` false _road))
                (:`Is Not Valid`
                  _))
              (`self.K2_DestroyActor` _array_element))
            (bind _ashand_bp_3 (cast `/Game/Characters/HandBP` (`GameplayStatics.GetPlayerCharacter` 0)))
            (`/Game/Characters/HandBP.ResetTrapCounts` _ashand_bp_3)
            (`GameplayStatics.PlaySoundAtLocation` "/Game/Audio/SoundEffects/ButtonPress.ButtonPress" (0.0 0.0 0.0) (struct) 1.0 1.0 0.0 null null null)
            (`SkeletalMeshComponent.PlayAnimation` (`self.SkeletalMesh`) "/Game/ArtAssets/ControlPanel/ControlPanelAnims/SmallButton/SButton_v_02_Anim_Montage.SButton_v_02_Anim_Montage" false)
            (`KismetSystemLibrary.Delay` (- (`self.Cooldown`) (`self.SoundDelay`)))
            (`self.ResetButton`)))
        (else
          (bind _ashand_bp_4 (cast `/Game/Characters/HandBP` Hand))
          (if (`Hand.RPressed` _ashand_bp_4)
            (if (`self.CanActivate`)
              (set `self.Pressed` true)
              (set `self.CanActivate` false)
              (`KismetSystemLibrary.PrintString` "RButton Pressed!" true true (struct :`R` 1.0 :`G` 0.021536 :`A` 1.0))
              (goto _label_2))))))))

(event `ResetButton`
  (set `self.Pressed` false)
  (set `self.CanActivate` true))

(event `self.ReceiveActorBeginOverlap`
  (params (OtherActor :type "Actor Object Reference"))
  (cast `/Game/Characters/HandBP` OtherActor)
  (set `self.Hovered` true))

(event `self.ReceiveActorEndOverlap`
  (params (OtherActor :type "Actor Object Reference"))
  (cast `/Game/Characters/HandBP` OtherActor)
  (set `self.Hovered` false))

(event `IncrementTutorial`
  (params (TrapArray :type "Array of Trap Object Reference"))
  (if (> (`KismetArrayLibrary.Array_Length` TrapArray) 0)
    (if (not (`self.Completed`))
      (`/Game/Blueprints/Tutorial/TutorialController.IncrementConsole` (`self.TutorialController`) (`self.TutorialCheckIndex`))
      (set `self.Completed` true))))

(fn `UserConstructionScript`)