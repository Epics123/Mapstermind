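; Control panel button that, when pressed by a HandBP hand, sets off an earthquake that flings every PiecelingBP.
; ActivateButton checks the matching left or right press flag, waits SoundDelay, gathers all Piecelings and plays button and quake sounds.
; TriggerEarthquake disables their controllers' input and launches each on a suggested high-arc velocity, restoring input and resetting the button shortly after.
; LandingLocation serves as arc target and is overwritten by each computed toss velocity.
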(event `self.ActivateButton`
  (params (Hand :type "Character Object Reference") (isLeft :type Boolean))
  (`/Engine/EditorBlueprintResources/StandardMacros.IsValid` Hand
    (:`Is Valid`
      (if isLeft
        (bind _ashand_bp (cast `/Game/Characters/Mapster/HandBP` Hand))
        (if (`Hand.LPressed` _ashand_bp)
          (set `self.Pressed` true)
          (set `self.CanActivate` false)
          (`KismetSystemLibrary.PrintString` "LButton Pressed!" true true (struct :`R` 1.0 :`G` 0.9675 :`A` 1.0))
          (`KismetSystemLibrary.Delay` (`self.SoundDelay`) :!label _label)
          (`GameplayStatics.PlaySoundAtLocation` "/Game/Audio/SoundEffects/ButtonPress.ButtonPress" (0.0 0.0 0.0) (struct) 1.0 1.0 0.0 null null null)
          (bind _outactors (`GameplayStatics.GetAllActorsOfClass` "/Game/Characters/Piecelings/PiecelingBP.PiecelingBP_C"))
          (set `self.LittleGuysArray` _outactors)
          (`GameplayStatics.PlaySoundAtLocation` "/Game/Audio/SoundEffects/Earthquake.Earthquake" (0.0 0.0 0.0) (struct) 0.8 0.8 0.0 null null null)
          (`self.TriggerEarthquake`))
        (else
          (bind _ashand_bp_2 (cast `/Game/Characters/Mapster/HandBP` Hand))
          (if (`Hand.RPressed` _ashand_bp_2)
            (set `self.Pressed` true)
            (set `self.CanActivate` false)
            (`KismetSystemLibrary.PrintString` "RButton Pressed!" true true (struct :`R` 1.0 :`G` 0.021536 :`A` 1.0))
            (goto _label)))))))

(event `TriggerEarthquake`
  (for _array_element (`self.LittleGuysArray`)
    (`self.DisableInput` (`Pawn.GetController` _array_element) null)
    (`self.LaunchPlayer` _array_element))
  (`KismetSystemLibrary.Delay` 0.2)
  (for _array_element_2 (`self.LittleGuysArray`)
    (`self.EnableInput` (`Pawn.GetController` _array_element_2) null))
  (set `self.Pressed` false)
  (set `self.CanActivate` true))

(event `LaunchPlayer`
  (params (NewParam :type "/Game/Characters/Piecelings/PiecelingBP Object Reference"))
  (bind _tossvelocity (`GameplayStatics.BlueprintSuggestProjectileVelocity` (`self.K2_GetActorLocation` NewParam) (`self.LandingLocation`) 1500.0 0.0 "DoNotTrace" 0.0 true true))
  (bind _output_get (set `self.LandingLocation` _tossvelocity))
  (`Character.LaunchCharacter` NewParam _output_get true true))

(fn `UserConstructionScript`)