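; Control panel button actor that a HandBP presses to trigger an earthquake that stuns and launches every PiecelingBP.
; Hand overlap drives a custom-depth highlight, with stencil values distinguishing ready, unavailable and pressed states.
; A press requires the matching hand's input and a pulled ControlPanelLever, then plays sound, animation and camera shake.
; Piecelings lose input and arc toward a landing location via suggested projectile velocity; input returns, then a cooldown re-arms button and lever.
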(event `self.ReceiveBeginPlay`)

(event `self.ReceiveTick`
  (params (DeltaSeconds :type "Float (single-precision)"))
  (if (`self.Hovered`)
    (`PrimitiveComponent.SetRenderCustomDepth` (`self.SkeletalMesh`) true)
    (if (`self.CanActivate`)
      (`PrimitiveComponent.SetCustomDepthStencilValue` (`self.SkeletalMesh`) 1)
      (goto _label :!via `Reset`)
      (else
        (`PrimitiveComponent.SetCustomDepthStencilValue` (`self.SkeletalMesh`) 0)
        (goto _label :!via `Reset`)))
    (else
      (`/Engine/EditorBlueprintResources/StandardMacros.DoOnce` false :!label _label
        (:`Completed`
          (`PrimitiveComponent.SetRenderCustomDepth` (`self.SkeletalMesh`) false))))))

(event `self.ActivateButton`
  (params (Hand :type "Character Object Reference") (isLeft :type Boolean))
  (bind _skeletalmesh (`self.SkeletalMesh`))
  (`/Engine/EditorBlueprintResources/StandardMacros.IsValid` Hand
    (:`Is Valid`
      (if isLeft
        (bind _ashand_bp (cast `/Game/Characters/Mapster/HandBP` Hand))
        (if (`Hand.LPressed` _ashand_bp)
          (if (`self.CanActivate`)
            (bind _returnvalue (`GameplayStatics.GetActorOfClass` "/Game/Blueprints/ControlPanel/ControlPanelLever.ControlPanelLever_C"))
            (if (`/Game/Blueprints/ControlPanel/ControlPanelLever.Pulled` _returnvalue)
              (set `self.Pressed` true)
              (set `self.CanActivate` false)
              (`PrimitiveComponent.SetRenderCustomDepth` _skeletalmesh true :!label _label_2)
              (`PrimitiveComponent.SetCustomDepthStencilValue` _skeletalmesh 2)
              (`KismetSystemLibrary.Delay` (`self.SoundDelay`))
              (`GameplayStatics.PlaySoundAtLocation` "/Game/Audio/SoundEffects/ButtonPress.ButtonPress" (0.0 0.0 0.0) (struct) 1.0 1.0 0.0 null null null)
              (`GameplayStatics.PlaySoundAtLocation` "/Game/Audio/SoundEffects/Earthquake.Earthquake" (0.0 0.0 0.0) (struct) 0.8 0.8 0.0 null null null)
              (`SkeletalMeshComponent.PlayAnimation` (`self.SkeletalMesh`) "/Game/ArtAssets/ControlPanel/ControlPanelAnims/SmallButton/SButton_v_02_Anim_Montage.SButton_v_02_Anim_Montage" false)
              (if (<= (`KismetArrayLibrary.Array_Length` (`self.LittleGuysArray`)) 0)
                (bind _outactors (`GameplayStatics.GetAllActorsOfClass` "/Game/Characters/Piecelings/PiecelingBP.PiecelingBP_C"))
                (set `self.LittleGuysArray` _outactors))
              (`GameplayStatics.PlayWorldCameraShake` "/Game/Blueprints/Weapons/EarthquakeShake.EarthquakeShake_C" (`PlayerCameraManager.GetCameraLocation` (`GameplayStatics.GetPlayerCameraManager` 0)) 0.0 500.0)
              (`self.TriggerEarthquake`))))
        (else
          (bind _ashand_bp_2 (cast `/Game/Characters/Mapster/HandBP` Hand))
          (if (`Hand.RPressed` _ashand_bp_2)
            (if (`self.CanActivate`)
              (bind _returnvalue_2 (`GameplayStatics.GetActorOfClass` "/Game/Blueprints/ControlPanel/ControlPanelLever.ControlPanelLever_C"))
              (if (`/Game/Blueprints/ControlPanel/ControlPanelLever.Pulled` _returnvalue_2)
                (set `self.Pressed` true)
                (set `self.CanActivate` false)
                (goto _label_2)))))))))

(event `self.ReceiveActorBeginOverlap`
  (params (OtherActor :type "Actor Object Reference"))
  (cast `/Game/Characters/Mapster/HandBP` OtherActor)
  (set `self.Hovered` true))

(event `self.ReceiveActorEndOverlap`
  (params (OtherActor :type "Actor Object Reference"))
  (cast `/Game/Characters/Mapster/HandBP` OtherActor)
  (set `self.Hovered` false))

(event `TriggerEarthquake`
  (for _array_element (`self.LittleGuysArray`)
    (`self.DisableInput` _array_element null)
    (`self.LaunchPlayer` _array_element))
  (`KismetSystemLibrary.Delay` (`self.PlayerStunTime`))
  (for _array_element_2 (`self.LittleGuysArray`)
    (`self.EnableInput` _array_element_2 null))
  (`KismetSystemLibrary.Delay` (`self.EarthquakeCooldown`))
  (set `self.Pressed` false)
  (set `self.CanActivate` true)
  (bind _returnvalue (`GameplayStatics.GetActorOfClass` "/Game/Blueprints/ControlPanel/ControlPanelLever.ControlPanelLever_C"))
  (set `/Game/Blueprints/ControlPanel/ControlPanelLever.Pulled` false _returnvalue)
  (set `Lever.CanActivate` true _returnvalue))

(event `LaunchPlayer`
  (params (NewParam :type "/Game/Characters/Piecelings/PiecelingBP Object Reference"))
  (bind _tossvelocity (`GameplayStatics.BlueprintSuggestProjectileVelocity` (`self.K2_GetActorLocation` NewParam) (`self.LandingLocation`) (`self.PlayerLaunchSpeed`) 0.0 "DoNotTrace" 0.0 true))
  (`Character.LaunchCharacter` NewParam _tossvelocity true true))

(fn `UserConstructionScript`)