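; Hand-operated control panel button that triggers the Whirlpool, usable only while the ControlPanelLever is pulled.
; HandBP overlaps set a hover flag, which Tick turns into a custom-depth highlight with stencil values reflecting availability.
; ActivateButton checks the left or right hand press, then plays sound and animation and activates the Whirlpool.
; After a cooldown, it re-enables itself and resets the lever, both found through GetActorOfClass.
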(event `self.ReceiveBeginPlay`)

(event `self.ReceiveTick`
  (params (DeltaSeconds :type "Float (single-precision)"))
  (if (`self.Hovered`)
    (`PrimitiveComponent.SetRenderCustomDepth` (`self.SkeletalMesh`) true)
    (if (`self.CanActivate`)
      (`PrimitiveComponent.SetCustomDepthStencilValue` (`self.SkeletalMesh`) 1)
      (goto _label :!via `Reset`)
      (else
        (`PrimitiveComponent.SetCustomDepthStencilValue` (`self.SkeletalMesh`) 0)
        (goto _label :!via `Reset`)))
    (else
      (`/Engine/EditorBlueprintResources/StandardMacros.DoOnce` false :!label _label
        (:`Completed`
          (`PrimitiveComponent.SetRenderCustomDepth` (`self.SkeletalMesh`) false))))))

(event `self.ActivateButton`
  (params (Hand :type "Character Object Reference") (isLeft :type Boolean))
  (bind _skeletalmesh (`self.SkeletalMesh`))
  (`/Engine/EditorBlueprintResources/StandardMacros.IsValid` Hand
    (:`Is Valid`
      (if isLeft
        (bind _ashand_bp (cast `/Game/Characters/Mapster/HandBP` Hand))
        (if (`Hand.LPressed` _ashand_bp)
          (if (`self.CanActivate`)
            (bind _returnvalue (`GameplayStatics.GetActorOfClass` "/Game/Blueprints/ControlPanel/ControlPanelLever.ControlPanelLever_C"))
            (if (`/Game/Blueprints/ControlPanel/ControlPanelLever.Pulled` _returnvalue)
              (set `self.Pressed` true)
              (set `self.CanActivate` false)
              (`PrimitiveComponent.SetRenderCustomDepth` _skeletalmesh true :!label _label_2)
              (`PrimitiveComponent.SetCustomDepthStencilValue` _skeletalmesh 2)
              (`KismetSystemLibrary.Delay` (`self.SoundDelay`))
              (`GameplayStatics.PlaySoundAtLocation` "/Game/Audio/SoundEffects/ButtonPress.ButtonPress" (0.0 0.0 0.0) (struct) 1.0 1.0 0.0 null null null)
              (`SkeletalMeshComponent.PlayAnimation` (`self.SkeletalMesh`) "/Game/ArtAssets/ControlPanel/ControlPanelAnims/SmallButton/SButton_v_02_Anim_Montage.SButton_v_02_Anim_Montage" false)
              (bind _returnvalue_2 (`GameplayStatics.GetActorOfClass` "/Game/Blueprints/Traps/Whirlpool.Whirlpool_C"))
              (`/Game/Blueprints/Traps/Whirlpool.ActivateWhirlpool` _returnvalue_2)
              (`KismetSystemLibrary.Delay` (`self.WhirlpoolCooldown`))
              (set `self.Pressed` false)
              (set `self.CanActivate` true)
              (bind _returnvalue_3 (`GameplayStatics.GetActorOfClass` "/Game/Blueprints/ControlPanel/ControlPanelLever.ControlPanelLever_C"))
              (set `/Game/Blueprints/ControlPanel/ControlPanelLever.Pulled` false _returnvalue_3)
              (set `Lever.CanActivate` true _returnvalue_3))))
        (else
          (bind _ashand_bp_2 (cast `/Game/Characters/Mapster/HandBP` Hand))
          (if (`Hand.RPressed` _ashand_bp_2)
            (if (`self.CanActivate`)
              (bind _returnvalue_4 (`GameplayStatics.GetActorOfClass` "/Game/Blueprints/ControlPanel/ControlPanelLever.ControlPanelLever_C"))
              (if (`/Game/Blueprints/ControlPanel/ControlPanelLever.Pulled` _returnvalue_4)
                (set `self.Pressed` true)
                (set `self.CanActivate` false)
                (goto _label_2)))))))))

(event `self.ReceiveActorBeginOverlap`
  (params (OtherActor :type "Actor Object Reference"))
  (cast `/Game/Characters/Mapster/HandBP` OtherActor)
  (set `self.Hovered` true))

(event `self.ReceiveActorEndOverlap`
  (params (OtherActor :type "Actor Object Reference"))
  (cast `/Game/Characters/Mapster/HandBP` OtherActor)
  (set `self.Hovered` false))

(fn `UserConstructionScript`)