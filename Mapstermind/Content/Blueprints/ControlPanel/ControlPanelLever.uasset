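; Control panel lever actor that a player's hand can hover and flip once.
; Hand overlaps on the hit sphere set a hover flag, which Tick turns into a custom-depth highlight with stencil values showing whether it can activate.
; HandActivateLever plays the toggle animation, then on the first pull latches Pulled, switches the highlight stencil, plays a flick sound and clears CanActivate.
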(event `self.ReceiveTick`
  (params (DeltaSeconds :type "Float (single-precision)"))
  (if (`self.Hovered`)
    (`PrimitiveComponent.SetRenderCustomDepth` (`self.SkeletalMesh`) true)
    (if (`self.CanActivate`)
      (`PrimitiveComponent.SetCustomDepthStencilValue` (`self.SkeletalMesh`) 1)
      (goto _label :!via `Reset`)
      (else
        (`PrimitiveComponent.SetCustomDepthStencilValue` (`self.SkeletalMesh`) 0)
        (goto _label :!via `Reset`)))
    (else
      (`/Engine/EditorBlueprintResources/StandardMacros.DoOnce` false :!label _label
        (:`Completed`
          (`PrimitiveComponent.SetRenderCustomDepth` (`self.SkeletalMesh`) false))))))

(event `self.HandActivateLever`
  (params (Hand :type "Character Object Reference") (isLeft :type Boolean))
  (bind _skeletalmesh (`self.SkeletalMesh`))
  (bind _ashand_bp (cast `/Game/Characters/Mapster/HandBP` Hand))
  (`SkeletalMeshComponent.PlayAnimation` (`self.SkeletalMesh`) "/Game/ArtAssets/ControlPanel/ControlPanelAnims/ToggleSwitch/ToggleSwitch_v_02_Anim_Montage.ToggleSwitch_v_02_Anim_Montage" false)
  (if (not (`self.Pulled`))
    (set `self.Pulled` true)
    (`PrimitiveComponent.SetRenderCustomDepth` _skeletalmesh true)
    (`PrimitiveComponent.SetCustomDepthStencilValue` _skeletalmesh 2)
    (`GameplayStatics.PlaySoundAtLocation` "/Game/Audio/SoundEffects/SwitchFlick.SwitchFlick" (0.0 0.0 0.0) (struct) 1.0 1.0 0.0 null null null)
    (set `self.CanActivate` false)))

(event `self.ReceiveActorBeginOverlap`
  (params (OtherActor :type "Actor Object Reference")))

(event `self.LeverHitSphere.OnComponentBeginOverlap`
  (params (OverlappedComponent :type "PrimitiveComponent Object Reference") (OtherActor :type "Actor Object Reference") (OtherComp :type "PrimitiveComponent Object Reference") (OtherBodyIndex :type Integer) (bFromSweep :type Boolean) (SweepResult :type "HitResult Structure (by ref)"))
  (cast `/Game/Characters/Mapster/HandBP` OtherActor)
  (set `self.Hovered` true))

(event `self.LeverHitSphere.OnComponentEndOverlap`
  (params (OverlappedComponent :type "PrimitiveComponent Object Reference") (OtherActor :type "Actor Object Reference") (OtherComp :type "PrimitiveComponent Object Reference") (OtherBodyIndex :type Integer))
  (cast `/Game/Characters/Mapster/HandBP` OtherActor)
  (set `self.Hovered` false))

(fn `UserConstructionScript`)