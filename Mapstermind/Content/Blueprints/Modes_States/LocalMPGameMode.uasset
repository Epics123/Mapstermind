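; Game mode for local multiplayer levels, where a Hand and Piecelings play through timed tasks to open an exit door.
; BeginPlay creates players at tagged PlayerStarts, possesses pawns from PersistantInstance character picks, and sets the GameCam view.
; The tutorial starts its timer immediately, while other levels disable input and play a start sequence.
; Six soundtrack layers start together, and completed tasks unmute submixes until the final one reveals the exit.
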(event `self.ReceiveBeginPlay`
  (bind _submixes (`self.SubMixes`))
  (set `self.Seconds` (`self.MaxTime`))
  ;[1 0.3664 0] Init input receivers
  (`self.GetPlayerStartPoints`)
  (`self.SpawnInputReceivers`)
  (`self.LoadCharacterSelectInfo`)
  (bind _returnvalue (`GameplayStatics.GetCurrentLevelName` true))
  (if (`KismetStringLibrary.EqualEqual_StrStr` _returnvalue "TutorialScene")
    (`self.CreateTimer`)
    (else
      (`self.DisableAllPlayersInput`)
      (bind _returnvalue_2 (`|CreateWidget` "/Game/Blueprints/Widgets/StartSequence.StartSequence_C"))
      (`UserWidget.AddToViewport` _returnvalue_2 0)
      (set `self.SequenceWidget` _returnvalue_2)
      (bind _asstart_sequence (cast `/Game/Blueprints/Widgets/StartSequence` (`self.SequenceWidget`)))
      (`/Game/Blueprints/Widgets/StartSequence.PlayStartSequence` _asstart_sequence)))
  (bind _returnvalue_3 (`GameplayStatics.GetActorOfClass` "/Script/Engine.CameraActor"))
  (if (`ActorComponent.ComponentHasTag` (`CameraActor.CameraComponent` _returnvalue_3) "GameCam")
    (bind _returnvalue_4 (`GameplayStatics.GetActorOfClass` "/Game/Characters/Mapster/HandBP.HandBP_C"))
    (`/Engine/EditorBlueprintResources/StandardMacros.IsValid` _returnvalue_4
      (:`Is Valid`
        (bind _asplayer_controller (cast `PlayerController` (`Pawn.GetController` _returnvalue_4)))
        (`PlayerController.SetViewTargetWithBlend` (`GameplayStatics.GetPlayerController` (`GameplayStatics.GetPlayerControllerID` _asplayer_controller)) _returnvalue_3 0.0 "VTBlend_Linear" 0.0 false))
      (:`Is Not Valid`
        (`PlayerController.SetViewTargetWithBlend` (`GameplayStatics.GetPlayerController` 0) _returnvalue_3 0.0 "VTBlend_Linear" 0.0 false)))
    (`GameplayStatics.PlaySoundAtLocation` "/Game/Audio/Music/Tracks/Mapstermind_Soundtrack_Track1.Mapstermind_Soundtrack_Track1" (0.0 0.0 0.0) (struct) 1.0 1.0 0.0 null null null)
    (`GameplayStatics.PlaySoundAtLocation` "/Game/Audio/Music/Tracks/Mapstermind_Soundtrack_Track2.Mapstermind_Soundtrack_Track2" (0.0 0.0 0.0) (struct) 1.0 1.0 0.0 null null null)
    (`GameplayStatics.PlaySoundAtLocation` "/Game/Audio/Music/Tracks/Mapstermind_Soundtrack_Track3.Mapstermind_Soundtrack_Track3" (0.0 0.0 0.0) (struct) 1.0 1.0 0.0 null null null)
    (`GameplayStatics.PlaySoundAtLocation` "/Game/Audio/Music/Tracks/Mapstermind_Soundtrack_Track4.Mapstermind_Soundtrack_Track4" (0.0 0.0 0.0) (struct) 1.0 1.0 0.0 null null null)
    (`GameplayStatics.PlaySoundAtLocation` "/Game/Audio/Music/Tracks/Mapstermind_Soundtrack_Track5.Mapstermind_Soundtrack_Track5" (0.0 0.0 0.0) (struct) 1.0 1.0 0.0 null null null)
    (`GameplayStatics.PlaySoundAtLocation` "/Game/Audio/Music/Tracks/Mapstermind_Soundtrack_Track6.Mapstermind_Soundtrack_Track6" (0.0 0.0 0.0) (struct) 1.0 1.0 0.0 null null null)
    (set `self.GameOver` false)
    (for _index (range 1 (`KismetArrayLibrary.Array_Length` _submixes))
      (`SoundSubmix.SetSubmixOutputVolume` (`|GetArrayItem` _submixes _index) 0.0))
    (bind _outactors (`GameplayStatics.GetAllActorsOfClass` "/Game/Blueprints/ControlPanel/ConsoleTape.ConsoleTape_C"))
    (for _array_element _outactors
      (`PrimitiveComponent.SetCastShadow` (`/Game/Blueprints/ControlPanel/ConsoleTape.Widget` _array_element) false))))

(fn `CreateTimer`
  (set `self.TimerCreated` true)
  (bind _returnvalue (`GameplayStatics.GetActorOfClass` "/Game/Blueprints/Level/BigHourglass.BigHourglass_C"))
  (bind _output_get (set `self.BigHourglass` _returnvalue))
  (bind _outactors (`GameplayStatics.GetAllActorsOfClass` "/Game/Blueprints/Level/ClockPercentage.ClockPercentage_C"))
  (bind _astimer (cast `/Game/Blueprints/Widgets/Level/Timer` (`WidgetComponent.GetWidget` (`/Game/Blueprints/Level/ClockPercentage.Widget` (`|GetArrayItem` _outactors)))))
  (set `self.Timer` _astimer)
  (bind _returnvalue_2 (`GameplayStatics.GetCurrentLevelName` true))
  (`/Game/Blueprints/Widgets/Level/Timer.RunTimer` _astimer (`KismetStringLibrary.EqualEqual_StrStr` _returnvalue_2 "TutorialScene")))

(fn `DecrementTask`
  (returns (Tasks :type Integer))
  (set `self.NumTasksCompleted` (- (`self.NumTasksCompleted`) 1.0))
  (return 0))

(fn `DisableAllPlayersInput`
  (for _array_element (`self.PlayerControllers`)
    (`self.DisableInput` (`Controller.K2_GetPawn` _array_element) _array_element)))

(fn `EnableAllPlayersInput`
  (for _array_element (`self.PlayerControllers`)
    (`self.EnableInput` (`Controller.K2_GetPawn` _array_element) _array_element)))

(fn `GetPlayerStartPoints`
  (bind _outactors (`GameplayStatics.GetAllActorsOfClass` "/Script/Engine.PlayerStart"))
  (set `self.PlayerSpawns` _outactors))

(fn `IncrementTask`
  (returns (CompletedTaskNum :type Integer))
  (if (< (`self.TrackNum`) (`KismetArrayLibrary.Array_Length` (`self.SubMixes`)))
    (bind _output_get (set `self.TrackNum` (+ (`self.TrackNum`) 1)))
    (`SoundSubmix.SetSubmixOutputVolume` (`|GetArrayItem` (`self.SubMixes`) _output_get) 1.0))
  (bind _output_get_2 (set `self.NumTasksCompleted` (+ (`self.NumTasksCompleted`) 1.0)))
  (if (== (`self.NumTasksCompleted`) (`self.MaxTasks`))
    (`self.ShowExitDoor`))
  (return (`KismetMathLibrary.FTrunc` _output_get_2)))

(fn `LoadCharacterSelectInfo`
  (locals (SpawnIndex :type Integer))
  (bind _aspersistant_instance (cast `/Game/Blueprints/Modes_States/PersistantInstance` (`GameplayStatics.GetGameInstance`)))
  (for _array_element (`self.PlayerControllers`)
    (bind _returnvalue (`GameplayStatics.GetPlayerControllerID` _array_element))
    (bind _value (`BlueprintMapLibrary.Map_Find` (`/Game/Blueprints/Modes_States/PersistantInstance.SelectedMeshes` _aspersistant_instance) _returnvalue))
    (if (== _value "/Game/ArtAssets/Characters/Animations/Mapster/Left/Mapster_Hand_L.Mapster_Hand_L")
      (bind _returnvalue_2 (`|SpawnActorFromClass` "/Game/Characters/Mapster/HandBP.HandBP_C" (`self.GetTransform` (`|GetArrayItem` (`self.PlayerSpawns`))) "Undefined" "OverrideRootScale" null _returnvalue null))
      (`Controller.Possess` _array_element _returnvalue_2)
      (elif (!= _value null)
        (if (== (`local.SpawnIndex`) 0)
          (`/Engine/EditorBlueprintResources/StandardMacros.IncrementInt` (`local.SpawnIndex`)
            (:`  `
              _)))
        (bind _returnvalue_3 (`|SpawnActorFromClass` "/Game/Characters/Piecelings/PiecelingBP.PiecelingBP_C" (`self.GetTransform` (`|GetArrayItem` (`self.PlayerSpawns`) (`local.SpawnIndex`))) "Undefined" "OverrideRootScale" null _returnvalue null))
        (`self.SetPlayerMeshAndPos` _returnvalue_3 _value)
        (`Controller.Possess` _array_element _returnvalue_3)
        (`/Engine/EditorBlueprintResources/StandardMacros.IncrementInt` (`local.SpawnIndex`))))))

(fn `NameToInt`
  (params (PlayerStart :type "PlayerStart Object Reference"))
  (returns (ReturnValue :type Integer))
  (return (`KismetStringLibrary.Conv_StringToInt` (`KismetStringLibrary.Conv_NameToString` (`PlayerStart.PlayerStartTag` PlayerStart)))))

(fn `SetAnimBP`
  (params (MeshIndex :type Integer) (Player :type "/Game/Characters/Piecelings/PiecelingBP Object Reference"))
  (bind _skeletalmesh (`/Game/Characters/Piecelings/PiecelingBP.SkeletalMesh` (`local.Player`)))
  (bind _skeletalmesh_2 (`/Game/Characters/Piecelings/PiecelingBP.SkeletalMesh` (`local.Player`)))
  (bind _skeletalmesh_3 (`/Game/Characters/Piecelings/PiecelingBP.SkeletalMesh` (`local.Player`)))
  (bind _skeletalmesh_4 (`/Game/Characters/Piecelings/PiecelingBP.SkeletalMesh` (`local.Player`)))
  (bind _skeletalmesh_5 (`/Game/Characters/Piecelings/PiecelingBP.SkeletalMesh` (`local.Player`)))
  (bind _skeletalmesh_6 (`/Game/Characters/Piecelings/PiecelingBP.SkeletalMesh` (`local.Player`)))
  (switch `int` MeshIndex
    (:`0`
      (`SceneComponent.SetRelativeScale3D` _skeletalmesh_2 (75.0 75.0 75.0))
      (`SceneComponent.K2_SetRelativeLocation` _skeletalmesh_2 (27.0 -985.0 -176.0) false false)
      (`SkeletalMeshComponent.SetAnimInstanceClass` (`/Game/Characters/Piecelings/PiecelingBP.SkeletalMesh` (`local.Player`)) "/Game/Characters/Piecelings/PiecelingAnimBps/BBConeAnimBP.BBConeAnimBP_C"))
    (:`1`
      (`SceneComponent.SetRelativeScale3D` _skeletalmesh_3 (75.0 75.0 75.0))
      (`SceneComponent.K2_SetRelativeLocation` _skeletalmesh_3 (27.0 -165.0 -176.0) false false)
      (`SkeletalMeshComponent.SetAnimInstanceClass` (`/Game/Characters/Piecelings/PiecelingBP.SkeletalMesh` (`local.Player`)) "/Game/Characters/Piecelings/PiecelingAnimBps/MWTHAnimBP.MWTHAnimBP_C"))
    (:`2`
      (`SceneComponent.SetRelativeScale3D` _skeletalmesh_6 (150.0 150.0 150.0))
      (`SceneComponent.K2_SetRelativeLocation` _skeletalmesh_6 (27.0 4.0 -176.0) false false)
      (`SkeletalMeshComponent.SetAnimInstanceClass` (`/Game/Characters/Piecelings/PiecelingBP.SkeletalMesh` (`local.Player`)) "/Game/Characters/Piecelings/PiecelingAnimBps/PumpkinAnimBP.PumpkinAnimBP_C"))
    (:`3`
      (`SceneComponent.SetRelativeScale3D` _skeletalmesh_4 (75.0 75.0 75.0))
      (`SceneComponent.K2_SetRelativeLocation` _skeletalmesh_4 (27.0 625.0 -176.0) false false)
      (`SkeletalMeshComponent.SetAnimInstanceClass` (`/Game/Characters/Piecelings/PiecelingBP.SkeletalMesh` (`local.Player`)) "/Game/Characters/Piecelings/PiecelingAnimBps/TrashcanAnimBP.TrashcanAnimBP_C"))
    (:`4`
      (`SceneComponent.SetRelativeScale3D` _skeletalmesh (75.0 75.0 75.0))
      (`SceneComponent.K2_SetRelativeLocation` _skeletalmesh (-27.0 225.0 -176.0) false false))
    (:`5`
      (`SceneComponent.SetRelativeScale3D` _skeletalmesh_5 (75.0 75.0 75.0))
      (`SceneComponent.K2_SetRelativeLocation` _skeletalmesh_5 (27.0 1050.0 -176.0) false false)
      (`SkeletalMeshComponent.SetAnimInstanceClass` (`/Game/Characters/Piecelings/PiecelingBP.SkeletalMesh` (`local.Player`)) "/Game/Characters/Piecelings/PiecelingAnimBps/PConeAnimBP.PConeAnimBP_C"))))

(fn `SetPlayerMesh`
  (params (Player :type "/Game/Characters/Piecelings/PiecelingBP Object Reference") (PlayerIndex :type Integer))
  (bind _skeletalmesh (`/Game/Characters/Piecelings/PiecelingBP.SkeletalMesh` (`local.Player`)))
  (bind _skeletalmesh_2 (`/Game/Characters/Piecelings/PiecelingBP.SkeletalMesh` (`local.Player`)))
  (bind _skeletalmesh_3 (`/Game/Characters/Piecelings/PiecelingBP.SkeletalMesh` (`local.Player`)))
  (switch `int` PlayerIndex
    (:`1`
      (`SkinnedMeshComponent.SetSkinnedAssetAndUpdate` _skeletalmesh_2 "/Game/ArtAssets/Characters/Animations/BabyCone/NewAnims/bbconeanims_v_02.bbconeanims_v_02" true)
      (`SceneComponent.SetRelativeScale3D` _skeletalmesh_2 (75.0 75.0 75.0))
      (`SceneComponent.K2_SetRelativeLocation` _skeletalmesh_2 (27.0 -985.0 -176.0) false false)
      (`SkeletalMeshComponent.SetAnimInstanceClass` (`/Game/Characters/Piecelings/PiecelingBP.SkeletalMesh` (`local.Player`)) "/Game/Characters/Piecelings/PiecelingAnimBps/BBConeAnimBP.BBConeAnimBP_C"))
    (:`2`
      (`SkinnedMeshComponent.SetSkinnedAssetAndUpdate` _skeletalmesh_3 "/Game/ArtAssets/Characters/Animations/Pumpkin/NewAnims/pumpkinanim_v_2.pumpkinanim_v_2" true)
      (`SceneComponent.SetRelativeScale3D` _skeletalmesh_3 (150.0 150.0 150.0))
      (`SceneComponent.K2_SetRelativeLocation` _skeletalmesh_3 (27.0 4.0 -176.0) false false)
      (`SkeletalMeshComponent.SetAnimInstanceClass` (`/Game/Characters/Piecelings/PiecelingBP.SkeletalMesh` (`local.Player`)) "/Game/Characters/Piecelings/PiecelingAnimBps/PumpkinAnimBP.PumpkinAnimBP_C"))
    (:`3`
      (`SkinnedMeshComponent.SetSkinnedAssetAndUpdate` _skeletalmesh "/Game/ArtAssets/Characters/Animations/ManWithHat/NewAnims/manwhatanims_v_02.manwhatanims_v_02" true)
      (`SceneComponent.SetRelativeScale3D` _skeletalmesh (75.0 75.0 75.0))
      (`SceneComponent.K2_SetRelativeLocation` _skeletalmesh (27.0 -165.0 -176.0) false false)
      (`SkeletalMeshComponent.SetAnimInstanceClass` (`/Game/Characters/Piecelings/PiecelingBP.SkeletalMesh` (`local.Player`)) "/Game/Characters/Piecelings/PiecelingAnimBps/MWTHAnimBP.MWTHAnimBP_C"))))

(fn `SetPlayerMeshAndPos`
  (params (Player :type "/Game/Characters/Piecelings/PiecelingBP Object Reference") (Mesh :type "SkeletalMesh Object Reference"))
  (bind _skeletalmesh (`/Game/Characters/Piecelings/PiecelingBP.SkeletalMesh` (`local.Player`)))
  (`SkinnedMeshComponent.SetSkinnedAssetAndUpdate` _skeletalmesh Mesh true)
  (`PrimitiveComponent.SetRenderCustomDepth` _skeletalmesh true)
  (`PrimitiveComponent.SetCustomDepthStencilValue` _skeletalmesh (`/Game/Characters/Piecelings/PiecelingBP.Index` (`local.Player`)))
  (bind _aspersistant_instance (cast `/Game/Blueprints/Modes_States/PersistantInstance` (`GameplayStatics.GetGameInstance`)))
  (bind (_value _returnvalue) (`BlueprintMapLibrary.Map_Find` (`/Game/Blueprints/Modes_States/PersistantInstance.MeshOffsets` _aspersistant_instance) (`local.Mesh`)))
  (if _returnvalue
    (`self.SetAnimBP` _value (`local.Player`))))

(fn `ShowExitDoor`
  (bind _outactors (`GameplayStatics.GetAllActorsOfClass` "/Game/Blueprints/Level/ExitDoor.ExitDoor_C"))
  (bind _output (`|GetArrayItem` _outactors))
  (`PrimitiveComponent.SetCollisionEnabled` (`/Game/Blueprints/Level/ExitDoor.Box` _output) "QueryAndPhysics")
  (`SceneComponent.SetVisibility` (`/Game/Blueprints/Level/ExitDoor.DoorBase` _output) true false)
  (`/Game/Blueprints/Level/ExitDoor.OpenExit` _output))

(fn `Spawn Player`
  (params (CurrentPlayerIndex :type Integer) (InputReceiver :type "/Game/Characters/InputReceiver Object Reference"))
  (returns (Return :type Boolean))
  ;[0.1014 0.1704 1] Create and posses player
  (bind _returnvalue (`GameplayStatics.GetCurrentLevelName` true))
  (if (not (`KismetStringLibrary.EqualEqual_StrStr` _returnvalue "TitleScene"))
    (if (== (`local.CurrentPlayerIndex`) 0)
      (bind _returnvalue_2 (`|SpawnActorFromClass` "/Game/Characters/Mapster/HandBP.HandBP_C" (`self.GetTransform` InputReceiver) "Undefined" "OverrideRootScale" null (`local.CurrentPlayerIndex`) null))
      (`Controller.Possess` (`GameplayStatics.GetPlayerController` (`local.CurrentPlayerIndex`)) _returnvalue_2)
      (else
        (if (not (`self.TimerCreated`))
          (`self.CreateTimer`))
        (bind _returnvalue_3 (`|SpawnActorFromClass` "/Game/Characters/Piecelings/PiecelingBP.PiecelingBP_C" (`self.GetTransform` InputReceiver) "Undefined" "OverrideRootScale" null (`local.CurrentPlayerIndex`) null))
        (`self.SetPlayerMesh` _returnvalue_3 (`local.CurrentPlayerIndex`))
        (`Controller.Possess` (`GameplayStatics.GetPlayerController` (`local.CurrentPlayerIndex`)) _returnvalue_3)))
    (return false)))

(fn `SpawnInputReceivers`
  (locals (Index :type Integer))
  (bind _index (`local.Index`))
  (bind _returnvalue (`GameplayStatics.GetPlayerController` (`local.Index`)))
  ;[0.8338 1 0.2846] Spawn an imput reciever to detect starter input
  (for (_ _array_index) (`self.PlayerSpawns`)
    (set `local.Index` _array_index)
    (for _array_element (`self.PlayerSpawns`)
      (if (== (`self.NameToInt` _array_element) (`local.Index`))
        (`GameplayStatics.CreatePlayer` -1)
        (bind _returnvalue_2 (`|SpawnActorFromClass` "/Game/Characters/InputReceiver.InputReceiver_C" (`self.GetTransform` (`|GetArrayItem` (`self.PlayerSpawns`) _index)) "Undefined" "OverrideRootScale" null _index null))
        (`KismetArrayLibrary.Array_AddUnique` (`self.PlayerInputReceivers`) _returnvalue_2)
        (`Controller.Possess` _returnvalue _returnvalue_2)
        (`KismetArrayLibrary.Array_AddUnique` (`self.PlayerControllers`) _returnvalue)))))

(fn `StopTimer`
  (set `/Game/Blueprints/Widgets/Level/Timer.Stop` true (`self.Timer`)))

(fn `UpdateTimer`
  (bind _returnvalue (`GameplayStatics.GetActorOfClass` "/Game/Blueprints/Level/ClockPercentage.ClockPercentage_C"))
  (bind _astimer (cast `/Game/Blueprints/Widgets/Level/Timer` (`WidgetComponent.GetWidget` (`/Game/Blueprints/Level/ClockPercentage.Widget` _returnvalue))))
  (`/Game/Blueprints/Widgets/Level/ClockProgressBar.Update Time Bar` (`/Game/Blueprints/Widgets/Level/Timer.ClockProgressBar` _astimer) (`KismetMathLibrary.Conv_IntToDouble` (`self.Seconds`)) (`KismetMathLibrary.Conv_IntToDouble` (`self.MaxTime`))))

(fn `UserConstructionScript`)