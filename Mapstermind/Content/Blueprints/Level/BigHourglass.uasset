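; Level hourglass actor that visualises the match time by scaling its top and bottom sand meshes.
; On BeginPlay it reads the maximum and remaining time from LocalMPGameMode.
; StartHourglass skips tutorials, otherwise waits briefly and sets one-second timers for DecreaseTop and IncreaseBottom.
; These functions set each mesh's Z scale from its own time-left or time-passed counter as a proportion of the maximum.
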(event `self.ReceiveBeginPlay`
  (bind _aslocal_mpgame_mode (cast `/Game/Blueprints/Modes_States/LocalMPGameMode` (`GameplayStatics.GetGameMode`)))
  (bind _output_get (set `self.GameMode` _aslocal_mpgame_mode))
  (set `self.MaxTime` (`KismetMathLibrary.Conv_IntToDouble` (`/Game/Blueprints/Modes_States/LocalMPGameMode.MaxTime` _output_get)))
  (set `self.TimeLeft` (`KismetMathLibrary.Conv_IntToDouble` (`/Game/Blueprints/Modes_States/LocalMPGameMode.Seconds` _output_get))))

(event `StartHourglass`
  (params (Tutorial :type Boolean))
  (if (not Tutorial)
    (`KismetSystemLibrary.Delay` 1.0)
    (`KismetSystemLibrary.K2_SetTimer` null "DecreaseTop" 1.0)
    (`KismetSystemLibrary.K2_SetTimer` null "IncreaseBottom" 1.0)))

(fn `DecreaseTop`
  (bind _topsand (`self.TopSand`))
  (bind (_returnvalue_x _returnvalue_y) (`KismetMathLibrary.BreakVector` (`SceneComponent.K2_GetComponentScale` _topsand)))
  (bind _result (`/Engine/EditorBlueprintResources/StandardMacros.DecrementInt` (`KismetMathLibrary.FTrunc` (`self.TimeLeft`)))
    (:`  `
      (if (not (<= _result 0))
        (bind _output_get (set `self.TimeLeftProportion` (/ (`self.TimeLeft`) (`self.MaxTime`))))
        (`SceneComponent.SetWorldScale3D` _topsand (`KismetMathLibrary.MakeVector` _returnvalue_x _returnvalue_y _output_get))))))

(fn `IncreaseBottom`
  (bind _bottomsand (`self.BottomSand`))
  (bind (_returnvalue_x _returnvalue_y) (`KismetMathLibrary.BreakVector` (`SceneComponent.K2_GetComponentScale` _bottomsand)))
  (bind _result (`/Engine/EditorBlueprintResources/StandardMacros.IncrementInt` (`self.TimePassed`))
    (:`  `
      (if (not (>= _result (`KismetMathLibrary.FTrunc` (`self.MaxTime`))))
        (bind _output_get (set `self.TimePassedProportion` (/ (`KismetMathLibrary.Conv_IntToDouble` (`self.TimePassed`)) (`self.MaxTime`))))
        (`SceneComponent.SetWorldScale3D` _bottomsand (`KismetMathLibrary.MakeVector` _returnvalue_x _returnvalue_y _output_get))))))

(fn `UserConstructionScript`)