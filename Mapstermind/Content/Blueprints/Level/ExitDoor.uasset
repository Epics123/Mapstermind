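; ExitDoor is the level exit that removes Piecelings that reach it and triggers their win.
; It starts hidden with Box collision off; OpenExit reveals door and sign and swings the door via timeline-driven RInterpTo, without re-enabling collision here.
; Box overlap destroys each entering PiecelingBP; when none remain, it shows the PiecelingsWin widget, sets GameOver on LocalMPGameMode and stops its timer.
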(event `self.ReceiveBeginPlay`
  (`PrimitiveComponent.SetCollisionEnabled` (`self.Box`) "NoCollision")
  (`SceneComponent.SetVisibility` (`self.DoorBase`) false false)
  (`SceneComponent.SetVisibility` (`self.Door`) false false)
  (`SceneComponent.SetVisibility` (`self.ExitSign`) false false))

(event `self.ReceiveActorBeginOverlap`
  (params (OtherActor :type "Actor Object Reference")))

(event `self.Box.OnComponentBeginOverlap`
  (params (OverlappedComponent :type "PrimitiveComponent Object Reference") (OtherActor :type "Actor Object Reference") (OtherComp :type "PrimitiveComponent Object Reference") (OtherBodyIndex :type Integer) (bFromSweep :type Boolean) (SweepResult :type "HitResult Structure (by ref)"))
  (bind _aspieceling_bp (cast `/Game/Characters/Piecelings/PiecelingBP` OtherActor))
  (`self.K2_DestroyActor` _aspieceling_bp)
  (bind _outactors (`GameplayStatics.GetAllActorsOfClass` "/Game/Characters/Piecelings/PiecelingBP.PiecelingBP_C"))
  (if (<= (`KismetArrayLibrary.Array_Length` _outactors) 0)
    (bind _returnvalue (`|CreateWidget` "/Game/Blueprints/Widgets/GameResult/PiecelingsWin.PiecelingsWin_C"))
    (`UserWidget.AddToViewport` _returnvalue 0)
    (bind _aslocal_mpgame_mode (cast `/Game/Blueprints/Modes_States/LocalMPGameMode` (`GameplayStatics.GetGameMode`)))
    (set `/Game/Blueprints/Modes_States/LocalMPGameMode.GameOver` true _aslocal_mpgame_mode)
    (`/Game/Blueprints/Modes_States/LocalMPGameMode.StopTimer` _aslocal_mpgame_mode)))

(event `OpenExit`
  (`SceneComponent.SetVisibility` (`self.Door`) true false)
  (`SceneComponent.SetVisibility` (`self.ExitSign`) true false)
  (bind (_direction _alpha) (`Timeline|OpenDoor` :!via `PlayFromStart`)
    (:`Update`
      (`SceneComponent.K2_SetRelativeRotation` (`self.Door`) (`KismetMathLibrary.RInterpTo` (`SceneComponent.RelativeRotation` (`self.Door`)) (`self.EndDoorRot`) _alpha 1.0) false false))))

(fn `UserConstructionScript`)