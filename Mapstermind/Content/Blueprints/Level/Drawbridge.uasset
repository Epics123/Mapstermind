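; Drawbridge actor that, when RaiseBridge is triggered, lifts for a set uptime, then lowers again with sound.
; Raising first launches overlapping ThirdPersonCharacters toward left or right landing points by their Y position, using high-arc suggested projectile velocities.
; Characters entering the trigger box mid-raise also cause a throw, as GoingDown is set during the raise.
; Timelines drive RInterpTo rotation, and two boxes become blocking walls while up.
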(event `self.ReceiveBeginPlay`)

(event `RaiseBridge`
  (if (`self.Isdown`)
    (set `self.Isdown` false)
    (set `self.Going down` true)
    (`self.Throw Players`)
    (`GameplayStatics.PlaySoundAtLocation` "/Game/Audio/SoundEffects/DrawbridgeRaise.DrawbridgeRaise" (0.0 0.0 0.0) (struct) 1.0 1.0 0.0 null null null)
    (`KismetSystemLibrary.Delay` (`self.SoundDelay`))
    (`self.MoveBridgeUp`)
    (`KismetSystemLibrary.Delay` (`self.WallDelay`))
    (`self.Raise Walls`)
    (set `self.Going down` false)
    (`KismetSystemLibrary.Delay` (`self.Uptime`))
    (`GameplayStatics.PlaySoundAtLocation` "/Game/Audio/SoundEffects/DrawbridgeRaise.DrawbridgeRaise" (0.0 0.0 0.0) (struct) 1.0 1.0 0.0 null null null)
    (`KismetSystemLibrary.Delay` (`self.SoundDelay`))
    (`self.MoveBridgeDown`)
    (`self.Lower Walls`)
    (set `self.Isdown` true)))

(event `Raise Walls`
  (`PrimitiveComponent.SetCollisionEnabled` (`self.Box1`) "QueryAndPhysics")
  (`PrimitiveComponent.SetCollisionEnabled` (`self.Box2`) "QueryAndPhysics"))

(event `Throw Players`
  (for _array_element (`self.OverlappingPlayers`)
    (bind _returnvalue (`self.K2_GetActorLocation` _array_element))
    (if (<= (.y _returnvalue) (.y (`self.K2_GetActorLocation`)))
      (bind _tossvelocity (`GameplayStatics.BlueprintSuggestProjectileVelocity` _returnvalue (+ (* (`self.LandingLocationLeft`) (`self.LocationMultiplier`)) (`self.K2_GetActorLocation`)) (`self.LaunchSpeed`) 0.0 "DoNotTrace" 0.0 true))
      (`Character.LaunchCharacter` _array_element _tossvelocity true true)
      (else
        (bind _tossvelocity_2 (`GameplayStatics.BlueprintSuggestProjectileVelocity` _returnvalue (+ (* (`self.LandingLocationRight`) (`self.LocationMultiplier`)) (`self.K2_GetActorLocation`)) (`self.LaunchSpeed`) 0.0 "DoNotTrace" 0.0 true))
        (`Character.LaunchCharacter` _array_element _tossvelocity_2 true true)))))

(event `Lower Walls`
  (`PrimitiveComponent.SetCollisionEnabled` (`self.Box1`) "NoCollision")
  (`PrimitiveComponent.SetCollisionEnabled` (`self.Box2`) "NoCollision"))

(event `self.Box.OnComponentBeginOverlap`
  (params (OverlappedComponent :type "PrimitiveComponent Object Reference") (OtherActor :type "Actor Object Reference") (OtherComp :type "PrimitiveComponent Object Reference") (OtherBodyIndex :type Integer) (bFromSweep :type Boolean) (SweepResult :type "HitResult Structure (by ref)"))
  (bind _asthird_person_character (cast `/Game/Characters/ThirdPersonCharacter` OtherActor))
  (`KismetArrayLibrary.Array_Add` (`self.OverlappingPlayers`) _asthird_person_character)
  (if (`self.Going down`)
    (`self.Throw Players`)))

(event `self.Box.OnComponentEndOverlap`
  (params (OverlappedComponent :type "PrimitiveComponent Object Reference") (OtherActor :type "Actor Object Reference") (OtherComp :type "PrimitiveComponent Object Reference") (OtherBodyIndex :type Integer))
  (bind _asthird_person_character (cast `/Game/Characters/ThirdPersonCharacter` OtherActor))
  (`KismetArrayLibrary.Array_RemoveItem` (`self.OverlappingPlayers`) _asthird_person_character))

(event `MoveBridgeUp`
  (bind _drawbridge_base (`self.drawBridge_base`))
  (bind (_direction _alpha) (`Timeline|MoveDrawbridge` :!via `PlayFromStart`)
    (:`Update`
      (`SceneComponent.K2_SetRelativeRotation` _drawbridge_base (`KismetMathLibrary.RInterpTo` (`SceneComponent.RelativeRotation` _drawbridge_base) (`self.EndRotation`) _alpha 1.0) false false))))

(event `MoveBridgeDown`
  (bind _drawbridge_base (`self.drawBridge_base`))
  (bind (_direction _alpha) (`Timeline|Timeline_0` :!via `PlayFromStart`)
    (:`Update`
      (`SceneComponent.K2_SetRelativeRotation` _drawbridge_base (`KismetMathLibrary.RInterpTo` (`SceneComponent.RelativeRotation` _drawbridge_base) (`self.OriginalRotation`) _alpha 1.0) false false))))

(fn `UserConstructionScript`)