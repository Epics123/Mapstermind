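; LeverManager runs a two-lever pumping task that opens a TreasureChest and launches its goblet.
; On BeginPlay it registers itself with every AlternateLever and finds the chest.
; The first pull sets which lever starts, then valid pulls alternate between levers, each advancing the chest lid and turn count.
; Reaching PumpCount launches the goblet and calls IncrementTask, which is an empty stub here.
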(event `self.ReceiveBeginPlay`
  (bind _outactors (`GameplayStatics.GetAllActorsOfClass` "/Game/Blueprints/Tasks/AlternateLever.AlternateLever_C"))
  (for _array_element _outactors
    (set `/Game/Blueprints/Tasks/AlternateLever.Manager` self _array_element))
  (bind _returnvalue (`GameplayStatics.GetActorOfClass` "/Game/Blueprints/Tasks/TreasureChest.TreasureChest_C"))
  (set `self.Chest` _returnvalue))

(event `EnableMovement`
  (bind _playerref (`self.PlayerRef`))
  (`CharacterMovementComponent.SetMovementMode` (`Character.CharacterMovement` _playerref) "MOVE_Walking" 0)
  (set `CapstonePrototype1Character.PullingLever` false _playerref))

(event `FlipLever`
  (params (PulledLever :type "/Game/Blueprints/Tasks/AlternateLever Object Reference") (Pieceling :type "/Game/Characters/Piecelings/PiecelingBP Object Reference"))
  (bind _start_lever (`self.Start Lever`))
  (bind _follow_lever (`self.Follow Lever`))
  (`/Engine/EditorBlueprintResources/StandardMacros.IsValid` (`self.Start Lever`) ; Is this first pull?
    (:`Is Valid`
      _)
    (:`Is Not Valid`
      (`self.SetLevers` PulledLever Pieceling)))
  (if (`/Game/Blueprints/Tasks/AlternateLever.CurrentTurn` PulledLever)
    (`/Game/Blueprints/Tasks/AlternateLever.Activate` PulledLever)
    (set `CapstonePrototype1Character.PullingLever` true (`self.PlayerRef`))
    (`self.EnableMovement`)
    (`/Game/Blueprints/Tasks/TreasureChest.OpenTop` (`self.Chest`) (`self.Turn Count`))
    (bind _result (`/Engine/EditorBlueprintResources/StandardMacros.IncrementInt` (`self.Turn Count`))
      (:`  `
        (if (>= _result (`self.Pump Count`))
          (`/Game/Blueprints/Tasks/TreasureChest.LaunchGoblet` (`self.Chest`))
          (`self.IncrementTask`)
          (`self.EnableMovement`)
          (else
            (`KismetSystemLibrary.Delay` 0.2)
            (`/Game/Blueprints/Tasks/AlternateLever.ResetLeverPull` PulledLever)
            (set `/Game/Blueprints/Tasks/AlternateLever.CurrentTurn` (not (`/Game/Blueprints/Tasks/AlternateLever.CurrentTurn` _follow_lever)) _follow_lever)
            (set `/Game/Blueprints/Tasks/AlternateLever.CurrentTurn` (not (`/Game/Blueprints/Tasks/AlternateLever.CurrentTurn` _start_lever)) _start_lever)))))
    (else
      (`self.EnableMovement`))))

(event `SetLevers`
  (params (PassedLever :type "/Game/Blueprints/Tasks/AlternateLever Object Reference") (Pieceling :type "/Game/Characters/Piecelings/PiecelingBP Object Reference"))
  (`/Engine/EditorBlueprintResources/StandardMacros.IsValid` (`self.PlayerRef`)
    (:`Is Valid`
      _)
    (:`Is Not Valid`
      (set `self.PlayerRef` Pieceling)))
  (if (== PassedLever (`self.Lever1`))
    (bind _output_get (set `self.Start Lever` (`self.Lever1`)))
    (set `self.Follow Lever` (`self.Lever2`))
    (set `/Game/Blueprints/Tasks/AlternateLever.CurrentTurn` true _output_get)
    (else
      (bind _output_get_2 (set `self.Start Lever` (`self.Lever2`)))
      (set `self.Follow Lever` (`self.Lever1`))
      (set `/Game/Blueprints/Tasks/AlternateLever.CurrentTurn` true _output_get_2))))

(fn `CheckPulled`
  (returns (Pulled :type Boolean))
  (return false))

(fn `IncrementTask`)

(fn `UserConstructionScript`)