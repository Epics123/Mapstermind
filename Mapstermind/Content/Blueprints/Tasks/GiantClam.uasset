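; Giant clam task actor that receives hat and eyes items and is surrounded by a ring of clamlings.
; When a ClamHat or ClamEyes overlaps ItemTrigger, it calls that item's Place at HatPoint or EyePoint.
; The construction script spawns Clamling child actors radially from count, radius, angular offset and vertical offset, caching them with cube shadows off.
; GenerateClamlingSpawn is a similar position helper with an inverted angle ratio, not called in this graph.
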(event `self.ReceiveBeginPlay`)

(event `self.ItemTrigger.OnComponentBeginOverlap`
  (params (OverlappedComponent :type "PrimitiveComponent Object Reference") (OtherActor :type "Actor Object Reference") (OtherComp :type "PrimitiveComponent Object Reference") (OtherBodyIndex :type Integer) (bFromSweep :type Boolean) (SweepResult :type "HitResult Structure (by ref)"))
  (bind _asclam_hat (cast `/Game/Blueprints/Tasks/ClamHat` OtherActor)
    (:`then`
      (`/Game/Blueprints/Tasks/ClamHat.Place` _asclam_hat (`SceneComponent.K2_GetComponentLocation` (`self.HatPoint`))))
    (:`CastFailed`
      (bind _asclam_eyes (cast `/Game/Blueprints/Tasks/ClamEyes` OtherActor))
      (`/Game/Blueprints/Tasks/ClamEyes.Place` _asclam_eyes (`SceneComponent.K2_GetComponentLocation` (`self.EyePoint`))))))

(fn `GenerateClamlingSpawn`
  (params (Index :type Integer))
  (returns (SpawnPos :type "Vector Structure"))
  (locals (Angle :type "Float (double-precision)") (Pos :type "Vector Structure"))
  (bind _returnvalue (/ (`KismetMathLibrary.Conv_IntToDouble` (`self.ClamlingCount`)) 360.0))
  (bind _output_get (set `local.Pos` (`KismetMathLibrary.GreaterGreater_VectorRotator` (`KismetMathLibrary.MakeVector` (`self.SpawnRadius`)) (`KismetMathLibrary.MakeRotator` 0.0 0.0 (+ (* Index _returnvalue) (`KismetMathLibrary.MapRangeClamped` (`self.Offset`) 0.0 1.0 0.0 _returnvalue))))))
  (return _output_get))

(fn `UserConstructionScript`
  (bind _clamlingcount (`self.ClamlingCount`))
  (bind _returnvalue (/ 360.0 (`KismetMathLibrary.Conv_IntToDouble` _clamlingcount)))
  (`KismetArrayLibrary.Array_Clear` (`self.Clamlings`))
  (`KismetArrayLibrary.Array_Clear` (`self.ChildActors`))
  (for _index (range (+ _clamlingcount 1))
    (bind _returnvalue_2 (`AddComponent|NODE_AddChildActorComponent-1` :`RelativeTransform` (`KismetMathLibrary.MakeTransform` (- (`KismetMathLibrary.GreaterGreater_VectorRotator` (`KismetMathLibrary.MakeVector` (`self.SpawnRadius`)) (`KismetMathLibrary.MakeRotator` 0.0 0.0 (+ (* _index _returnvalue) (`KismetMathLibrary.MapRangeClamped` (`self.Offset`) 0.0 1.0 0.0 _returnvalue)))) (`KismetMathLibrary.MakeVector` 0.0 0.0 (`self.VerticalOffset`))))))
    (`ChildActorComponent.SetChildActorClass` _returnvalue_2 "/Game/Blueprints/Tasks/Clamling.Clamling_C")
    (`KismetArrayLibrary.Array_Add` (`self.ChildActors`) _returnvalue_2))
  (for _array_element (`self.ChildActors`)
    (bind _asclamling (cast `/Game/Blueprints/Tasks/Clamling` (`ChildActorComponent.ChildActor` _array_element)))
    (`KismetArrayLibrary.Array_Add` (`self.Clamlings`) _asclamling)
    (`PrimitiveComponent.SetCastShadow` (`/Game/Blueprints/Tasks/Clamling.Cube` _asclamling) false)))