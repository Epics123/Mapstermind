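; Pearl is a carriable task item that a PiecelingBP player can pick up, drop or place, tagged with the PEARL item type.
; Pickup attaches it to the player at a given location, sets it as HeldItem and calls OpenPearl on the level's MermaidTask.
; Drop detaches it and clears the player's item references.
; Place also positions it with a fixed rotation and disables its pickup sphere collision.
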(event `self.ReceiveBeginPlay`
  (set `self.itemType` "PEARL"))

(event `PickUp`
  (params (Parent :type "Actor Object Reference") (Location :type "Vector Structure"))
  (`self.K2_AttachToActor` Parent "None" "KeepWorld" "KeepWorld" "KeepWorld")
  (`self.K2_SetActorLocation` Location)
  (bind _aspieceling_bp (cast `/Game/Characters/Piecelings/PiecelingBP` Parent))
  (bind _output_get (set `self.Player` _aspieceling_bp))
  (set `/Game/Characters/Piecelings/PiecelingBP.HeldItem` self _output_get)
  (bind _returnvalue (`GameplayStatics.GetActorOfClass` "/Game/Blueprints/Tasks/MermaidTask.MermaidTask_C"))
  (`/Game/Blueprints/Tasks/MermaidTask.OpenPearl` _returnvalue))

(event `Drop`
  (bind _player (`self.Player`))
  (`self.K2_DetachFromActor` "KeepWorld" "KeepWorld" "KeepWorld")
  (set `/Game/Characters/Piecelings/PiecelingBP.HeldItem` null _player)
  (set `/Game/Characters/Piecelings/PiecelingBP.CurrentItem` null _player)
  (set `self.Player` null))

(event `Place`
  (params (Location :type "Vector Structure"))
  (bind _player (`self.Player`))
  (`self.K2_DetachFromActor` "KeepWorld" "KeepRelative" "KeepWorld")
  (`self.K2_SetActorLocation` Location)
  (`self.K2_SetActorRelativeRotation` (struct :`Yaw` 54.0))
  (`PrimitiveComponent.SetCollisionEnabled` (`self.PickUpSphere`) "NoCollision")
  (set `/Game/Characters/Piecelings/PiecelingBP.HeldItem` null _player)
  (set `/Game/Characters/Piecelings/PiecelingBP.CurrentItem` null _player)
  (set `self.Player` null))

(fn `UserConstructionScript`)