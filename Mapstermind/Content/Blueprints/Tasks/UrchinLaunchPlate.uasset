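; UrchinLaunchPlate is a pressure plate that launches its referenced Urchin when a falling PiecelingBP lands on it.
; A valid overlap disarms the plate, changes its material, plays a sound, then calls Launch on the Urchin after SoundDelay.
; ResetPlate, which nothing in this graph calls, waits out PlateCooldown and re-arms the plate with its Test material unless MultiDone is set.
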(event `self.PressurePlateCollision.OnComponentBeginOverlap`
  (params (OverlappedComponent :type "PrimitiveComponent Object Reference") (OtherActor :type "Actor Object Reference") (OtherComp :type "PrimitiveComponent Object Reference") (OtherBodyIndex :type Integer) (bFromSweep :type Boolean) (SweepResult :type "HitResult Structure (by ref)"))
  (bind _aspieceling_bp (cast `/Game/Characters/Piecelings/PiecelingBP` OtherActor))
  (if (`NavMovementComponent.IsFalling` (`Character.CharacterMovement` _aspieceling_bp))
    (if (`self.CanActivate`)
      (set `self.CanActivate` false)
      (set `self.Pressed` true)
      (`PrimitiveComponent.SetMaterial` (`self.PresurePlateMesh`) 0 null)
      (`GameplayStatics.PlaySoundAtLocation` "/Game/Audio/SoundEffects/Pressure_Plate.Pressure_Plate" (0.0 0.0 0.0) (struct) 1.0 1.0 0.0 null null null)
      (`KismetSystemLibrary.Delay` (`self.SoundDelay`))
      (`/Game/Blueprints/Tasks/SeaUrchin.Launch` (`self.Urchin`)))))

(event `ResetPlate`
  (`KismetSystemLibrary.Delay` (`self.PlateCooldown`))
  (if (not (`self.MultiDone`))
    (set `self.CanActivate` true)
    (set `self.Pressed` false)
    (`PrimitiveComponent.SetMaterial` (`self.PresurePlateMesh`) 0 "/Game/Materials/Test/Test.Test")))

(fn `UserConstructionScript`)