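; FollowerLever is the follower half of a paired lever task, where pulls alternate with a partner lever.
; When pulled on its active turn, it swaps to a pulled mesh, disables activation and hides the pull prompt on its HUD widget.
; It then hands the lead back to PartnerLever, or on the last turn triggers the partner's final turn and restores player walking.
; TradeFollow and ResetLeverPull re-arm it.
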(event `self.ReceiveBeginPlay`
  (`parent.ReceiveBeginPlay`))

(event `EnableMovement`)

(event `self.Activate_Lever_Pull`
  (bind _playerref (`self.PlayerRef`))
  (`KismetSystemLibrary.PrintString` "PUSH")
  (if (`self.ActiveTurn`)
    (set `self.Pulled` true)
    (`StaticMeshComponent.SetStaticMesh` (`self.LeverMesh`) "/Game/ArtAssets/Tasks/leverPiecelingPos2.leverPiecelingPos2")
    (set `self.CanActivate` false)
    (bind _aslever_hud (cast `/Game/Blueprints/Widgets/Level/LeverHUD` (`WidgetComponent.GetWidget` (`self.Widget`))))
    (`/Game/Blueprints/Widgets/Level/LeverHUD.HidePull` _aslever_hud)
    (if (`self.LastTurn`)
      (`/Game/Blueprints/Tasks/LeadingLever.FinalTurn` (`self.PartnerLever`))
      (`/Engine/EditorBlueprintResources/StandardMacros.IsValid` _playerref
        (:`Is Valid`
          (`CharacterMovementComponent.SetMovementMode` (`Character.CharacterMovement` _playerref) "MOVE_Walking" 0)
          (set `CapstonePrototype1Character.PullingLever` false _playerref)
          (`KismetSystemLibrary.PrintString` "Follow Final")))
      (else
        (`/Game/Blueprints/Tasks/LeadingLever.TradeLead` (`self.PartnerLever`))))))

(event `self.Reset_Lever_Pull`
  (set `self.ActiveTurn` true :!label _label)
  (set `self.Pulled` false)
  (`StaticMeshComponent.SetStaticMesh` (`self.LeverMesh`) "/Game/ArtAssets/Tasks/leverPiecelingFull.leverPiecelingFull")
  (set `self.CanActivate` true))

(event `TradeFollow`
  (params (LastTurn :type Boolean))
  (goto _label))

(fn `EnableMovement_0`)

(fn `UserConstructionScript`
  (`parent.UserConstructionScript`))