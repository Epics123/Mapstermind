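; Crown pickup item for the mermaid task, tagged with the crown item type when play begins.
; On pickup, if not already grabbed, it disables its mesh collision, attaches to the grabbing actor at the given location and tells the level's MermaidTask to open the crown.
; Dropping detaches it, clears the grabbed flag and tells MermaidTask to close the crown, without re-enabling collision.
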(event `self.ReceiveBeginPlay`
  (set `self.itemType` "CROWN"))

(event `Pickup`
  (params (Parent :type "Actor Object Reference") (Location :type "Vector Structure"))
  (if (not (`self.Grabbed`))
    (`PrimitiveComponent.SetCollisionEnabled` (`self.CrownMesh`) "NoCollision")
    (`self.K2_AttachToActor` Parent "None" "KeepWorld" "KeepWorld" "KeepWorld")
    (`self.K2_SetActorLocation` Location)
    (bind _returnvalue (`GameplayStatics.GetActorOfClass` "/Game/Blueprints/Tasks/MermaidTask.MermaidTask_C"))
    (`/Game/Blueprints/Tasks/MermaidTask.OpenCrown` _returnvalue)
    (set `self.Grabbed` true)))

(event `Drop`
  (`self.K2_DetachFromActor` "KeepWorld" "KeepWorld" "KeepWorld")
  (set `self.Grabbed` false)
  (bind _returnvalue (`GameplayStatics.GetActorOfClass` "/Game/Blueprints/Tasks/MermaidTask.MermaidTask_C"))
  (`/Game/Blueprints/Tasks/MermaidTask.CloseCrown` _returnvalue))

(fn `UserConstructionScript`)