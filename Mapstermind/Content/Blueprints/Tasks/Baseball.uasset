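; Baseball task item that a Pieceling picks up and throws at the Stadium to advance its event task.
; Pickup attaches it to the carrier, opens the Stadium, enables throwing and hides the screen-space prompt widget.
; Throw detaches it, clears the holder's item, then a timeline lerps the mesh along a parabolic arc and increments the Stadium task on landing.
; Reset respawns a fresh ball at the starting location.
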(event `self.ReceiveBeginPlay`
  (bind _returnvalue (`GameplayStatics.GetActorOfClass` "/Game/Blueprints/Tasks/Stadium.Stadium_C"))
  (`/Engine/EditorBlueprintResources/StandardMacros.IsValid` _returnvalue
    (:`Is Valid`
      (set `self.Stadium` _returnvalue)
      (set `self.OrigLocation` (`self.K2_GetActorLocation`))
      (bind _aspickup_ui (cast `/Game/Blueprints/Widgets/UITextures/Tutorial/Final/Piecelings/PickupUI` (`WidgetComponent.GetWidget` (`self.PickupWidget`))))
      (set `self.PickupUI` _aspickup_ui)
      (`WidgetComponent.SetWidgetSpace` (`self.PickupWidget`) "Screen"))))

(event `PickupUI_Visible`
  (`SceneComponent.SetVisibility` (`self.PickupWidget`) true false)
  (`/Game/Blueprints/Widgets/UITextures/Tutorial/Final/Piecelings/PickupUI.PlayAnim` (`self.PickupUI`)))

(event `PickupUI_Invisible`
  (`SceneComponent.SetVisibility` (`self.PickupWidget`) false false)
  (`/Game/Blueprints/Widgets/UITextures/Tutorial/Final/Piecelings/PickupUI.StopAnim` (`self.PickupUI`)))

(event `self.ReceiveTick`
  (params (DeltaSeconds :type "Float (single-precision)")))

(event `PickUp`
  (params (Parent :type "Actor Object Reference") (Location :type "Vector Structure"))
  (bind _stadium (`self.Stadium`))
  (if (`self.CanPickUp`)
    (`self.K2_AttachToActor` Parent "None" "KeepWorld" "KeepWorld" "KeepWorld")
    (`self.K2_SetActorLocation` Location)
    (`/Engine/EditorBlueprintResources/StandardMacros.IsValid` _stadium
      (:`Is Valid`
        (`/Game/Blueprints/Tasks/Stadium.OpenStadium` _stadium)
        (set `self.CanThrow` true)
        (`self.PickupUI_Invisible`)))))

(event `Throw`
  (if (`self.CanThrow`)
    (set `self.CanThrow` false)
    (`self.K2_DetachFromActor` "KeepWorld" "KeepWorld" "KeepWorld")
    (bind _aspieceling_bp (cast `/Game/Characters/Piecelings/PiecelingBP` (`self.GetParentActor`))
      (:`then`
        (set `/Game/Characters/Piecelings/PiecelingBP.HeldItem` null _aspieceling_bp))
      (:`CastFailed`
        _))
    (set `self.OriginalHeight` (.z (`self.K2_GetActorLocation`)))
    (`KismetMathLibrary.Vector_Set` (`self.StadiumLocation`) (- (.x (`self.K2_GetActorLocation` (`self.Stadium`))) 300.0) (- (.y (`self.K2_GetActorLocation` (`self.Stadium`))) 300.0) (.z (`self.K2_GetActorLocation` (`self.Stadium`))))
    (bind (_direction _deltatime) (`Timeline|LERP Timeline` :!via `PlayFromStart`)
      (:`Update`
        ;[0 0.9838 1] Lerping the Baseball
        (`KismetMathLibrary.Vector_Set` (`self.ThrowLocVec`) (`KismetMathLibrary.Lerp` (.x (`SceneComponent.K2_GetComponentLocation` (`self.StaticMesh`))) (.x (`self.StadiumLocation`)) _deltatime) (`KismetMathLibrary.Lerp` (.y (`SceneComponent.K2_GetComponentLocation` (`self.StaticMesh`))) (.y (`self.StadiumLocation`)) _deltatime) (+ (+ (`self.ThrowHeight`) (* (* (`self.ThrowHeight`) -4.0) (`KismetMathLibrary.MultiplyMultiply_FloatFloat` (* (+ _deltatime -0.07) 7.0) 2.0))) (`self.OriginalHeight`)))
        (`SceneComponent.K2_SetWorldLocation` (`self.StaticMesh`) (`self.ThrowLocVec`) false false))
      (:`Finished`
        ;[0.943 0.08227 1] Completing the Task
        (if (not (`self.ThrowFinished`))
          (set `self.ThrowFinished` true)
          (`/Game/Blueprints/Tasks/Stadium.EventTaskIncrement` (`self.Stadium`))
          (`SceneComponent.K2_SetWorldLocation` (`self.StaticMesh`) (`self.StadiumLocation`) false false)
          (`self.K2_SetActorLocation` (`self.StadiumLocation`)))))))

(event `Reset ball`
  (`|SpawnActorFromClass` "/Temp/Diff/temp-c2493c6c506271c24487b8b5cd67bcf2923aad5c-Baseball.Baseball_C" (`KismetMathLibrary.MakeTransform` (`self.OrigLocation`)) "Undefined" "OverrideRootScale" null null)
  (`self.K2_DestroyActor`))

(event `Drop`
  (params (Parent :type "Actor Object Reference"))
  (bind _aspieceling_bp (cast `/Game/Characters/Piecelings/PiecelingBP` Parent))
  (`self.K2_DetachFromActor` _aspieceling_bp "KeepWorld" "KeepWorld" "KeepWorld")
  (set `/Game/Characters/Piecelings/PiecelingBP.HeldItem` null _aspieceling_bp))

(fn `UserConstructionScript`)