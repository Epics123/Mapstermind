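; MultiLever is a task that completes once its three child SingleLever actors are all pulled at the same time.
; Tick polls the levers, mirrors each on a TaskIndicator light, and fires completion once through a DoOnce.
; Completion disables the levers' activation, collision and widgets, then sets every Pieceling to walking.
; It also increments the GameMode task message and advances the TutorialController if one is found.
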(event `self.ReceiveBeginPlay`
  (bind _assingle_lever (cast `/Game/Blueprints/Tasks/SingleLever` (`ChildActorComponent.ChildActor` (`self.ChildActor`))))
  (set `self.Lever1` _assingle_lever)
  (bind _assingle_lever_2 (cast `/Game/Blueprints/Tasks/SingleLever` (`ChildActorComponent.ChildActor` (`self.ChildActor1`))))
  (set `self.Lever2` _assingle_lever_2)
  (bind _assingle_lever_3 (cast `/Game/Blueprints/Tasks/SingleLever` (`ChildActorComponent.ChildActor` (`self.ChildActor2`))))
  (set `self.Lever3` _assingle_lever_3)
  (set `/Game/Blueprints/Tasks/SingleLever.IsMulti` true (`self.Lever1`))
  (set `/Game/Blueprints/Tasks/SingleLever.IsMulti` true (`self.Lever2`))
  (set `/Game/Blueprints/Tasks/SingleLever.IsMulti` true (`self.Lever3`))
  (bind _returnvalue (`GameplayStatics.GetActorOfClass` "/Game/Blueprints/Tutorial/TutorialController.TutorialController_C"))
  (set `self.TutorialController` _returnvalue))

(event `self.CompleteTask`
  (bind _lever1 (`self.Lever1`))
  (bind _lever2 (`self.Lever2`))
  (bind _tutorialcontroller (`self.TutorialController`))
  (bind _lever3 (`self.Lever3`))
  (set `Lever.CanActivate` false _lever1)
  (`PrimitiveComponent.SetCollisionEnabled` (`/Game/Blueprints/Tasks/SingleLever.DetectionSphere` _lever1) "NoCollision")
  (`SceneComponent.SetVisibility` (`/Game/Blueprints/Tasks/SingleLever.Widget` _lever1) false false)
  (set `Lever.CanActivate` false _lever2)
  (`PrimitiveComponent.SetCollisionEnabled` (`/Game/Blueprints/Tasks/SingleLever.DetectionSphere` _lever2) "NoCollision")
  (`SceneComponent.SetVisibility` (`/Game/Blueprints/Tasks/SingleLever.Widget` _lever2) false false)
  (set `Lever.CanActivate` false _lever3)
  (`PrimitiveComponent.SetCollisionEnabled` (`/Game/Blueprints/Tasks/SingleLever.DetectionSphere` _lever3) "NoCollision")
  (`SceneComponent.SetVisibility` (`/Game/Blueprints/Tasks/SingleLever.Widget` _lever3) false false)
  (message `/Game/Blueprints/Modes_States/LocalMPGameModeInterface.IncrementTask` (`GameplayStatics.GetGameMode`))
  (set `self.Completed` true)
  (bind _outactors (`GameplayStatics.GetAllActorsOfClass` "/Game/Characters/Piecelings/PiecelingBP.PiecelingBP_C"))
  (for _array_element _outactors
    (`CharacterMovementComponent.SetMovementMode` (`Character.CharacterMovement` _array_element) "MOVE_Walking" 0))
  (`/Engine/EditorBlueprintResources/StandardMacros.IsValid` _tutorialcontroller
    (:`Is Valid`
      (`/Game/Blueprints/Tutorial/TutorialController.IncrementTask` _tutorialcontroller 0))))

(event `self.ReceiveTick`
  (params (DeltaSeconds :type "Float (single-precision)"))
  (`self.SetIndicatorLights` (`self.Completed`))
  (if (and (`/Game/Blueprints/Tasks/SingleLever.Pulled` (`self.Lever1`)) (`/Game/Blueprints/Tasks/SingleLever.Pulled` (`self.Lever2`)) (`/Game/Blueprints/Tasks/SingleLever.Pulled` (`self.Lever3`)))
    (`/Engine/EditorBlueprintResources/StandardMacros.DoOnce` false
      (:`Completed`
        (`self.CompleteTask`)
        (`/Game/Blueprints/Tasks/TaskTripleIndicator.CompleteTask` (`self.TaskIndicator`))))))

(fn `SetIndicatorLights`
  (params (Complete :type Boolean))
  (bind _taskindicator (`self.TaskIndicator`))
  (bind _taskindicator_2 (`self.TaskIndicator`))
  (bind _taskindicator_3 (`self.TaskIndicator`))
  (if (not Complete)
    (`|ExecutionSequence`
      (:`then_0`
        (if (`/Game/Blueprints/Tasks/SingleLever.Pulled` (`self.Lever1`))
          (`/Game/Blueprints/Tasks/TaskTripleIndicator.ActivateLight` _taskindicator_3 3)
          (else
            (`/Game/Blueprints/Tasks/TaskTripleIndicator.DeactivateLight` _taskindicator_3 3))))
      (:`then_1`
        (if (`/Game/Blueprints/Tasks/SingleLever.Pulled` (`self.Lever2`))
          (`/Game/Blueprints/Tasks/TaskTripleIndicator.ActivateLight` _taskindicator 0)
          (else
            (`/Game/Blueprints/Tasks/TaskTripleIndicator.DeactivateLight` _taskindicator 0))))
      (:`then_2`
        (if (`/Game/Blueprints/Tasks/SingleLever.Pulled` (`self.Lever3`))
          (`/Game/Blueprints/Tasks/TaskTripleIndicator.ActivateLight` _taskindicator_2 2)
          (else
            (`/Game/Blueprints/Tasks/TaskTripleIndicator.DeactivateLight` _taskindicator_2 2)))))))

(fn `UserConstructionScript`)