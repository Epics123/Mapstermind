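; Multiplayer task pressure plate that completes when a required number of third-person characters land on it while falling, within its overlap at the same time.
; Falling overlaps build a unique character list whose count drives the indicator lights; an insufficient count schedules a short timer to reset count and lights.
; Completion fires once, playing a sound, incrementing the game mode's task message, completing the TaskIndicator and flipping an optional linked Pipe.
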(event `self.PressurePlateCollision.OnComponentBeginOverlap`
  (params (OverlappedComponent :type "PrimitiveComponent Object Reference") (OtherActor :type "Actor Object Reference") (OtherComp :type "PrimitiveComponent Object Reference") (OtherBodyIndex :type Integer) (bFromSweep :type Boolean) (SweepResult :type "HitResult Structure (by ref)"))
  (bind _pipe (`self.Pipe`))
  (bind _overlapingcharacters (`self.OverlapingCharacters`))
  (bind _asthird_person_character (cast `/Game/Characters/ThirdPersonCharacter` OtherActor))
  (if (`NavMovementComponent.IsFalling` (`Character.CharacterMovement` _asthird_person_character))
    (`KismetArrayLibrary.Array_AddUnique` _overlapingcharacters _asthird_person_character)
    (bind _output_get (set `self.NumPlayers` (`KismetArrayLibrary.Array_Length` _overlapingcharacters)))
    (if (not (`self.Complete`))
      (`self.TaskLigts` _output_get)
      (if (and (`self.CanActivate`) (== (`self.NumPlayers`) (`self.MaxPlayersToActivate`)))
        (`/Engine/EditorBlueprintResources/StandardMacros.DoOnce` false
          (:`Completed`
            (set `self.CanActivate` false)
            (`GameplayStatics.PlaySoundAtLocation` "/Game/Audio/SoundEffects/Pressure_Plate.Pressure_Plate" (0.0 0.0 0.0) (struct) 1.0 1.0 0.0 null null null)
            (set `self.Complete` true)
            (bind _completedtasknum (message `/Game/Blueprints/Modes_States/LocalMPGameModeInterface.IncrementTask` (`GameplayStatics.GetGameMode`)))
            (`KismetSystemLibrary.PrintString` (`KismetStringLibrary.Conv_IntToString` _completedtasknum))
            (`/Game/Blueprints/Tasks/TaskTripleIndicator.CompleteTask` (`self.TaskIndicator`))
            (`/Engine/EditorBlueprintResources/StandardMacros.IsValid` _pipe
              (:`Is Valid`
                (`/Game/Blueprints/Tasks/SewerPipeTask.FlipModel` _pipe)))))
        (else
          (`KismetSystemLibrary.K2_SetTimerDelegate` (delegate `ResetNumPlayers`) 0.1))))
    (else
      (set `self.NumPlayers` 0))))

(event `self.PressurePlateCollision.OnComponentEndOverlap`
  (params (OverlappedComponent :type "PrimitiveComponent Object Reference") (OtherActor :type "Actor Object Reference") (OtherComp :type "PrimitiveComponent Object Reference") (OtherBodyIndex :type Integer))
  (bind _overlapingcharacters (`self.OverlapingCharacters`))
  (bind _asthird_person_character (cast `/Game/Characters/ThirdPersonCharacter` OtherActor))
  (`KismetArrayLibrary.Array_RemoveItem` _overlapingcharacters _asthird_person_character)
  (set `self.NumPlayers` (`KismetArrayLibrary.Array_Length` _overlapingcharacters)))

(event `ResetNumPlayers`
  (set `self.NumPlayers` 0)
  (`/Game/Blueprints/Tasks/TaskTripleIndicator.DeactivateLight` (`self.TaskIndicator`) 0)
  (`/Game/Blueprints/Tasks/TaskTripleIndicator.DeactivateLight` (`self.TaskIndicator`) 2)
  (`/Game/Blueprints/Tasks/TaskTripleIndicator.DeactivateLight` (`self.TaskIndicator`) 3))

(event `TaskLigts`
  (params (Num :type Integer))
  (if (== Num 1)
    (`/Game/Blueprints/Tasks/TaskTripleIndicator.ActivateLight` (`self.TaskIndicator`) 0)))

(fn `UserConstructionScript`)