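; Pressure plate task actor that triggers when a PiecelingBP overlaps it while falling, such as landing from a jump.
; A press changes the plate material and locks out further presses.
; In single mode it plays a sound, then after a delay increments the game mode's task message, marks itself completed and flips an optional linked Pipe.
; Otherwise it re-arms after a cooldown unless MultiDone is set.
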(event `self.PressurePlateCollision.OnComponentBeginOverlap`
  (params (OverlappedComponent :type "PrimitiveComponent Object Reference") (OtherActor :type "Actor Object Reference") (OtherComp :type "PrimitiveComponent Object Reference") (OtherBodyIndex :type Integer) (bFromSweep :type Boolean) (SweepResult :type "HitResult Structure (by ref)"))
  (bind _asthird_person_character (cast `/Game/Characters/Piecelings/PiecelingBP` OtherActor))
  (if (`NavMovementComponent.IsFalling` (`Character.CharacterMovement` _asthird_person_character))
    (if (`self.CanActivate`)
      (set `self.Completed` false)
      (set `self.CanActivate` false)
      (set `self.Pressed` true)
      (`self.CompleteTask`))))

(event `self.CompleteTask`
  (bind _pipe (`self.Pipe`))
  (`PrimitiveComponent.SetMaterial` (`self.PresurePlateMesh`) 0 null)
  (if (`self.IsSingle`)
    (`GameplayStatics.PlaySoundAtLocation` "/Game/Audio/SoundEffects/Pressure_Plate.Pressure_Plate" (0.0 0.0 0.0) (struct) 1.0 1.0 0.0 null null null)
    (`KismetSystemLibrary.Delay` (`self.SoundDelay`))
    (message `/Game/Blueprints/Modes_States/LocalMPGameModeInterface.IncrementTask` (`GameplayStatics.GetGameMode`))
    (set `self.Completed` true)
    (`/Engine/EditorBlueprintResources/StandardMacros.IsValid` _pipe
      (:`Is Valid`
        (`/Game/Blueprints/Tasks/SewerPipeTask.FlipModel` _pipe)))
    (else
      (`self.ResetPlate`))))

(event `ResetPlate`
  (`KismetSystemLibrary.Delay` (`self.PlateCooldown`))
  (if (not (`self.MultiDone`))
    (set `self.CanActivate` true)
    (set `self.Pressed` false)
    (`PrimitiveComponent.SetMaterial` (`self.PresurePlateMesh`) 0 "/Game/Materials/Test/Test.Test")))

(fn `UserConstructionScript`)