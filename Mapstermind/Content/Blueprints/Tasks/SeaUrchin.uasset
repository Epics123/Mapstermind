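; Sea urchin task actor whose mesh pops up in a vertical arc when launched, then resets its linked Plate.
; Launch stores the actor's starting location and plays a timeline that feeds a quadratic formula, scaled by LaunchHeight, to set the mesh's height while X and Y follow the actor.
; When the timeline finishes, the mesh snaps back to its original location and ResetPlate is called on the Plate.
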(event `Launch`
  (set `self.Original Height` (.z (`self.K2_GetActorLocation`)))
  (set `self.OriginalLocation` (`self.K2_GetActorLocation`))
  (bind (_direction _deltatime) (`Timeline|Lerp Timeline` :!via `PlayFromStart`)
    (:`Update`
      (`KismetMathLibrary.Vector_Set` (`self.LaunchLocVector`) (.x (`self.K2_GetActorLocation`)) (.y (`self.K2_GetActorLocation`)) (+ (+ (`self.Launch Height`) (* (* (`self.Launch Height`) -4.0) (`KismetMathLibrary.MultiplyMultiply_FloatFloat` (* (+ _deltatime -0.07) 7.0) 2.0))) (`self.Original Height`)))
      (`SceneComponent.K2_SetWorldLocation` (`self.StaticMesh`) (`self.LaunchLocVector`) false false))
    (:`Finished`
      (`SceneComponent.K2_SetWorldLocation` (`self.StaticMesh`) (`self.OriginalLocation`) false false)
      (`/Game/Blueprints/Tasks/UrchinLaunchPlate.ResetPlate` (`self.Plate`)))))

(fn `UserConstructionScript`)