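; Tutorial baseball task actor that gets picked up and thrown at the TutorialStadium to complete its task.
; Pickup attaches it to the carrier and calls OpenStadium.
; Throw runs a timeline toward an offset stadium point, though the lerp alpha is fixed at zero, then completes the task and destroys the ball.
; Drop detaches the passed Pieceling, then resets by calling OpenStadium, spawning a replacement and destroying itself.
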(event `self.ReceiveBeginPlay`
  (bind _returnvalue (`GameplayStatics.GetActorOfClass` "/Game/Blueprints/Tutorial/Tasks/TutorialStadium.TutorialStadium_C"))
  (`/Engine/EditorBlueprintResources/StandardMacros.IsValid` _returnvalue
    (:`Is Valid`
      (set `self.Stadium` _returnvalue)
      (set `self.OrigLocation` (`self.K2_GetActorLocation`)))))

(event `self.ReceiveTick`
  (params (DeltaSeconds :type "Float (single-precision)")))

(event `PickUp`
  (params (Parent :type "Actor Object Reference") (Location :type "Vector Structure"))
  (bind _stadium (`self.Stadium`))
  (if (`self.CanPickUp`)
    (`self.K2_AttachToActor` Parent "None" "KeepWorld" "KeepWorld" "KeepWorld")
    (`self.K2_SetActorLocation` Location)
    (`/Engine/EditorBlueprintResources/StandardMacros.IsValid` _stadium
      (:`Is Valid`
        (`/Game/Blueprints/Tutorial/Tasks/TutorialStadium.OpenStadium` _stadium)))))

(event `Throw`
  (if (`self.CanThrow`)
    (`self.K2_DetachFromActor` "KeepWorld" "KeepWorld" "KeepWorld")
    (`KismetMathLibrary.Vector_Set` (`self.StadiumLocation`) (- (.x (`self.K2_GetActorLocation` (`self.Stadium`))) 300.0) (- (.y (`self.K2_GetActorLocation` (`self.Stadium`))) 300.0) (.z (`self.K2_GetActorLocation` (`self.Stadium`))))
    (`Timeline|LERP Timeline`
      (:`Update`
        ;[0 0.9838 1] Lerping the Baseball
        (`SceneComponent.K2_SetWorldLocation` (`self.StaticMesh`) (`KismetMathLibrary.VLerp` (`SceneComponent.K2_GetComponentLocation` (`self.StaticMesh`)) (`self.StadiumLocation`)) false false))
      (:`Finished`
        ;[0.943 0.08227 1] Completing the Task
        (`Task.CompleteTask` (`self.Stadium`))
        (`self.K2_DestroyActor`)))))

(event `Reset ball`
  (bind _stadium (`self.Stadium`))
  (`/Game/Blueprints/Tutorial/Tasks/TutorialStadium.OpenStadium` _stadium)
  (`/Game/Blueprints/Tutorial/Tasks/TutorialStadium.SpawnBall` _stadium)
  (`self.K2_DestroyActor`))

(event `Drop`
  (params (Parent :type "Actor Object Reference"))
  (bind _aspieceling_bp (cast `/Game/Characters/Piecelings/PiecelingBP` Parent))
  (`self.K2_DetachFromActor` _aspieceling_bp "KeepWorld" "KeepWorld" "KeepWorld")
  (`self.Reset ball`))

(fn `UserConstructionScript`)