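; Lever task actor that a Pieceling grabs and pulls, registering the pull only when it is this lever's turn.
; An overlap sphere links one Pieceling to the lever and toggles the LeverHUD prompt, while ActivateLever freezes its movement.
; Activate passes a DoOnce to play a thunk and, on its turn, swap the mesh, set Pulled and restore movement.
; ResetLeverPull re-arms the lever, and CheckPulled exposes its state.
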(event `ResetLeverPull`
  (set `self.Pulled` false)
  (set `self.CanActivate` true)
  (`StaticMeshComponent.SetStaticMesh` (`self.LeverMesh`) "/Game/ArtAssets/LevelCity/Props/Mesh/leverPiecelingPos1.leverPiecelingPos1")
  (goto _label :!via `Reset`))

(event `self.ReceiveBeginPlay`
  (`PrimitiveComponent.SetCastShadow` (`self.Widget`) false))

(event `Activate`
  (`/Engine/EditorBlueprintResources/StandardMacros.DoOnce` false :!label _label
    (:`Completed`
      (`GameplayStatics.PlaySoundAtLocation` "/Game/Audio/SoundEffects/Thunk.Thunk" (0.0 0.0 0.0) (struct) 0.7 1.0 0.0 null null null)
      (if (`self.CurrentTurn`)
        (set `self.Pulled` true)
        (`StaticMeshComponent.SetStaticMesh` (`self.LeverMesh`) "/Game/ArtAssets/LevelCity/Props/Mesh/leverPiecelingPos2.leverPiecelingPos2")
        (set `self.CanActivate` false)
        (`self.EnableMovement`)
        (bind _aslever_hud (cast `/Game/Blueprints/Widgets/Level/LeverHUD` (`WidgetComponent.GetWidget` (`self.Widget`))))
        (`/Game/Blueprints/Widgets/Level/LeverHUD.HidePull` _aslever_hud)
        (set `self.CurrentTurn` false)))))

(event `self.ReceiveTick`
  (params (DeltaSeconds :type "Float (single-precision)")))

(event `IncrementTask`
  (message `/Game/Blueprints/Modes_States/LocalMPGameModeInterface.IncrementTask` (`GameplayStatics.GetGameMode`)))

(event `EnableMovement`
  (bind _playerref (`self.PlayerRef`))
  (`/Engine/EditorBlueprintResources/StandardMacros.IsValid` _playerref
    (:`Is Valid`
      (`CharacterMovementComponent.SetMovementMode` (`Character.CharacterMovement` _playerref) "MOVE_Walking" 0)
      (set `CapstonePrototype1Character.PullingLever` false _playerref))))

(event `self.ActivateLever`
  (params (Character :type "CapstonePrototype1Character Object Reference"))
  (`CharacterMovementComponent.DisableMovement` (`Character.CharacterMovement` Character))
  (set `self.CanActivate` false)
  (bind _aspieceling_bp (cast `/Game/Characters/Piecelings/PiecelingBP` Character))
  (set `self.PlayerRef` _aspieceling_bp))

(event `self.DetectionSphere.OnComponentBeginOverlap`
  (params (OverlappedComponent :type "PrimitiveComponent Object Reference") (OtherActor :type "Actor Object Reference") (OtherComp :type "PrimitiveComponent Object Reference") (OtherBodyIndex :type Integer) (bFromSweep :type Boolean) (SweepResult :type "HitResult Structure (by ref)"))
  (bind _aspieceling_bp (cast `/Game/Characters/Piecelings/PiecelingBP` OtherActor))
  (`/Engine/EditorBlueprintResources/StandardMacros.IsValid` (`self.PlayerRef`)
    (:`Is Not Valid`
      (set `/Game/Characters/Piecelings/PiecelingBP.CurrentLever` self _aspieceling_bp)
      (set `self.PlayerRef` _aspieceling_bp)
      (if (`self.CanActivate`)
        (bind _aslever_hud (cast `/Game/Blueprints/Widgets/Level/LeverHUD` (`WidgetComponent.GetWidget` (`self.Widget`))))
        (`/Game/Blueprints/Widgets/Level/LeverHUD.ShowGrab` _aslever_hud)))))

(event `self.DetectionSphere.OnComponentEndOverlap`
  (params (OverlappedComponent :type "PrimitiveComponent Object Reference") (OtherActor :type "Actor Object Reference") (OtherComp :type "PrimitiveComponent Object Reference") (OtherBodyIndex :type Integer))
  (bind _aspieceling_bp (cast `/Game/Characters/Piecelings/PiecelingBP` OtherActor))
  (set `/Game/Characters/Piecelings/PiecelingBP.CurrentLever` null _aspieceling_bp)
  (set `self.PlayerRef` null)
  (bind _aslever_hud (cast `/Game/Blueprints/Widgets/Level/LeverHUD` (`WidgetComponent.GetWidget` (`self.Widget`))))
  (`/Game/Blueprints/Widgets/Level/LeverHUD.HidePull` _aslever_hud))

(fn `CheckPulled`
  (returns (Pulled :type Boolean))
  (return (`self.Pulled`)))

(fn `UserConstructionScript`)