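; Single pull-lever task actor that plays a thunk when activated, with a DoOnce guarding against repeat pulls.
; In multi mode it swaps to the pulled mesh, disables activation, hides the HUD pull prompt and starts a cooldown timer that resets the lever and DoOnce.
; Otherwise it increments the task, clears the player's lever-pulled flag and restores walking movement after a short timer.
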(event `ResetLeverPull`
  (set `self.Pulled` false :!label _label)
  (set `self.CanActivate` true)
  (`StaticMeshComponent.SetStaticMesh` (`self.LeverMesh`) "/Game/ArtAssets/Tasks/leverPiecelingFull.leverPiecelingFull")
  (goto _label_2 :!via `Reset`))

(event `self.Reset_Lever_Pull`
  (goto _label))

(event `self.Activate_Lever_Pull`
  (`/Engine/EditorBlueprintResources/StandardMacros.DoOnce` false :!label _label_2
    (:`Completed`
      (`GameplayStatics.PlaySoundAtLocation` "/Game/Audio/SoundEffects/Thunk.Thunk" (0.0 0.0 0.0) (struct) 0.7 1.0 0.0 null null null)
      (if (`self.IsMulti`)
        (set `self.Pulled` true)
        (`StaticMeshComponent.SetStaticMesh` (`self.LeverMesh`) "/Game/ArtAssets/Tasks/leverPiecelingPos2.leverPiecelingPos2")
        (`KismetSystemLibrary.K2_SetTimerDelegate` (delegate `ResetLeverPull`) (`self.LeverCooldown`))
        (set `self.CanActivate` false)
        (`self.EnableMovement_0`)
        (bind _aslever_hud (cast `/Game/Blueprints/Widgets/Level/LeverHUD` (`WidgetComponent.GetWidget` (`self.Widget`))))
        (`/Game/Blueprints/Widgets/Level/LeverHUD.HidePull` _aslever_hud)
        (else
          (`self.IncrementTask`)
          (set `/Game/Characters/Piecelings/PiecelingBP.LeverPulled` false (`self.PlayerRef`))
          (`KismetSystemLibrary.K2_SetTimerDelegate` (delegate `EnableMovement`) 1.0))))))

(event `EnableMovement`
  (bind _playerref (`self.PlayerRef`))
  (`/Engine/EditorBlueprintResources/StandardMacros.IsValid` _playerref
    (:`Is Valid`
      (`CharacterMovementComponent.SetMovementMode` (`Character.CharacterMovement` _playerref) "MOVE_Walking" 0)
      (set `CapstonePrototype1Character.PullingLever` false _playerref))))

(fn `EnableMovement_0`)

(fn `UserConstructionScript`
  (`parent.UserConstructionScript`))