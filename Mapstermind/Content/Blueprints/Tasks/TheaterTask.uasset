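; Theater puzzle task actor that collects a Comedy mask and a Tragedy mask in an overlap box.
; Each mask is released from its player, placed at its own point and stored, then the TaskIndicator activates a light and a thunk plays.
; Once both masks are valid, it spawns a scaled SinglePressurePlate and assigns it as the indicator's Task.
; The light, sound and plate spawn all require a valid TaskIndicator.
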(event `self.MaskCollectionBox.OnComponentBeginOverlap`
  (params (OverlappedComponent :type "PrimitiveComponent Object Reference") (OtherActor :type "Actor Object Reference") (OtherComp :type "PrimitiveComponent Object Reference") (OtherBodyIndex :type Integer) (bFromSweep :type Boolean) (SweepResult :type "HitResult Structure (by ref)"))
  (bind _comedymaskpoint (`self.ComedyMaskPoint`))
  (bind _tragedymaskpoint (`self.TragedyMaskPoint`))
  (bind _ascomedy_mask (cast `/Game/Blueprints/Tasks/ComedyMask` OtherActor)
    (:`then`
      (set `/Game/Characters/Piecelings/PiecelingBP.HeldItem` null (`/Game/Blueprints/Tasks/Mask.Player` _ascomedy_mask))
      (`/Game/Blueprints/Tasks/Mask.Place` _ascomedy_mask (`SceneComponent.K2_GetComponentLocation` _comedymaskpoint) (`SceneComponent.RelativeRotation` _comedymaskpoint))
      (bind _output_get (set `self.ComedyMask` _ascomedy_mask))
      (set `/Game/Characters/Piecelings/PiecelingBP.HeldItem` null (`/Game/Blueprints/Tasks/Mask.Player` _output_get))
      (set `/Game/Blueprints/Tasks/Mask.Player` null _output_get)
      (`/Engine/EditorBlueprintResources/StandardMacros.IsValid` (`self.TaskIndicator`)
        (:`Is Valid`
          (`/Game/Blueprints/Tasks/TaskDoubleIndicator.ActivateLight` (`self.TaskIndicator`) true))))
    (:`CastFailed`
      (bind _astragedy_mask (cast `/Game/Blueprints/Tasks/TragedyMask` OtherActor))
      (set `/Game/Characters/Piecelings/PiecelingBP.HeldItem` null (`/Game/Blueprints/Tasks/Mask.Player` _astragedy_mask))
      (`/Game/Blueprints/Tasks/Mask.Place` _astragedy_mask (`SceneComponent.K2_GetComponentLocation` _tragedymaskpoint) (`SceneComponent.RelativeRotation` _tragedymaskpoint))
      (bind _output_get_2 (set `self.TragedyMask` _astragedy_mask))
      (set `/Game/Characters/Piecelings/PiecelingBP.HeldItem` null (`/Game/Blueprints/Tasks/Mask.Player` _output_get_2))
      (set `/Game/Blueprints/Tasks/Mask.Player` null _output_get_2)
      (`/Engine/EditorBlueprintResources/StandardMacros.IsValid` (`self.TaskIndicator`)
        (:`Is Valid`
          (`/Game/Blueprints/Tasks/TaskDoubleIndicator.ActivateLight` (`self.TaskIndicator`) false)))))
  (`GameplayStatics.PlaySoundAtLocation` "/Game/Audio/SoundEffects/Thunk.Thunk" (0.0 0.0 0.0) (struct) 1.0 0.8 0.0 null null null)
  (`/Engine/EditorBlueprintResources/StandardMacros.IsValid` _output_get
    (:`Is Valid`
      (`/Engine/EditorBlueprintResources/StandardMacros.IsValid` _output_get_2
        (:`Is Valid`
          (bind _returnvalue (`|SpawnActorFromClass` "/Game/Blueprints/Tasks/SinglePressurePlate.SinglePressurePlate_C" (`KismetMathLibrary.MakeTransform` (`SceneComponent.K2_GetComponentLocation` (`self.PlateSpawnPoint`)) (struct :`Yaw` 90.0) (2.5 2.5 2.5)) "Undefined" "OverrideRootScale" null null))
          (set `/Game/Blueprints/Tasks/TaskDoubleIndicator.Task` _returnvalue (`self.TaskIndicator`)))))))

(fn `UserConstructionScript`)