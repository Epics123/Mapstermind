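; Task indicator actor that shows when its linked Task is completed.
; Tick polls the Task's Completed flag and fires CompleteTask once through a DoOnce.
; CompleteTask plays a ding at the world origin, switches the base to a green light material and runs a timeline that rotates the indicator.
; The rotation uses RInterpTo toward EndRotation, with the timeline's Alpha fed in as DeltaTime.
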(event `self.ReceiveTick`
  (params (DeltaSeconds :type "Float (single-precision)"))
  (bind _task (`self.Task`))
  (`/Engine/EditorBlueprintResources/StandardMacros.IsValid` _task
    (:`Is Valid`
      (if (`Task.Completed` _task)
        (`/Engine/EditorBlueprintResources/StandardMacros.DoOnce` false
          (:`Completed`
            (`self.CompleteTask`)))))))

(event `CompleteTask`
  (`GameplayStatics.PlaySoundAtLocation` "/Game/Audio/SoundEffects/TaskCompleteDing.TaskCompleteDing" (0.0 0.0 0.0) (struct) 0.75 1.0 0.0 null null null)
  (`PrimitiveComponent.SetMaterial` (`self.TaskIndicatorBase`) 0 "/Game/ArtAssets/UI/Task_Indicator/mat_GreenLight.mat_GreenLight")
  (bind (_direction _alpha) (`Timeline|RotateIndicator` :!via `PlayFromStart`)
    (:`Update`
      (`SceneComponent.K2_SetRelativeRotation` (`self.RotatingIndicator`) (`KismetMathLibrary.RInterpTo` (`SceneComponent.RelativeRotation` (`self.RotatingIndicator`)) (`self.EndRotation`) _alpha 1.0) false false))))

(fn `UserConstructionScript`)