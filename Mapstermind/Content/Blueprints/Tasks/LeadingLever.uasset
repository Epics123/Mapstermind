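; LeadingLever is the lead half of a two-lever task in which paired levers alternate pulls.
; Pulling on its active turn swaps the mesh, hides the HUD pull prompt, counts the turn, restores player walking and hands off to PartnerLever via TradeFollow.
; TradeLead counts the partner's pull and re-arms this lever.
; Reaching PumpCount on either count increments the task, with debug prints throughout.
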(event `self.ReceiveBeginPlay`
  (`parent.ReceiveBeginPlay`))

(event `self.Activate_Lever_Pull`
  (bind _turncount (`self.TurnCount`))
  (bind _playerref (`self.PlayerRef`))
  (bind _playerref_2 (`self.PlayerRef`))
  (`KismetSystemLibrary.PrintString` "PUL")
  (`KismetSystemLibrary.PrintString` (`KismetStringLibrary.Conv_IntToString` (`self.TurnCount`)))
  (if (`self.ActiveTurn`)
    (set `self.Pulled` true)
    (`StaticMeshComponent.SetStaticMesh` (`self.LeverMesh`) "/Game/ArtAssets/Tasks/leverPiecelingPos2.leverPiecelingPos2")
    (set `self.CanActivate` false)
    (`/Engine/EditorBlueprintResources/StandardMacros.IncrementInt` _turncount
      (:`  `
        (`KismetSystemLibrary.PrintString` "Lead Count")
        (bind _aslever_hud (cast `/Game/Blueprints/Widgets/Level/LeverHUD` (`WidgetComponent.GetWidget` (`self.Widget`))))
        (`/Game/Blueprints/Widgets/Level/LeverHUD.HidePull` _aslever_hud)
        (if (>= _turncount (`self.PumpCount`))
          (`self.IncrementTask`)
          (`KismetSystemLibrary.PrintString` "Done")
          (`/Engine/EditorBlueprintResources/StandardMacros.IsValid` _playerref_2
            (:`Is Valid`
              (`CharacterMovementComponent.SetMovementMode` (`Character.CharacterMovement` _playerref_2) "MOVE_Walking" 0)))
          (else
            (`/Engine/EditorBlueprintResources/StandardMacros.IsValid` _playerref :!label _label
              (:`Is Valid`
                (`CharacterMovementComponent.SetMovementMode` (`Character.CharacterMovement` _playerref) "MOVE_Walking" 0)
                (set `CapstonePrototype1Character.PullingLever` false _playerref)
                (`/Game/Blueprints/Tasks/FollowerLever.TradeFollow` (`self.PartnerLever`) _playerref)))))))))

(event `EnableMovement`
  (goto _label))

(event `TradeLead`
  (`/Engine/EditorBlueprintResources/StandardMacros.IncrementInt` (`self.TurnCount`)
    (:`  `
      (`KismetSystemLibrary.PrintString` "Partner Count")
      (set `self.ActiveTurn` true :!label _label_2)
      (set `self.Pulled` false)
      (`StaticMeshComponent.SetStaticMesh` (`self.LeverMesh`) "/Game/ArtAssets/Tasks/leverPiecelingFull.leverPiecelingFull")
      (set `self.CanActivate` true)
      (if (>= (`self.TurnCount`) (`self.PumpCount`))
        (`self.IncrementTask`)
        (`KismetSystemLibrary.PrintString` "done")))))

(event `self.Reset_Lever_Pull`
  (goto _label_2))

(fn `EnableMovement_0`)

(fn `UserConstructionScript`
  (`parent.UserConstructionScript`))