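; Task indicator actor with three status lights and a rotating part that shows when its linked Task is completed.
; Tick polls the Task's Completed flag and fires CompleteTask once, playing a ding at world origin, turning the lights green and starting a timeline that interpolates the indicator toward EndRotation.
; ActivateLight and DeactivateLight events switch individual lights green or red through material slots 0, 2 and 3.
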(event `self.ReceiveTick`
  (params (DeltaSeconds :type "Float (single-precision)"))
  (bind _task (`self.Task`))
  (`/Engine/EditorBlueprintResources/StandardMacros.IsValid` _task
    (:`Is Valid`
      (if (`Task.Completed` _task)
        (`/Engine/EditorBlueprintResources/StandardMacros.DoOnce` false
          (:`Completed`
            (`self.CompleteTask`)))))))

(event `CompleteTask`
  (`GameplayStatics.PlaySoundAtLocation` "/Game/Audio/SoundEffects/TaskCompleteDing.TaskCompleteDing" (0.0 0.0 0.0) (struct) 0.75 1.0 0.0 null null null)
  (for _index (range 4)
    (`self.ActivateLight` _index))
  (bind (_direction _aplha) (`Timeline|RotateIndicator` :!via `PlayFromStart`)
    (:`Update`
      (`SceneComponent.K2_SetRelativeRotation` (`self.RotatingIndicator`) (`KismetMathLibrary.RInterpTo` (`SceneComponent.RelativeRotation` (`self.RotatingIndicator`)) (`self.EndRotation`) _aplha 1.0) false false))))

(event `ActivateLight`
  (params (Index :type Integer))
  (switch `int` Index
    (:`0`
      (`PrimitiveComponent.SetMaterial` (`self.TaskIndicatorBase`) Index "/Game/ArtAssets/UI/Task_Indicator/mat_GreenLight.mat_GreenLight"))
    (:`2`
      (`PrimitiveComponent.SetMaterial` (`self.TaskIndicatorBase`) Index "/Game/ArtAssets/UI/Task_Indicator/mat_GreenLight.mat_GreenLight"))
    (:`3`
      (`PrimitiveComponent.SetMaterial` (`self.TaskIndicatorBase`) Index "/Game/ArtAssets/UI/Task_Indicator/mat_GreenLight.mat_GreenLight"))))

(event `DeactivateLight`
  (params (Index :type Integer))
  (switch `int` Index
    (:`0`
      (`PrimitiveComponent.SetMaterial` (`self.TaskIndicatorBase`) Index "/Game/ArtAssets/UI/Task_Indicator/mat_RedLight1.mat_RedLight1"))
    (:`2`
      (`PrimitiveComponent.SetMaterial` (`self.TaskIndicatorBase`) Index "/Game/ArtAssets/UI/Task_Indicator/mat_RedLight1.mat_RedLight1"))
    (:`3`
      (`PrimitiveComponent.SetMaterial` (`self.TaskIndicatorBase`) Index "/Game/ArtAssets/UI/Task_Indicator/mat_RedLight1.mat_RedLight1"))))

(fn `UserConstructionScript`)