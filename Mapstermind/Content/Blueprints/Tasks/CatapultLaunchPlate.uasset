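; Pressure plate actor for a catapult task that fires the catapult when a Pieceling lands on it.
; On overlap with the plate collision, it reacts only to a PiecelingBP whose movement component is falling, so walking onto it does nothing.
; It calls Fire on the Catapult found through GetActorOfClass, then blocks reactivation with a CanActivate flag until a cooldown delay ends.
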(event `self.ReceiveBeginPlay`)

(event `self.PressurePlateCollision.OnComponentBeginOverlap`
  (params (OverlappedComponent :type "PrimitiveComponent Object Reference") (OtherActor :type "Actor Object Reference") (OtherComp :type "PrimitiveComponent Object Reference") (OtherBodyIndex :type Integer) (bFromSweep :type Boolean) (SweepResult :type "HitResult Structure (by ref)"))
  (bind _asthird_person_character (cast `/Game/Characters/Piecelings/PiecelingBP` OtherActor))
  (if (`NavMovementComponent.IsFalling` (`Character.CharacterMovement` _asthird_person_character))
    (if (`self.CanActivate`)
      (set `self.CanActivate` false)
      (bind _returnvalue (`GameplayStatics.GetActorOfClass` "/Game/Blueprints/Weapons/Catapult.Catapult_C"))
      (`/Game/Blueprints/Weapons/Catapult.Fire` _returnvalue)
      (`KismetSystemLibrary.Delay` (`self.Cooldown time`))
      (set `self.CanActivate` true))))

(fn `UserConstructionScript`)