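; DoublePlate is a task actor that completes when both of its pressure plates are pressed at the same time.
; BeginPlay casts two child actors to SinglePressurePlate and clears their IsSingle flag.
; Tick mirrors each plate's state on the TaskIndicator lights until completion, which fires once.
; Completion locks both plates, notifies the indicator, increments the GameMode's task message and flips an optional Pipe's model.
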(event `self.ReceiveBeginPlay`
  (bind _assingle_pressure_plate (cast `/Game/Blueprints/Tasks/SinglePressurePlate` (`ChildActorComponent.ChildActor` (`self.ChildActor1`))))
  (bind _output_get (set `self.Plate1` _assingle_pressure_plate))
  (set `/Game/Blueprints/Tasks/SinglePressurePlate.IsSingle` false _output_get)
  (bind _assingle_pressure_plate_2 (cast `/Game/Blueprints/Tasks/SinglePressurePlate` (`ChildActorComponent.ChildActor` (`self.ChildActor2`))))
  (bind _output_get_2 (set `self.Plate2` _assingle_pressure_plate_2))
  (set `/Game/Blueprints/Tasks/SinglePressurePlate.IsSingle` false _output_get_2))

(event `self.ReceiveTick`
  (params (DeltaSeconds :type "Float (single-precision)"))
  (bind _pipe (`self.Pipe`))
  (`self.SetIndicatorLights` (`self.Completed`))
  (if (and (`/Game/Blueprints/Tasks/SinglePressurePlate.Pressed` (`self.Plate1`)) (`/Game/Blueprints/Tasks/SinglePressurePlate.Pressed` (`self.Plate2`)))
    (`/Engine/EditorBlueprintResources/StandardMacros.DoOnce` false
      (:`Completed`
        (`self.Complete Task`)
        (`/Game/Blueprints/Tasks/TaskDoubleIndicator.CompleteTask` (`self.TaskIndicator`))
        (`/Engine/EditorBlueprintResources/StandardMacros.IsValid` _pipe
          (:`Is Valid`
            (`/Game/Blueprints/Tasks/SewerPipeTask.FlipModel` _pipe)))))))

(event `Complete Task`
  (bind _plate1 (`self.Plate1`))
  (bind _plate2 (`self.Plate2`))
  (set `/Game/Blueprints/Tasks/SinglePressurePlate.CanActivate` false _plate1)
  (set `/Game/Blueprints/Tasks/SinglePressurePlate.MultiDone` true _plate1)
  (set `/Game/Blueprints/Tasks/SinglePressurePlate.CanActivate` false _plate2)
  (set `/Game/Blueprints/Tasks/SinglePressurePlate.MultiDone` true _plate2)
  (bind _completedtasknum (message `/Game/Blueprints/Modes_States/LocalMPGameModeInterface.IncrementTask` (`GameplayStatics.GetGameMode`)))
  (`KismetSystemLibrary.PrintString` (`KismetStringLibrary.Conv_IntToString` _completedtasknum))
  (set `self.Completed` true))

(fn `SetIndicatorLights`
  (params (Complete :type Boolean))
  (bind _taskindicator (`self.TaskIndicator`))
  (bind _taskindicator_2 (`self.TaskIndicator`))
  (if (not Complete)
    (`|ExecutionSequence`
      (:`then_0`
        (if (`/Game/Blueprints/Tasks/SinglePressurePlate.Pressed` (`self.Plate1`))
          (`/Game/Blueprints/Tasks/TaskDoubleIndicator.ActivateLight` _taskindicator_2 true)
          (else
            (`/Game/Blueprints/Tasks/TaskDoubleIndicator.DeactivateLight` _taskindicator_2 true))))
      (:`then_1`
        (if (`/Game/Blueprints/Tasks/SinglePressurePlate.Pressed` (`self.Plate2`))
          (`/Game/Blueprints/Tasks/TaskDoubleIndicator.ActivateLight` _taskindicator false)
          (else
            (`/Game/Blueprints/Tasks/TaskDoubleIndicator.DeactivateLight` _taskindicator false)))))))

(fn `UserConstructionScript`)