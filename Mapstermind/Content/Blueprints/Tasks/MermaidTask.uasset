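; Mermaid statue task actor that collects three items: a crown, a pearl and a goblet.
; Each item has a deposit area that open and close events show or hide, and overlaps only count while it is open.
; AddToStatue identifies the item by cast, destroys it, reveals its mesh, flags it as added and closes that area.
; Only the crown must also be grabbed to be accepted.
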(event `self.CrownArea.OnComponentBeginOverlap`
  (params (OverlappedComponent :type "PrimitiveComponent Object Reference") (OtherActor :type "Actor Object Reference") (OtherComp :type "PrimitiveComponent Object Reference") (OtherBodyIndex :type Integer) (bFromSweep :type Boolean) (SweepResult :type "HitResult Structure (by ref)"))
  (bind _ascrown_pickup (cast `/Game/Blueprints/Tasks/CrownPickup` OtherActor))
  (if (`/Game/Blueprints/Tasks/CrownPickup.Grabbed` _ascrown_pickup)
    (if (`self.CrownOpen`)
      (`self.AddToStatue` _ascrown_pickup))))

(event `OpenCrown`
  ;[0 1 0] Opening Item Deposit Areas
  (`SceneComponent.SetVisibility` (`self.CrownArea`) true false)
  (set `self.CrownOpen` true))

(event `CloseCrown`
  ;[1 0 0] Closing Item Deposit Areas
  (`SceneComponent.SetVisibility` (`self.CrownArea`) false false)
  (set `self.CrownOpen` false))

(event `OpenPearl`
  ;[0 1 0] Opening Item Deposit Areas
  (`SceneComponent.SetVisibility` (`self.PearlArea`) true false)
  (set `self.PearlOpen` true))

(event `ClosePearl`
  ;[1 0 0] Closing Item Deposit Areas
  (`SceneComponent.SetVisibility` (`self.PearlArea`) false false)
  (set `self.PearlOpen` false))

(event `self.PearlArea.OnComponentBeginOverlap`
  (params (OverlappedComponent :type "PrimitiveComponent Object Reference") (OtherActor :type "Actor Object Reference") (OtherComp :type "PrimitiveComponent Object Reference") (OtherBodyIndex :type Integer) (bFromSweep :type Boolean) (SweepResult :type "HitResult Structure (by ref)"))
  (bind _aspearl (cast `/Game/Blueprints/Tasks/Pearl` OtherActor))
  (if (`self.PearlOpen`)
    (`self.AddToStatue` _aspearl)))

(event `OpenGoblet`
  ;[0 1 0] Opening Item Deposit Areas
  (`SceneComponent.SetVisibility` (`self.GobletArea`) true false)
  (set `self.GobletOpen` true))

(event `CloseGoblet`
  ;[1 0 0] Closing Item Deposit Areas
  (`SceneComponent.SetVisibility` (`self.GobletArea`) false false)
  (set `self.GobletOpen` false))

(event `self.GobletArea.OnComponentBeginOverlap`
  (params (OverlappedComponent :type "PrimitiveComponent Object Reference") (OtherActor :type "Actor Object Reference") (OtherComp :type "PrimitiveComponent Object Reference") (OtherBodyIndex :type Integer) (bFromSweep :type Boolean) (SweepResult :type "HitResult Structure (by ref)"))
  (bind _asgoblet (cast `/Game/Blueprints/Tasks/Goblet` OtherActor))
  (if (`self.GobletOpen`)
    (`self.AddToStatue` _asgoblet)))

(event `AddToStatue`
  (params (Item :type "Item Object Reference"))
  (bind _ascrown_pickup (cast `/Game/Blueprints/Tasks/CrownPickup` Item)
    (:`then`
      (`self.K2_DestroyActor` _ascrown_pickup)
      (`SceneComponent.SetVisibility` (`self.CrownMesh`) true false)
      (set `self.CrownAdded` true)
      (`self.CloseCrown`))
    (:`CastFailed`
      (bind _aspearl (cast `/Game/Blueprints/Tasks/Pearl` Item)
        (:`then`
          (`self.K2_DestroyActor` _aspearl)
          (`SceneComponent.SetVisibility` (`self.PearlMesh`) true false)
          (set `self.PearlAdded` true)
          (`self.ClosePearl`))
        (:`CastFailed`
          (bind _asgoblet (cast `/Game/Blueprints/Tasks/Goblet` Item))
          (`self.K2_DestroyActor` _asgoblet)
          (`SceneComponent.SetVisibility` (`self.GobletMesh`) true false)
          (set `self.GobletAdded` true)
          (`self.CloseGoblet`))))))

(fn `UserConstructionScript`)