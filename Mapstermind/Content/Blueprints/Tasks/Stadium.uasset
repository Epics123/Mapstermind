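; Stadium task actor where baseballs are thrown, completing a single or three-throw task depending on its indicator.
; Overlap by a throwable Baseball closes the area's collision and triggers the throw.
; EventTaskIncrement either completes immediately or counts throws, lighting indicators and launching homeruns until the third.
; Homeruns move the ball along a timeline-driven parabolic arc to a random preset location, then re-enable pickup.
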(event `OpenStadium`
  (`SceneComponent.SetVisibility` (`self.AreaEffect`) false false)
  (`PrimitiveComponent.SetCollisionEnabled` (`self.AreaEffect`) "QueryOnly"))

(event `CloseStadium`
  (`SceneComponent.SetVisibility` (`self.AreaEffect`) false false)
  (`PrimitiveComponent.SetCollisionEnabled` (`self.AreaEffect`) "NoCollision"))

(event `self.ReceiveActorBeginOverlap`
  (params (OtherActor :type "Actor Object Reference"))
  (bind _asbaseball (cast `/Game/Blueprints/Tasks/Baseball` OtherActor))
  (if (`/Game/Blueprints/Tasks/Baseball.CanThrow` _asbaseball)
    (set `self.Baseball` _asbaseball)
    (`self.CloseStadium`)
    (`/Game/Blueprints/Tasks/Baseball.Throw` _asbaseball)))

(event `self.ReceiveHit`
  (params (MyComp :type "PrimitiveComponent Object Reference") (Other :type "Actor Object Reference") (OtherComp :type "PrimitiveComponent Object Reference") (bSelfMoved :type Boolean) (HitLocation :type "Vector Structure") (HitNormal :type "Vector Structure") (NormalImpulse :type "Vector Structure") (Hit :type "HitResult Structure (by ref)")))

(event `EventTaskIncrement`
  (`/Engine/EditorBlueprintResources/StandardMacros.IsValid` (`self.TripleTaskIndicator`)
    (:`Is Valid`
      (set `self.NumThrows` (+ (`self.NumThrows`) 1))
      (if (== (`self.NumThrows`) 1)
        (`/Game/Blueprints/Tasks/TaskTripleIndicator.ActivateLight` (`self.TripleTaskIndicator`) (- (`self.NumThrows`) 1))
        (`self.EventHomerun`)
        (else
          (`/Game/Blueprints/Tasks/TaskTripleIndicator.ActivateLight` (`self.TripleTaskIndicator`) (`self.NumThrows`))
          (if (== (`self.NumThrows`) 3)
            (message `/Game/Blueprints/Modes_States/LocalMPGameModeInterface.IncrementTask` (`GameplayStatics.GetGameMode`))
            (`/Game/Blueprints/Tasks/TaskTripleIndicator.CompleteTask` (`self.TripleTaskIndicator`))
            (`SceneComponent.SetVisibility` (`/Game/Blueprints/Tasks/Baseball.StaticMesh` (`self.Baseball`)) false false)
            (else
              (`self.EventHomerun`))))))
    (:`Is Not Valid`
      (`self.CompleteTask`))))

(event `self.CompleteTask`
  (`GameplayStatics.PlaySoundAtLocation` "/Game/Audio/SoundEffects/CatchersMitt1.CatchersMitt1" (0.0 0.0 0.0) (struct) 1.0 1.0 0.0 null null null)
  (message `/Game/Blueprints/Modes_States/LocalMPGameModeInterface.IncrementTask` (`GameplayStatics.GetGameMode`))
  (`/Game/Blueprints/Tasks/TaskIndicator.CompleteTask` (`self.TaskIndicator`)))

(event `EventHomerun`
  (`GameplayStatics.PlaySoundAtLocation` "/Game/Audio/SoundEffects/MetalBat3.MetalBat3" (0.0 0.0 0.0) (struct) 1.0 1.0 0.0 null null null)
  ;[1 0.1834 0.5005] Setting the start location for the homerun in the center of the stadium
  (set `self.HomerunStartLoc` (`SceneComponent.K2_GetComponentLocation` (`self.HitPoint`)))
  ;[0.7274 0.2752 1] Setting the end location for the homerun to be at a random location in the array
  (set `self.HomerunEndLoc` (`|GetArrayItem` (`self.HomerunLocations`) (`KismetMathLibrary.RandomIntegerInRange` 0 (- (`KismetArrayLibrary.Array_Length` (`self.HomerunLocations`)) 1))))
  (`self.K2_SetActorLocation` (`self.Baseball`) (`self.HomerunStartLoc`) false false)
  (`SceneComponent.K2_SetWorldLocation` (`/Game/Blueprints/Tasks/Baseball.StaticMesh` (`self.Baseball`)) (`self.HomerunStartLoc`) false true)
  (set `/Game/Blueprints/Tasks/Baseball.CanPickUp` false (`self.Baseball`))
  (set `/Game/Blueprints/Tasks/Baseball.CanThrow` false (`self.Baseball`))
  (bind (_direction _deltatime) (`Timeline|LERP Timeline` :!via `PlayFromStart`)
    (:`Update`
      ;[0 0.9838 1] Lerping the Baseball
      (`KismetMathLibrary.Vector_Set` (`self.HitLocVector`) (`KismetMathLibrary.Lerp` (.x (`SceneComponent.K2_GetComponentLocation` (`/Game/Blueprints/Tasks/Baseball.StaticMesh` (`self.Baseball`)))) (.x (`self.HomerunEndLoc`)) _deltatime) (`KismetMathLibrary.Lerp` (.y (`SceneComponent.K2_GetComponentLocation` (`/Game/Blueprints/Tasks/Baseball.StaticMesh` (`self.Baseball`)))) (.y (`self.HomerunEndLoc`)) _deltatime) (+ (+ (`self.homerunHeight`) (* (* (`self.homerunHeight`) -4.0) (`KismetMathLibrary.MultiplyMultiply_FloatFloat` (* (+ _deltatime -0.07) 7.0) 2.0))) (.z (`self.HomerunStartLoc`))))
      (`self.K2_SetActorLocation` (`self.Baseball`) (`self.HitLocVector`) false true)
      (`SceneComponent.K2_SetWorldLocation` (`/Game/Blueprints/Tasks/Baseball.StaticMesh` (`self.Baseball`)) (`self.HitLocVector`) false true))
    (:`Finished`
      ;[1 0.826 0] Allow the ball to be picked up when the hit is finished
      (`self.K2_SetActorLocation` (`self.Baseball`) (`self.HomerunEndLoc`) false true)
      (`SceneComponent.K2_SetWorldLocation` (`/Game/Blueprints/Tasks/Baseball.StaticMesh` (`self.Baseball`)) (`self.HomerunEndLoc`) false true)
      (set `/Game/Blueprints/Tasks/Baseball.CanPickUp` true (`self.Baseball`))
      (set `/Game/Blueprints/Tasks/Baseball.ThrowFinished` false (`self.Baseball`)))))

(fn `SpawnBall`
  (`|SpawnActorFromClass` "/Game/Blueprints/Tasks/TutorialBaseball.TutorialBaseball_C" (`KismetMathLibrary.MakeTransform` (`SceneComponent.K2_GetComponentLocation` (`self.BaseballSpawnPoint`))) "Undefined" "OverrideRootScale" null null))

(fn `UserConstructionScript`)