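; Bubble actor carrying a crown for the mermaid task, looping along a track spline until a sea urchin pops it.
; A timeline drives the movement from elapsed time and speed, restarting at the spline's end.
; Popping hides the bubble and drops the crown with physics, then swaps the actor for a CrownPickup after a delay.
; Pickup and Drop events handle attachment and tell MermaidTask to open or close the crown.
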(event `self.ReceiveBeginPlay`
  (set `self.itemType` "CROWN")
  (`self.FollowSpline`))

(event `self.ReceiveActorBeginOverlap`
  (params (OtherActor :type "Actor Object Reference"))
  (cast `/Game/Blueprints/Tasks/SeaUrchin` OtherActor)
  (if (`self.CanPop`)
    (`self.Pop`)
    (set `self.CanPop` false)))

(event `Pop`
  (`SceneComponent.SetVisibility` (`self.BubbleMesh`) false false)
  (`PrimitiveComponent.SetSimulatePhysics` (`self.CrownMesh`) true)
  (`PrimitiveComponent.SetCollisionEnabled` (`self.CrownMesh`) "QueryAndPhysics")
  (`GameplayStatics.PlaySoundAtLocation` "/Game/Audio/SoundEffects/BubblePop.BubblePop" (0.0 0.0 0.0) (struct) 1.0 1.0 0.0 null null null)
  (`KismetSystemLibrary.Delay` (`self.FallTime`))
  (`|SpawnActorFromClass` "/Game/Blueprints/Tasks/CrownPickup.CrownPickup_C" (`KismetMathLibrary.MakeTransform` (`SceneComponent.K2_GetComponentLocation` (`self.CrownMesh`)) (`SceneComponent.K2_GetComponentRotation` (`self.CrownMesh`))) "Undefined" "OverrideRootScale" null null)
  (`self.K2_DestroyActor`))

(event `FollowSpline`
  (bind _distance (`self.Distance`))
  (bind _track (`self.Track`))
  (bind _bubblespline (`/Game/Blueprints/Tasks/BubbleTrack.BubbleSpline` _track))
  (if (`self.CanPop`)
    (set `self.Distance` 0.0)
    (set `self.Time` 0.0)
    (`Timeline|Path` :!via `PlayFromStart`
      (:`Update`
        (if (`self.CanPop`)
          (bind _output_get (set `self.Time` (+ (`self.Time`) (`GameplayStatics.GetWorldDeltaSeconds`))))
          (set `self.Distance` (* _output_get (`self.Speed`)))
          (`/Engine/EditorBlueprintResources/StandardMacros.IsValid` _track
            (:`Is Valid`
              (`self.K2_SetActorLocation` (`SplineComponent.GetLocationAtDistanceAlongSpline` _bubblespline _distance "World"))
              (if (>= _distance (`SplineComponent.GetSplineLength` _bubblespline))
                (`self.FollowSpline`)))))))))

(event `Pickup`
  (params (Parent :type "Actor Object Reference") (Location :type "Vector Structure"))
  (if (not (`self.Grabbed`))
    (`PrimitiveComponent.SetSimulatePhysics` (`self.CrownMesh`) false)
    (`self.K2_AttachToActor` Parent "None" "KeepWorld" "KeepWorld" "KeepWorld")
    (`self.K2_SetActorLocation` Location)
    (bind _returnvalue (`GameplayStatics.GetActorOfClass` "/Game/Blueprints/Tasks/MermaidTask.MermaidTask_C"))
    (`/Game/Blueprints/Tasks/MermaidTask.OpenCrown` _returnvalue)
    (set `self.Grabbed` true)))

(event `Drop`
  (params (Parent :type "Actor Object Reference"))
  (cast `/Game/Characters/Piecelings/PiecelingBP` Parent)
  (`self.K2_DetachFromActor` "KeepWorld" "KeepWorld" "KeepWorld")
  (set `self.Grabbed` false)
  (bind _returnvalue (`GameplayStatics.GetActorOfClass` "/Game/Blueprints/Tasks/MermaidTask.MermaidTask_C"))
  (`/Game/Blueprints/Tasks/MermaidTask.CloseCrown` _returnvalue))

(fn `UserConstructionScript`)