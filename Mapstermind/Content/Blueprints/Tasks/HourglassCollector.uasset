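; Hourglass collection point that adds time to the local multiplayer game's clock when an hourglass enters its box.
; On overlap with an Hourglass actor, it calls IncreaseTime, destroys the hourglass and plays the ClockWind sound at the world origin.
; IncreaseTime casts the game mode to LocalMPGameMode and adds TimeIncrease to its Seconds value.
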(event `self.Box.OnComponentBeginOverlap`
  (params (OverlappedComponent :type "PrimitiveComponent Object Reference") (OtherActor :type "Actor Object Reference") (OtherComp :type "PrimitiveComponent Object Reference") (OtherBodyIndex :type Integer) (bFromSweep :type Boolean) (SweepResult :type "HitResult Structure (by ref)"))
  (cast `/Game/Blueprints/Tasks/Hourglass` OtherActor)
  (`self.IncreaseTime`)
  (`self.K2_DestroyActor` OtherActor)
  (`GameplayStatics.PlaySoundAtLocation` "/Game/Audio/SoundEffects/ClockWind.ClockWind" (0.0 0.0 0.0) (struct) 1.0 1.0 0.0 null null null))

(event `IncreaseTime`
  (bind _aslocal_mpgame_mode (cast `/Game/Blueprints/Modes_States/LocalMPGameMode` (`GameplayStatics.GetGameMode`)))
  (set `/Game/Blueprints/Modes_States/LocalMPGameMode.Seconds` (+ (`/Game/Blueprints/Modes_States/LocalMPGameMode.Seconds` _aslocal_mpgame_mode) (`self.TimeIncrease`)) _aslocal_mpgame_mode))

(fn `UserConstructionScript`)