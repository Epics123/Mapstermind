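; Treasure chest actor whose lid opens to a rotation chosen by pump number and which launches a goblet along a spline.
; OpenTop plays a timeline that eases the lid toward the indexed rotation, feeding timeline alpha into RInterpTo as delta time.
; LaunchGoblet flags the chest open, spawns a goblet and moves it by speed-based spline distance on timeline updates; the end-of-spline check does nothing.
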(event `OpenTop`
  (params (PumpNum :type Integer))
  (bind (_direction _alpha) (`Timeline|OpenChest` :!via `PlayFromStart`)
    (:`Update`
      (`SceneComponent.K2_SetRelativeRotation` (`self.ChestTop`) (`KismetMathLibrary.RInterpTo` (`SceneComponent.RelativeRotation` (`self.ChestTop`)) (`|GetArrayItem` (`self.ChestRotations`) PumpNum) _alpha 1.0) false false))))

(event `LaunchGoblet`
  (set `self.IsOpen` true)
  (bind _returnvalue (`|SpawnActorFromClass` "/Game/Blueprints/Tasks/Goblet.Goblet_C" (`KismetMathLibrary.MakeTransform` (0.0 0.0 0.0)) "Undefined" "OverrideRootScale" null null))
  (`self.FollowSpline` _returnvalue))

(event `FollowSpline`
  (params (Goblet :type "Actor Object Reference"))
  (bind _distance (`self.Distance`))
  (bind _spline (`self.Spline`))
  (set `self.Distance` 0.0)
  (set `self.Time` 0.0)
  (`Timeline|Timeline_0` :!via `PlayFromStart`
    (:`Update`
      (bind _output_get (set `self.Time` (+ (`self.Time`) (`GameplayStatics.GetWorldDeltaSeconds`))))
      (set `self.Distance` (* _output_get (`self.Speed`)))
      (`/Engine/EditorBlueprintResources/StandardMacros.IsValid` _spline
        (:`Is Valid`
          (`self.K2_SetActorLocation` Goblet (`SplineComponent.GetLocationAtDistanceAlongSpline` _spline _distance "World") false false)
          (if (>= _distance (`SplineComponent.GetSplineLength` _spline))
            _))))))

(fn `UserConstructionScript`)