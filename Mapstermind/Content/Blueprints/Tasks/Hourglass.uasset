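; Hourglass pickup actor that spins on all three axes and can be picked up and dropped, with a screen-space PickupUI prompt.
; Tick reapplies a cached world transform to the widget so the spin does not move it.
; PickUp attaches the actor to a parent at a given location and hides the prompt, while Drop detaches it and re-caches that transform from the root.
; Visibility events toggle the prompt and its animation.
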(event `self.ReceiveBeginPlay`
  (bind _aspickup_ui (cast `/Game/Blueprints/Widgets/UITextures/Tutorial/Final/Piecelings/PickupUI` (`WidgetComponent.GetWidget` (`self.PickupWidget`))))
  (set `self.PickupUI` _aspickup_ui)
  (`WidgetComponent.SetWidgetSpace` (`self.PickupWidget`) "Screen")
  (set `self.PositionUI` (`SceneComponent.GetSocketTransform` (`self.PickupWidget`) "None" "RTS_World")))

(event `self.ReceiveTick`
  (params (DeltaSeconds :type "Float (single-precision)"))
  (bind _returnvalue (* DeltaSeconds (`self.RotationRate`)))
  (`self.K2_AddActorLocalRotation` (`KismetMathLibrary.MakeRotator` _returnvalue _returnvalue _returnvalue))
  (`SceneComponent.K2_SetWorldTransform` (`self.PickupWidget`) (`self.PositionUI`) false false))

(event `PickUp`
  (params (Parent :type "Actor Object Reference") (Location :type "Vector Structure"))
  (`self.K2_AttachToActor` Parent "None" "KeepWorld" "KeepWorld" "KeepWorld")
  (`self.K2_SetActorLocation` Location)
  (`self.PickupUI_Invisible`))

(event `Drop`
  (`self.K2_DetachFromActor` "KeepWorld" "KeepWorld" "KeepWorld")
  (set `self.PositionUI` (`SceneComponent.GetSocketTransform` (`self.DefaultSceneRoot`) "None" "RTS_World")))

(event `PickupUI_Visible`
  (`SceneComponent.SetVisibility` (`self.PickupWidget`) true false)
  (`/Game/Blueprints/Widgets/UITextures/Tutorial/Final/Piecelings/PickupUI.PlayAnim` (`self.PickupUI`)))

(event `PickupUI_Invisible`
  (`SceneComponent.SetVisibility` (`self.PickupWidget`) false false)
  (`/Game/Blueprints/Widgets/UITextures/Tutorial/Final/Piecelings/PickupUI.StopAnim` (`self.PickupUI`)))

(fn `UserConstructionScript`)