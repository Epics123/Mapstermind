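; Task indicator actor with two status lights and a rotating part that signals when its linked Task is finished.
; ActivateLight and DeactivateLight switch the left or right material slot on the base mesh between green and red.
; Tick polls Task.Completed and, once, plays a ding at world origin and starts a timeline.
; That timeline turns the indicator toward EndRotation with RInterpTo, feeding the track value in as DeltaTime.
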(event `self.ReceiveTick`
  (params (DeltaSeconds :type "Float (single-precision)"))
  (bind _task (`self.Task`))
  (`/Engine/EditorBlueprintResources/StandardMacros.IsValid` _task
    (:`Is Valid`
      (if (`Task.Completed` _task)
        (`/Engine/EditorBlueprintResources/StandardMacros.DoOnce` false
          (:`Completed`
            (`self.CompleteTask`)))))))

(event `CompleteTask`
  (`GameplayStatics.PlaySoundAtLocation` "/Game/Audio/SoundEffects/TaskCompleteDing.TaskCompleteDing" (0.0 0.0 0.0) (struct) 0.75 1.0 0.0 null null null)
  (bind (_direction _aplha) (`Timeline|RotateIndicator` :!via `PlayFromStart`)
    (:`Update`
      (`SceneComponent.K2_SetRelativeRotation` (`self.RotatingIndicator`) (`KismetMathLibrary.RInterpTo` (`SceneComponent.RelativeRotation` (`self.RotatingIndicator`)) (`self.EndRotation`) _aplha 1.0) false false))))

(event `ActivateLight`
  (params (isLeft :type Boolean))
  (if isLeft
    (`PrimitiveComponent.SetMaterial` (`self.TaskIndicatorBase`) 3 "/Game/ArtAssets/UI/Task_Indicator/mat_GreenLight.mat_GreenLight")
    (else
      (`PrimitiveComponent.SetMaterial` (`self.TaskIndicatorBase`) 1 "/Game/ArtAssets/UI/Task_Indicator/mat_GreenLight.mat_GreenLight"))))

(event `DeactivateLight`
  (params (isLeft :type Boolean))
  (if isLeft
    (`PrimitiveComponent.SetMaterial` (`self.TaskIndicatorBase`) 3 "/Game/ArtAssets/UI/Task_Indicator/mat_RedLight1.mat_RedLight1")
    (else
      (`PrimitiveComponent.SetMaterial` (`self.TaskIndicatorBase`) 1 "/Game/ArtAssets/UI/Task_Indicator/mat_RedLight1.mat_RedLight1"))))

(fn `UserConstructionScript`)