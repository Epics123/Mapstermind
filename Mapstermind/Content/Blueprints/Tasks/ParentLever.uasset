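; ParentLever is a base lever task actor that Pieceling characters can grab and pull, with empty pull, reset and tick events.
; A detection sphere registers one Pieceling at a time, links the lever to it, resets the pull and toggles LeverHUD prompts.
; Activation disables the character's movement and further activation, while a separate event increments the GameMode's task message.
; On BeginPlay the prompt widget turns toward the first CameraActor and rises above the lever.
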(event `self.ReceiveBeginPlay`
  (bind _widget (`self.Widget`))
  (bind _outactors (`GameplayStatics.GetAllActorsOfClass` "/Script/Engine.CameraActor"))
  (bind (_returnvalue_roll _returnvalue_pitch _returnvalue_yaw) (`KismetMathLibrary.BreakRotator` (`KismetMathLibrary.FindLookAtRotation` (`SceneComponent.K2_GetComponentLocation` _widget) (`self.K2_GetActorLocation` (`|GetArrayItem` _outactors)))))
  (`SceneComponent.K2_SetWorldRotation` _widget (`KismetMathLibrary.MakeRotator` 0.0 _returnvalue_pitch _returnvalue_yaw) false false)
  (`SceneComponent.K2_SetWorldLocation` _widget (+ (`SceneComponent.K2_GetComponentLocation` _widget) (0.0 0.0 300.0)) false false))

(event `IncrementTask`
  (message `/Game/Blueprints/Modes_States/LocalMPGameModeInterface.IncrementTask` (`GameplayStatics.GetGameMode`)))

(event `Activate_Lever_Pull`)

(event `self.ReceiveTick`
  (params (DeltaSeconds :type "Float (single-precision)")))

(event `Reset_Lever_Pull`)

(event `self.ActivateLever`
  (params (Character :type "CapstonePrototype1Character Object Reference"))
  (`CharacterMovementComponent.DisableMovement` (`Character.CharacterMovement` Character))
  (set `self.CanActivate` false)
  (bind _aspieceling_bp (cast `/Game/Characters/Piecelings/PiecelingBP` Character))
  (set `self.PlayerRef` _aspieceling_bp))

(event `self.DetectionSphere.OnComponentBeginOverlap`
  (params (OverlappedComponent :type "PrimitiveComponent Object Reference") (OtherActor :type "Actor Object Reference") (OtherComp :type "PrimitiveComponent Object Reference") (OtherBodyIndex :type Integer) (bFromSweep :type Boolean) (SweepResult :type "HitResult Structure (by ref)"))
  (bind _aspieceling_bp (cast `/Game/Characters/Piecelings/PiecelingBP` OtherActor))
  (`/Engine/EditorBlueprintResources/StandardMacros.IsValid` (`self.PlayerRef`)
    (:`Is Not Valid`
      (set `/Game/Characters/Piecelings/PiecelingBP.NewCurrentLever` self _aspieceling_bp)
      (set `self.PlayerRef` _aspieceling_bp)
      (`self.Reset_Lever_Pull`)
      (if (`self.CanActivate`)
        (bind _aslever_hud (cast `/Game/Blueprints/Widgets/Level/LeverHUD` (`WidgetComponent.GetWidget` (`self.Widget`))))
        (`/Game/Blueprints/Widgets/Level/LeverHUD.ShowGrab` _aslever_hud)))))

(event `self.DetectionSphere.OnComponentEndOverlap`
  (params (OverlappedComponent :type "PrimitiveComponent Object Reference") (OtherActor :type "Actor Object Reference") (OtherComp :type "PrimitiveComponent Object Reference") (OtherBodyIndex :type Integer))
  (bind _aspieceling_bp (cast `/Game/Characters/Piecelings/PiecelingBP` OtherActor))
  (set `/Game/Characters/Piecelings/PiecelingBP.CurrentLever` null _aspieceling_bp)
  (set `self.PlayerRef` null)
  (bind _aslever_hud (cast `/Game/Blueprints/Widgets/Level/LeverHUD` (`WidgetComponent.GetWidget` (`self.Widget`))))
  (`/Game/Blueprints/Widgets/Level/LeverHUD.HidePull` _aslever_hud))

(fn `CheckPulled`
  (returns (Pulled :type Boolean))
  (return (`self.Pulled`)))

(fn `UserConstructionScript`)