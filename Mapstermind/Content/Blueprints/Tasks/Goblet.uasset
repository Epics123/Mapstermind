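; Goblet item for the mermaid task that the player's PiecelingBP can pick up and drop.
; On pickup it attaches to the carrier, moves to the given location, registers as the held item, calls OpenGoblet on the level's MermaidTask and hides its prompt.
; Drop detaches it and clears the player's held and current item references.
; A screen-space widget serves as the pickup prompt, animating while shown.
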(event `self.ReceiveBeginPlay`
  (set `self.itemType` "Goblet")
  (bind _aspickup_ui (cast `/Game/Blueprints/Widgets/UITextures/Tutorial/Final/Piecelings/PickupUI` (`WidgetComponent.GetWidget` (`self.PickupWidget`))))
  (set `self.PickupUI` _aspickup_ui)
  (`WidgetComponent.SetWidgetSpace` (`self.PickupWidget`) "Screen"))

(event `PickUp`
  (params (Parent :type "Actor Object Reference") (Location :type "Vector Structure"))
  (`self.K2_AttachToActor` Parent "None" "KeepWorld" "KeepWorld" "KeepWorld")
  (`self.K2_SetActorLocation` Location)
  (bind _aspieceling_bp (cast `/Game/Characters/Piecelings/PiecelingBP` Parent))
  (bind _output_get (set `self.Player` _aspieceling_bp))
  (set `/Game/Characters/Piecelings/PiecelingBP.HeldItem` self _output_get)
  (bind _returnvalue (`GameplayStatics.GetActorOfClass` "/Game/Blueprints/Tasks/MermaidTask.MermaidTask_C"))
  (`/Game/Blueprints/Tasks/MermaidTask.OpenGoblet` _returnvalue)
  (`self.PickupUI_invisible`))

(event `Drop`
  (bind _player (`self.Player`))
  (`self.K2_DetachFromActor` "KeepWorld" "KeepWorld" "KeepWorld")
  (set `/Game/Characters/Piecelings/PiecelingBP.HeldItem` null _player)
  (set `/Game/Characters/Piecelings/PiecelingBP.CurrentItem` null _player)
  (set `self.Player` null))

(event `PickupUI_visible`
  (`SceneComponent.SetVisibility` (`self.PickupWidget`) true false)
  (`/Game/Blueprints/Widgets/UITextures/Tutorial/Final/Piecelings/PickupUI.PlayAnim` (`self.PickupUI`)))

(event `PickupUI_invisible`
  (`SceneComponent.SetVisibility` (`self.PickupWidget`) false false)
  (`/Game/Blueprints/Widgets/UITextures/Tutorial/Final/Piecelings/PickupUI.StopAnim` (`self.PickupUI`)))

(fn `UserConstructionScript`)